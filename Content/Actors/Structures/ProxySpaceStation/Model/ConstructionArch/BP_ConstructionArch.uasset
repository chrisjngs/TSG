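; BP_ConstructionArch is a construction arch structure for the proxy space station, built procedurally along a spline.
; The construction script adds MiddleSection mesh instances, with the loop bound derived from spline length divided by mesh X size.
; That unfloored ratio, rather than mesh size, also serves as the distance step between instances.
; Instances use local spline positions without following spline rotation; BeginPlay is empty.
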(event EventBeginPlay)

(fn ConstructionScript
  (bind _spline (Variables|Default|GetSpline))
  (bind _middlesection (Variables|Default|GetMiddleSection))
  (bind _returnvalue (Spline|GetSplineLength _spline))
  (bind _staticmesh (Variables|/Script/Engine.StaticMeshComponent|GetStaticMesh _middlesection))
  (bind _returnvalue_2 (StaticMesh|GetBoundingBox _staticmesh))
  (bind _returnvalue_3 (- (.max _returnvalue_2) (.min _returnvalue_2)))
  (bind _returnvalue_4 (/ _returnvalue (.x _returnvalue_3)))
  (for _index (range 0 (Math|Float|Floor _returnvalue_4))
    (Components|InstancedStaticMesh|AddInstance (Variables|Default|GetMiddleSection) (Math|Transform|MakeTransform (Spline|GetLocationatDistanceAlongSpline (Variables|Default|GetSpline) (* _index _returnvalue_4) "Local")) false)))