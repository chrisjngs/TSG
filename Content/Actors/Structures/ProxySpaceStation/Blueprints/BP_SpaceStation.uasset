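; Space station actor that acts as a faction-aligned, targetable platform armed with missile silos.
; On BeginPlay it spawns a silo at each "Weapon"-tagged child actor component, plus weapon and sensor controllers.
; It hands these to a spawned PSC master, which it then initializes.
; Faction changes propagate to the PSC and platform components, while interface functions expose faction, targeting and launchers, with several left as stubs.
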(event EventBeginPlay
  (bind _returnvalue (Transformation|GetActorTransform))
  (CallFunction|SetFactionType (Variables|Init|GetFaction))
  (for _array_element (Actor|GetComponentsByClass self "/Script/Engine.ChildActorComponent")
    (if (Components|ComponentHasTag _array_element "Weapon")
      (bind _returnvalue_2 (Game|SpawnActorfromClass "/Game/Actors/WeaponSystems/__ParentActors/BP_MissileSiloWeaponParent_Base.BP_MissileSiloWeaponParent_Base_C" (Transformation|GetWorldTransform _array_element) "AlwaysSpawn" "MultiplyWithRoot" 0 "/Game/Actors/WeaponSystems/__DataAssets/DA_MissilSilo.DA_MissilSilo" 1 0))
      (Class|BPITargetable|SetFactionType(Message) _returnvalue_2 (Variables|Init|GetFaction))
      (Utilities|Array|Add (Variables|Default|GetMissileComponents) _returnvalue_2)))
  (Utilities|FlowControl|Sequence
    (:then_0
      (bind _returnvalue_3 (Game|SpawnActorfromClass "/Game/Actors/WeaponSystems/WeaponControllers/ZZZ_WeaponController/BP_WeaponController_Base.BP_WeaponController_Base_C" _returnvalue "AlwaysSpawn" "MultiplyWithRoot" 0 0))
      (Utilities|Array|Add (Variables|Default|GetPlatformComponentsShip) _returnvalue_3)
      (Class|BPIWeaponController|SetFaction(Message) _returnvalue_3 (Variables|Init|GetFaction)))
    (:then_1
      (bind _returnvalue_4 (Game|SpawnActorfromClass "/Game/Blueprints/Components/SensorSystem/BP_SensorController.BP_SensorController_C" _returnvalue "AlwaysSpawn" "MultiplyWithRoot" 0 0))
      (Utilities|Array|Add (Variables|Default|GetPlatformComponentsShip) _returnvalue_4))
    (:then_2
      (bind _returnvalue_5 (Game|SpawnActorfromClass "/Game/Blueprints/Components/PSC/BP_PSC_Master.BP_PSC_Master_C" _returnvalue "AlwaysSpawn" "MultiplyWithRoot" 0 "NewEnumerator3" 0))
      (bind _output_get (Variables|Default|SetPSC _returnvalue_5))
      (Class|BPIPSC|SetPlatformFaction(Message) _output_get (Variables|Init|GetFaction))
      (Class|BPIPSC|AssignPlatform(Message) _output_get self)
      (bind _output_get_2 (Variables|Default|SetPlatformComponents (Utilities|Struct|MakeS_ShipChildComponents (Variables|Default|GetPlatformComponentsShip) 0 0 (Variables|Default|GetMissileComponents) 0)))
      (Class|BPIPSC|SetPlatformComponents(Message) _output_get _output_get_2)
      (Class|BPIPSC|InitializePSC(Message) _output_get))))

(event EventSetFactionType
  (params (SetFaction :type E_FriendFoe%20Enum :default "NewEnumerator0"))
  (bind _output_get (Variables|Init|SetFaction SetFaction))
  (Class|BPIPSC|SetPlatformFaction(Message) (Variables|Default|GetPSC) _output_get)
  (CallFunction|UpdatePlatformComponentsFaction _output_get))

(event EventSetTargetable
  (params (Targetable :type Boolean))
  (Variables|Default|SetTargetable Targetable))

(fn ConstructionScript)

(fn UpdatePlatformComponentsFaction
  (params (NewFaction :type E_FriendFoe%20Enum :default "NewEnumerator0"))
  (bind _platformcomponents (Variables|Default|GetPlatformComponents))
  (bind _platformcomponents_2 (Variables|Default|GetPlatformComponents))
  (Utilities|FlowControl|Sequence
    (:then_0
      (if (Utilities|Array|IsNotEmpty (.ship _platformcomponents_2))
        (for _array_element (.ship _platformcomponents)
          (Class|BPITargetable|SetFactionType(Message) _array_element NewFaction))))
    (:then_1
      (if (Utilities|Array|IsNotEmpty (.offensive _platformcomponents_2))
        (for _array_element_2 (.offensive _platformcomponents)
          (Class|BPITargetable|SetFactionType(Message) _array_element_2 NewFaction))))
    (:then_2
      (if (Utilities|Array|IsNotEmpty (.defensive _platformcomponents_2))
        (for _array_element_3 (.defensive _platformcomponents)
          (Class|BPITargetable|SetFactionType(Message) _array_element_3 NewFaction))))
    (:then_3
      (if (Utilities|Array|IsNotEmpty (.missiles _platformcomponents_2))
        (for _array_element_4 (.missiles _platformcomponents)
          (Class|BPITargetable|SetFactionType(Message) _array_element_4 NewFaction))))
    (:then_4
      (if (Utilities|Array|IsNotEmpty (.sensors _platformcomponents_2))
        (for _array_element_5 (.sensors _platformcomponents)
          (Class|BPITargetable|SetFactionType(Message) _array_element_5 NewFaction))))))

(fn ContactType
  (return "NewEnumerator0"))

(fn GetDefensiveWeapons
  (return 0))

(fn GetFactionType
  (return (Variables|Init|GetFaction)))

(fn GetMissileLaunchers
  (return (Variables|Default|GetMissileComponents)))

(fn GetOffensiveWeapons
  (return 0))

(fn GetPlatformComponents
  (return 0))

(fn GetPlatformFaction
  (return "NewEnumerator0"))

(fn GetPSCControllers
  (return 0 0))

(fn GetTargetable
  (return (Variables|Default|GetTargetable)))

(fn GetTargetableType
  (return "NewEnumerator1"))

(fn ObjectDetected
  (params (DetectedObjectHit_In :type Hit%20Result%20Structure) (SensorThatDetected_In :type Actor%20Component%20Object%20Reference))
  (return "" 0))