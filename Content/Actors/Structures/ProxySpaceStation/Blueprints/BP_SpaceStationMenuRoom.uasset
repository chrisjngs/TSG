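; Space station menu room actor that relays ship element changes through a ShipChangedPassthrough call.
; It also implements ContactType, which returns a fixed enum value, and an ObjectDetected function that does nothing.
; Tick, MoveCamera and ManualRotation are empty stubs; their hologram spin, timeline camera blend and right-mouse rotation logic remains in the graph but is disconnected.
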(event Custom|MoveCamera
  (params (CameraToMove :type Cine%20Camera%20Component%20Object%20Reference) (CurrentLocation :type Transform) (NewLocation :type Transform))
  ;[0.15 0.15 0.15 0.5] Move the camera from one location to a new one over the timeline curve
)

(event Custom|ManualRotation)

(event Custom|ChangedShipElement_Event
  (Default|CallShipChangedPassthrough))

(event EventTick
  (params (DeltaSeconds :type Float%20%28single-precision%29))
  ;[0.15 0.15 0.15 0.5] Rotate the hologram
)

(fn ConstructionScript)

(fn ContactType
  (return "NewEnumerator3"))

(fn ObjectDetected
  (params (DetectedObjectHit_In :type Hit%20Result%20Structure) (SensorThatDetected_In :type Actor%20Component%20Object%20Reference))
  (return "" 0))