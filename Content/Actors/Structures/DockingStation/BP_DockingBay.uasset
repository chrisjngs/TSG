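; BP_DockingBay is an interactable docking bay structure that docks an interactor's piloted platform if it supports customization mode.
; On interact, it passes the platform to the DockingZone child actor and its parent actor, then calls debug stop on the platform's PMS_AC component.
; It also handles ping highlights: an optional attached crosshair and a retriggerable delay, then a timeline fade that clears overlay materials.
; Interface functions report its contact and interact types.
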(event EventOutlineStart
  (params (TimeOfHighlight :type Float%20%28double-precision%29) (CrosshairComponent :type Widget%20Component%20Object%20Reference) (IncludeWidget :type Boolean) (DynamicMaterial :type Material%20Instance%20Dynamic%20Object%20Reference))
  ;[0.15 0.15 0.15 0.5] Ping highlight logic
  (if IncludeWidget
    (Variables|Default|SetCrosshair%20Component CrosshairComponent)
    (Transformation|AttachComponentToComponent CrosshairComponent (Variables|Default|GetDefaultSceneRoot) "None" "SnapToTarget" "KeepWorld" "KeepWorld" true))
  (Utilities|FlowControl|RetriggerableDelay TimeOfHighlight)
  (for _array_element (Actor|GetComponentsByClass "/Script/Engine.MeshComponent")
    (bind _fadeouttrack (Timeline|Timeline PlayFromStart)
      (:Update
        (Rendering|Material|SetScalarParameterValue DynamicMaterial "FadeOut" _fadeouttrack :!class /Script/Engine.MaterialInstanceDynamic))
      (:Finished
        (Rendering|Material|SetOverlayMaterial _array_element 0 :!class /Script/Engine.MeshComponent)
        (if IncludeWidget
          (Utilities|IsValid (Variables|Default|GetCrosshair%20Component)
            (:Is%20Valid
              (Components|DestroyComponent (Variables|Default|GetCrosshair%20Component)))
            (:Is%20Not%20Valid
              (Development|PrintString "The given widget was not valid"))))))))

(event EventInteract
  (params (Interactor :type Actor%20Object%20Reference))
  (bind _pilotedplatform (Class|BPIPlayer|GetPilotedPlatform(Message) Interactor))
  (if (Utilities|DoesObjectImplementInterface _pilotedplatform "/Game/Blueprints/Components/CustomizationSystem/BPI_CustomizationMode.BPI_CustomizationMode_C")
    (Class|BPIDocking|SetDockedActor(Message) (Variables|/Script/Engine.ChildActorComponent|GetChildActor (Variables|Default|GetDockingZone)) _pilotedplatform)
    (Class|BPIDocking|SetDockedActor(Message) (Actor|GetParentActor) _pilotedplatform)
    (Default|EventDebugStop (Actor|GetComponentbyClass _pilotedplatform "/Game/Blueprints/Components/PMS_PlatformMovementSystem/PMS_AC.PMS_AC_C"))
    (else
      (Development|PrintString "No customization interface detected"))))

(fn ConstructionScript)

(fn ContactType
  (return "NewEnumerator0"))

(fn GetInteractType
  (return (Variables|Default|GetInteractType)))

(fn ObjectDetected
  (params (DetectedObjectHit_In :type Hit%20Result%20Structure) (SensorThatDetected_In :type Actor%20Component%20Object%20Reference))
  (return "" 0))