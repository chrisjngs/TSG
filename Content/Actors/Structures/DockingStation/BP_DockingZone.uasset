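; BP_DockingZone is a docking area actor for docking station structures that keeps a reference to the actor docked in it.
; Its construction script sizes the DockingArea box from DockingRange, and a setter and getter expose DockedActor.
; Interactions are forwarded to the parent actor, so the zone acts as a proxy for its owning actor.
; UpdateDockedActor, GetCameraLocations and GetHologramLocation are empty stubs, with no overlap detection in these graphs.
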(event EventInteract
  (params (Interactor :type Actor%20Object%20Reference))
  (Class|BPIInteract|Interact(Message) (Actor|GetParentActor) Interactor))

(event EventSetDockedActor
  (params (Docked :type Actor%20Object%20Reference))
  ;[0.15 0.15 0.15 0.5] This gets the docked actor and stores it for later use
  (Variables|Docking|Actor|SetDockedActor Docked))

(event EventUpdateDockedActor
  ;[0.15 0.15 0.15 0.5] This should be used to pass data to the docked actor. Such as tell the actor what components have been changed.
)

(fn ConstructionScript
  (Components|Box|SetBoxExtent (Variables|Docking|Zones|GetDockingArea) (Variables|Docking|Zones|GetDockingRange) true))

(fn GetCameraLocations
  (return 0 0))

(fn GetDockedActor
  (return (Variables|Docking|Actor|GetDockedActor)))

(fn GetHologramLocation
  (return 0))

(fn GetInteractType
  (return "NewEnumerator0"))