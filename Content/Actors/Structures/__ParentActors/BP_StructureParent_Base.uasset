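; Base parent Blueprint for structure actors, exposing a common set of platform query functions.
; Getters for controlled camera, weapons, missile launchers, platform components and PSC controllers are empty stubs, while the faction getter returns a fixed enum entry.
; GetScannedComponents is the only getter that references a component, returning StructureChildActor as its ParentActor output.
; The event graph and construction script contain no logic.
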(event EventBeginPlay)

(event Collision|EventActorBeginOverlap
  (params (OtherActor :type Actor%20Object%20Reference)))

(event EventTick
  (params (DeltaSeconds :type Float%20%28single-precision%29)))

(fn ConstructionScript)

(fn GetControlledCamera
  (return 0 0))

(fn GetDefensiveWeapons
  (return 0))

(fn GetMissileLaunchers
  (return 0))

(fn GetOffensiveWeapons
  (return 0))

(fn GetPlatformComponents
  (return 0))

(fn GetPlatformFaction
  (return "NewEnumerator0"))

(fn GetPSCControllers
  (return 0 0))

(fn GetScannedComponents
  (return (Variables|Default|GetStructure_ChildActor) 0))