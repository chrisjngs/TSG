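; Proxy ship pawn that flies by physics force, with thruster visuals, active sensor ping and a customization interface.
; Tick applies forward acceleration while accelerating and binds docking to zero it; construction adds a child actor at a weapon socket.
; Positive velocity on any axis triggers projectile-path prediction, shown only as debug drawing.
; The spline-mesh ribbon logic is unconnected in the event graph and duplicated in uncalled functions.
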(event Custom|EnableThrusters
  (bind _spaceshipenginethrust_blockout (Variables|Default|GetSpaceShipEngineThrust_Blockout))
  ;[0.15 0.15 0.15 0.5] Turn on engine thruster effect
  (if (Variables|Default|GetShipAccelerating)
    (Rendering|SetVisibility _spaceshipenginethrust_blockout true false)
    (else
      (Rendering|SetVisibility _spaceshipenginethrust_blockout false false))))

(event Custom|CameraLookat
  (bind _springarm (Variables|Default|GetSpringArm))
  ;[0.15 0.15 0.15 0.5] Comment
  (if (Variables|Default|GetPawnControlRotation)
    (Variables|/Script/Engine.SpringArmComponent|SetbUsePawnControlRotation _springarm true)
    (else
      (Variables|/Script/Engine.SpringArmComponent|SetbUsePawnControlRotation _springarm false))))

(event Custom|PredictiveRibbon
  ;[0.15 0.04468 0.09067 0.5] Predictive Ribbon
  ;;[0.15 0.15 0.15 0.5] Get all of the predicted points based on the current location and velocity
  (PreditctiveRibbon|ClearSplinePoints)
  (Utilities|Array|Clear (Variables|PredictiveRibbon|GetPredictedPoints))
  (bind _predictresult (Class|GameplayStatics|BlueprintPredictProjectilePathAdvanced (Utilities|Struct|MakePredictProjectilePathParams (Variables|Default|GetShipLocation) (Variables|Default|GetCurrentVelocity) false 5e+01 5.0 true "ECC_WorldStatic" "ObjectTypeQuery1" 0 2.0 1.0 "ForOneFrame"))))

(event Custom|ActivePing
  (bind _self self)
  ;[0.15 0.15 0.15 0.5] Active Ping
  ;;[0.15 0.15 0.15 0.5] Send out the active ping and get any returns
  (Default|SendPing (Variables|Default|GetBP_Ping_AC) (Variables|Pinging|GetPingRadius) _self (Variables|Default|GetSpaceShip_Blockout) _self))

(event Custom|ShipDocked
  ;[0.15 0.15 0.15 0.5] Move with Force
  (Variables|Default|SetCurrentAcceleration 0.0))

(event EventTick
  (params (DeltaSeconds :type Float%20%28single-precision%29))
  (bind _returnvalue (Transformation|GetActorTransform))
  (bind _currentacceleration (Variables|Default|GetCurrentAcceleration))
  ;[0.15 0.15 0.15 0.5] Move with Force
  (Variables|Default|SetDeltaSeconds (+ DeltaSeconds (Variables|Default|GetDeltaSeconds)))
  (Variables|Default|SetCurrentVelocity (Transformation|GetVelocity))
  (Variables|Default|SetShipLocation (Transformation|GetActorLocation))
  (if (Math|Boolean|ORBoolean (> (.x (Variables|Default|GetCurrentVelocity)) 0.0) (> (.y (Variables|Default|GetCurrentVelocity)) 0.0) (> (.z (Variables|Default|GetCurrentVelocity)) 0.0))
    (CallFunction|PredictiveRibbon))
  (if (Variables|Default|GetShipAccelerating)
    (Transformation|SetWorldLocationAndRotation (Variables|Default|GetSpaceShipEngineThrust_Blockout) (.location _returnvalue) (.rotation _returnvalue) false false)
    (Transformation|SetWorldScale3D (Variables|Default|GetSpaceShipEngineThrust_Blockout) (Math|Vector|MakeVector (Math|Float|Clamp(Float) _currentacceleration) 1.0 1.0))
    (Physics|AddForce (Variables|Default|GetSpaceShip_Blockout) (* _currentacceleration (Transformation|GetActorForwardVector) 1e+03) "None" true)
    (EventDispatchers|BindEventtoDocked (Variables|Default|GetBP_Customizable_AC) (delegate Custom|ShipDocked))
    (else
      (Variables|Default|SetShipAccelerating false)
      (CallFunction|EnableThrusters))))

(event EventCustomize
  (params (Actor%20Being%20Customized :type Actor%20Object%20Reference) (Actor%20Interacted%20With :type Actor%20Object%20Reference))
  ;[0.15 0.15 0.15 0.5] Call events to enter customization mode for the ship
  ;;[0.15 0.15 0.15 0.5] Use the Interface to call the event dispatcher
  (Default|CallCustomizeShip Actor%20Being%20Customized Actor%20Interacted%20With))

(fn ConstructionScript
  (bind _spaceship_blockout (Variables|Default|GetSpaceShip_Blockout))
  (bind _returnvalue (Transformation|GetSocketTransform _spaceship_blockout "WeaponSystem_TopLeft" "RTS_World"))
  (bind (_location _rotation _scale) (Math|Transform|BreakTransform _returnvalue))
  (AddComponent|AddChildActorComponent true (Math|Transform|MakeTransform _location _rotation (* _scale 0.5))))

(fn CalculateVelocity
  (params (Starting%20location :type Vector))
  (bind _output_get (Variables|Default|SetShipLocation Starting%20location))
  (Development|PrintString (Utilities|String|ToString(Vector) (Variables|/Script/Engine.MovementComponent|GetVelocity (Variables|Default|GetFloatingPawnMovement))))
  (return "0, 0, 0"))

(fn ClearSplinePoints
  (bind _ribbonmeshes (Variables|PredictiveRibbon|GetRibbonMeshes))
  (Components|DestroyComponent _ribbonmeshes)
  (Utilities|Array|Clear _ribbonmeshes)
  (Spline|ClearSplinePoints (Variables|Default|GetSplineRibbon) true))

(fn AddSplineMesh
  (bind _splineribbon (Variables|Default|GetSplineRibbon))
  ;[0.15 0.15 0.15 0.5] Add mesh components and set tangents of start and end points
  (for _index (range 0 (- (Spline|GetNumberOfSplinePoints (Variables|Default|GetSplineRibbon)) 2))
    (bind _returnvalue (AddComponent|AddSplineMeshComponent true))
    (Utilities|Array|Add (Variables|PredictiveRibbon|GetRibbonMeshes) _returnvalue)
    (SplineMesh|SetStartandEnd _returnvalue (.Location (Spline|GetLocationandTangentatSplinePoint _splineribbon _index "Local")) (.Tangent (Spline|GetLocationandTangentatSplinePoint _splineribbon _index "Local")) (.Location (Spline|GetLocationandTangentatSplinePoint _splineribbon (+ _index 1) "Local")) (.Tangent (Spline|GetLocationandTangentatSplinePoint _splineribbon (+ _index 1) "Local")) true :!class /Script/Engine.SplineMeshComponent)))

(fn CalculateFuturePositions
  (params (Array :type Array%20of%20Predict%20Projectile%20Path%20Point%20Data%20Structures))
  ;[0.15 0.15 0.15 0.5] x sub0 + v subz0 * t = 1/2asubxt^2 Getting predicted location based on change of angle and acceleration
  (for _array_element Array
    (Spline|AddSplinePoint (Variables|Default|GetSplineRibbon) (+ (+ (.Location (Utilities|Struct|BreakPredictProjectilePathPointData _array_element)) (* (.Velocity (Utilities|Struct|BreakPredictProjectilePathPointData _array_element)) (.Time (Utilities|Struct|BreakPredictProjectilePathPointData _array_element)))) (* (* (Variables|Default|GetCurrentAcceleration) (* (.Time (Utilities|Struct|BreakPredictProjectilePathPointData _array_element)) (.Time (Utilities|Struct|BreakPredictProjectilePathPointData _array_element)))) 0.5)) "Local" true))
  (return))

(fn GetPositionsBasedonVelocity
  (bind _predictedpoints (Variables|PredictiveRibbon|GetPredictedPoints))
  ;[0.15 0.15 0.15 0.5] Get all of the predicted points based on the current location and velocity
  (PreditctiveRibbon|ClearSplinePoints)
  (Utilities|Array|Clear (Variables|PredictiveRibbon|GetPredictedPoints))
  (bind _predictresult (Class|GameplayStatics|BlueprintPredictProjectilePathAdvanced (Utilities|Struct|MakePredictProjectilePathParams (Variables|Default|GetShipLocation) (Variables|Default|GetCurrentVelocity) false 4.0 5.0 true "ECC_WorldStatic" "ObjectTypeQuery1" 0 2.0 1.0)))
  (for _array_element (.PathData (Utilities|Struct|BreakPredictProjectilePathResult _predictresult))
    (Utilities|Array|Add _predictedpoints _array_element))
  (return _predictedpoints))

(fn ComponentType
  (return "NewEnumerator0"))

(fn ContactType
  (return "NewEnumerator0"))

(fn GetTotalReputationCost
  (return 0))

(fn ObjectDetected
  (params (DetectedObjectHit_In :type Hit%20Result%20Structure) (SensorThatDetected_In :type Actor%20Component%20Object%20Reference))
  (return "" 0))