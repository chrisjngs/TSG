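; BP_ProxyEngine is the proxy ship's engine Blueprint, meant to provide physics thrust, a thruster effect and pitch, yaw and roll controls.
; While ShipAccelerating is set, Tick aligns and scales the thrust component by CurrentAcceleration and applies forward force, otherwise EnableThrusters hides it.
; BeginPlay and all input events are empty.
; Mapping-context setup, acceleration changes and quaternion rotation logic exist only as disconnected nodes.
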(event Custom|EnableThrusters
  (bind _proxyengine_thrust (Variables|Default|GetProxyEngine_Thrust))
  ;[0.15 0.15 0.15 0.5] Turn on engine thruster effect
  (if (Variables|Default|GetShipAccelerating)
    (Rendering|SetVisibility _proxyengine_thrust true false)
    (else
      (Rendering|SetVisibility _proxyengine_thrust false false))))

(event Input|EnhancedActionEvents|EnhancedInputActionIA_Acceleration
  (params (ActionValue :type Float%20%28double-precision%29) (ElapsedSeconds :type Float%20%28double-precision%29) (TriggeredSeconds :type Float%20%28double-precision%29) (InputAction :type Input%20Action%20Object%20Reference :default "/Game/Inputs/Movement/IA_Acceleration.IA_Acceleration"))
  ;[0.15 0.15 0.15 0.5] Acceleration and Deceleration
)

(event Input|EnhancedActionEvents|EnhancedInputActionIA_Decceleration
  (params (ActionValue :type Float%20%28double-precision%29) (ElapsedSeconds :type Float%20%28double-precision%29) (TriggeredSeconds :type Float%20%28double-precision%29) (InputAction :type Input%20Action%20Object%20Reference :default "/Game/Inputs/Movement/IA_Decceleration.IA_Decceleration"))
  ;[0.15 0.15 0.15 0.5] Acceleration and Deceleration
)

(event Input|EnhancedActionEvents|EnhancedInputActionIA_CancelMomentum
  (params (ActionValue :type Boolean) (ElapsedSeconds :type Float%20%28double-precision%29) (TriggeredSeconds :type Float%20%28double-precision%29) (InputAction :type Input%20Action%20Object%20Reference :default "/Game/Inputs/Movement/IA_CancelMomentum.IA_CancelMomentum")))

(event Input|EnhancedActionEvents|EnhancedInputActionIA_PitchUp
  (params (ActionValue :type Float%20%28double-precision%29) (ElapsedSeconds :type Float%20%28double-precision%29) (TriggeredSeconds :type Float%20%28double-precision%29) (InputAction :type Input%20Action%20Object%20Reference :default "/Game/Inputs/Movement/IA_PitchUp.IA_PitchUp"))
  ;[0.15 0.15 0.15 0.5] Pitch Controls
)

(event Input|EnhancedActionEvents|EnhancedInputActionIA_YawRight
  (params (ActionValue :type Float%20%28double-precision%29) (ElapsedSeconds :type Float%20%28double-precision%29) (TriggeredSeconds :type Float%20%28double-precision%29) (InputAction :type Input%20Action%20Object%20Reference :default "/Game/Inputs/Movement/IA_YawRight.IA_YawRight"))
  ;[0.15 0.15 0.15 0.5] Yaw controls
)

(event Input|EnhancedActionEvents|EnhancedInputActionIA_RollRight
  (params (ActionValue :type Float%20%28double-precision%29) (ElapsedSeconds :type Float%20%28double-precision%29) (TriggeredSeconds :type Float%20%28double-precision%29) (InputAction :type Input%20Action%20Object%20Reference :default "/Game/Inputs/Movement/IA_RollRight.IA_RollRight"))
  ;[0.15 0.15 0.15 0.5] Roll controls
)

(event Input|EnhancedActionEvents|EnhancedInputActionIA_PitchDown
  (params (ActionValue :type Float%20%28double-precision%29) (ElapsedSeconds :type Float%20%28double-precision%29) (TriggeredSeconds :type Float%20%28double-precision%29) (InputAction :type Input%20Action%20Object%20Reference :default "/Game/Inputs/Movement/IA_PitchDown.IA_PitchDown"))
  ;[0.15 0.15 0.15 0.5] Pitch Controls
)

(event Input|EnhancedActionEvents|EnhancedInputActionIA_YawLeft
  (params (ActionValue :type Float%20%28double-precision%29) (ElapsedSeconds :type Float%20%28double-precision%29) (TriggeredSeconds :type Float%20%28double-precision%29) (InputAction :type Input%20Action%20Object%20Reference :default "/Game/Inputs/Movement/IA_YawLeft.IA_YawLeft"))
  ;[0.15 0.15 0.15 0.5] Yaw controls
)

(event Input|EnhancedActionEvents|EnhancedInputActionIA_RollLeft
  (params (ActionValue :type Float%20%28double-precision%29) (ElapsedSeconds :type Float%20%28double-precision%29) (TriggeredSeconds :type Float%20%28double-precision%29) (InputAction :type Input%20Action%20Object%20Reference :default "/Game/Inputs/Movement/IA_RollLeft.IA_RollLeft"))
  ;[0.15 0.15 0.15 0.5] Roll controls
)

(event EventBeginPlay
  ;[0.15 0.15 0.15 0.5] Enable the use of the mapping controller
)

(event EventTick
  (params (DeltaSeconds :type Float%20%28single-precision%29))
  (bind _returnvalue (Transformation|GetActorTransform))
  (bind _currentacceleration (Variables|Default|GetCurrentAcceleration))
  ;[0.15 0.15 0.15 0.5] Move with Force
  (if (Variables|Default|GetShipAccelerating)
    (Transformation|SetWorldLocationAndRotation (Variables|Default|GetProxyEngine_Thrust) (.location _returnvalue) (.rotation _returnvalue) false false)
    (Transformation|SetWorldScale3D (Variables|Default|GetProxyEngine_Thrust) (Math|Vector|MakeVector (Math|Float|Clamp(Float) _currentacceleration) 1.0 1.0))
    (Physics|AddForce (Variables|Default|GetProxyEngine) (* _currentacceleration (Transformation|GetActorForwardVector) 1e+03) "None" true)
    (else
      (Variables|Default|SetShipAccelerating false)
      (CallFunction|EnableThrusters))))

(fn ConstructionScript)

(fn CalculateVelocity
  (params (Starting%20location :type Vector))
  (bind _output_get (Variables|Default|SetShipLocation Starting%20location)))