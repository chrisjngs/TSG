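; Test ship actor for physics-based movement, with a prototype predicted-path ribbon.
; Tick applies forward acceleration force and scales the thruster effect while accelerating, but only when no velocity component is positive.
; PredictiveRibbon turns projectile prediction plus a kinematic offset into spline points and spline meshes, but its call is unwired and its clearing function is empty.
; Separate events toggle thruster visibility and spring arm control rotation.
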(event Custom|CameraLookat
  (bind _springarm (Variables|Default|GetSpringArm))
  ;[0.15 0.15 0.15 0.5] Comment
  (if (Variables|Default|GetPawnControlRotation)
    (Variables|/Script/Engine.SpringArmComponent|SetbUsePawnControlRotation _springarm true)
    (else
      (Variables|/Script/Engine.SpringArmComponent|SetbUsePawnControlRotation _springarm false))))

(event Custom|EnableThrusters
  (bind _thrusters (Variables|Default|GetThrusters))
  ;[0.15 0.15 0.15 0.5] Turn on engine thruster effect
  (if (Variables|Default|GetShipAccelerating)
    (Rendering|SetVisibility _thrusters true false)
    (else
      (Rendering|SetVisibility _thrusters false false))))

(event Custom|PredictiveRibbon
  (bind _splineribbon (Variables|Default|GetSplineRibbon))
  ;[0.15 0.04468 0.09067 0.5] Predictive Ribbon
  ;;[0.15 0.15 0.15 0.5] Get all of the predicted points based on the current location and velocity
  (CallFunction|ClearSplinePoints)
  (Utilities|Array|Clear (Variables|Default|GetPredictedPoints))
  (bind _predictresult (Class|GameplayStatics|BlueprintPredictProjectilePathAdvanced (Utilities|Struct|MakePredictProjectilePathParams (Variables|Default|GetShipLocation) (Variables|Default|GetCurrentVelocity) false 4.0 5.0 true "ECC_WorldStatic" "ObjectTypeQuery1" 0 2.0 1.0)))
  (for _array_element (.PathData (Utilities|Struct|BreakPredictProjectilePathResult _predictresult))
    (Utilities|Array|Add (Variables|Default|GetPredictedPoints) _array_element))
  ;;[0.15 0.15 0.15 0.5] x sub0 + v subz0 * t = 1/2asubxt^2 Getting predicted location based on change of angle and acceleration
  (for _array_element_2 (Variables|Default|GetPredictedPoints)
    (Spline|AddSplinePoint (Variables|Default|GetSplineRibbon) (+ (+ (.Location (Utilities|Struct|BreakPredictProjectilePathPointData _array_element_2)) (* (.Velocity (Utilities|Struct|BreakPredictProjectilePathPointData _array_element_2)) (.Time (Utilities|Struct|BreakPredictProjectilePathPointData _array_element_2)))) (* (* (Variables|Default|GetCurrentAcceleration) (* (.Time (Utilities|Struct|BreakPredictProjectilePathPointData _array_element_2)) (.Time (Utilities|Struct|BreakPredictProjectilePathPointData _array_element_2)))) 0.5)) "Local" true))
  ;;[0.15 0.15 0.15 0.5] Add mesh components and set tangents of start and end points
  (for _index (range 0 (- (Spline|GetNumberOfSplinePoints (Variables|Default|GetSplineRibbon)) 2))
    (bind _returnvalue (AddComponent|AddSplineMeshComponent true))
    (Utilities|Array|Add (Variables|Default|GetRibbonMeshes) _returnvalue)
    (SplineMesh|SetStartandEnd _returnvalue (.Location (Spline|GetLocationandTangentatSplinePoint _splineribbon _index "Local")) (.Tangent (Spline|GetLocationandTangentatSplinePoint _splineribbon _index "Local")) (.Location (Spline|GetLocationandTangentatSplinePoint _splineribbon (+ _index 1) "Local")) (.Tangent (Spline|GetLocationandTangentatSplinePoint _splineribbon (+ _index 1) "Local")) true :!class /Script/Engine.SplineMeshComponent)))

(event EventTick
  (params (DeltaSeconds :type Float%20%28single-precision%29))
  (bind _returnvalue (Transformation|GetActorTransform))
  (bind _currentacceleration (Variables|Default|GetCurrentAcceleration))
  ;[0.15 0.15 0.15 0.5] Move with Force
  (Variables|Default|Settime (+ DeltaSeconds (Variables|Default|Gettime)))
  (Variables|Default|SetCurrentVelocity (Transformation|GetVelocity))
  (Variables|Default|SetShipLocation (Transformation|GetActorLocation))
  (if (not (Math|Boolean|ORBoolean (> (.x (Variables|Default|GetCurrentVelocity)) 0.0) (> (.y (Variables|Default|GetCurrentVelocity)) 0.0) (> (.z (Variables|Default|GetCurrentVelocity)) 0.0)))
    (if (Variables|Default|GetShipAccelerating)
      (Transformation|SetWorldLocationAndRotation (Variables|Default|GetThrusters) (.location _returnvalue) (.rotation _returnvalue) false false)
      (Transformation|SetWorldScale3D (Variables|Default|GetThrusters) (Math|Vector|MakeVector (Math|Float|Clamp(Float) _currentacceleration) 1.0 1.0))
      (Physics|AddForce (Variables|Default|GetSpaceship) (* _currentacceleration (Transformation|GetActorForwardVector) 1e+03) "None" true)
      (else
        (Variables|Default|SetShipAccelerating false)
        (CallFunction|EnableThrusters)))))

(fn ConstructionScript)

(fn ClearSplinePoints)