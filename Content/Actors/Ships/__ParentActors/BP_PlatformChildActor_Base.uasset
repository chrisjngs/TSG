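; BP_PlatformChildActor_Base is a parent Blueprint for platform actors among the game's ships, providing shared targeting, faction and cost data.
; Its construction script applies ShipRenderMesh to ShipComponent.
; Events set the targetable state and faction, which getters expose alongside platform cost and pause-menu camera location.
; It always reports zero base rotation and one fixed targetable type.
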(event EventSetTargetable
  (params (Targetable :type Boolean))
  (Variables|Default|SetTargetable Targetable))

(event EventSetFactionType
  (params (SetFaction :type E_FriendFoe%20Enum :default "NewEnumerator0"))
  (Variables|Default|SetSet%20Faction SetFaction))

(fn ConstructionScript
  (Components|StaticMesh|SetStaticMesh (Variables|Default|GetShipComponent) (Variables|Default|GetShipRenderMesh)))

(fn GetFactionType
  (return (Variables|Default|GetSet%20Faction)))

(fn GetPauseCameraLocation
  (return (Variables|Default|GetPauseMenu_CameraLocation)))

(fn GetPlatformCost
  (return (Variables|Default|GetPlatformCost)))

(fn GetShipBaseRotation
  (return "0, 0, 0"))

(fn GetTargetable
  (return (Variables|Default|GetTargetable)))

(fn GetTargetableType
  (return "NewEnumerator0"))