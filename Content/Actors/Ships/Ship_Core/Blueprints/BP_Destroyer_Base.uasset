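; Base Blueprint for Destroyer-class ships, configured entirely in the Construction Script, with an empty event graph.
; It fills the CoreComponents struct with class data and with slot counts and anchors for weapon, point defense, sensor array and missile systems.
; Slots are discovered by scene component tag, so the layout follows the placed components.
; Only weapon slots get a child actor component, added at each anchor's relative transform.
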(event EventBeginPlay)

(event Collision|EventActorBeginOverlap
  (params (OtherActor :type Actor%20Object%20Reference)))

(event EventTick
  (params (DeltaSeconds :type Float%20%28single-precision%29)))

(fn ConstructionScript
  (bind _returnvalue (Actor|GetComponentsbyTag "/Script/Engine.SceneComponent" "MissileSystemSlot"))
  (bind _returnvalue_2 (Actor|GetComponentsbyTag "/Script/Engine.SceneComponent" "WeaponSystemSlot"))
  (bind _returnvalue_3 (Actor|GetComponentsbyTag "/Script/Engine.SceneComponent" "PointDefenseSystemSlot"))
  (bind _returnvalue_4 (Actor|GetComponentsbyTag "/Script/Engine.SceneComponent" "SensorArraySlot"))
  (bind _output_get (Variables|Default|SetCoreComponents (Utilities|Struct|MakeShipType_CoreComponents_Struct "Destroyer Class" 6 "NewEnumerator0" (Utilities|Array|Length _returnvalue_2) _returnvalue_2 (Utilities|Array|Length _returnvalue_3) _returnvalue_3 (Utilities|Array|Length _returnvalue_4) _returnvalue_4 (Utilities|Array|Length _returnvalue) _returnvalue "NewEnumerator1" "NewEnumerator1" 0)))
  (for _index (range 0 (- (.weaponsystemslots _output_get) 1))
    (AddComponent|AddChildActorComponent false (Transformation|GetRelativeTransform (Utilities|Array|Get(acopy) (.weaponsystemanchorpoints _output_get) _index)))))