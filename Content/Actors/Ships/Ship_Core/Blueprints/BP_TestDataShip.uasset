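; BP_TestDataShip is a test ship actor that builds itself from a data table row in the Construction Script.
; It finds the row whose PlatformName matches ShipName and spawns its PlatformBase as a child actor.
; Weapons, silos and sensors become child actors of their data asset's WeaponClass, placed using the relative transform of base components tagged with their attachment point.
; The capsule is then resized from the ship component's bounds origin.
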(fn ConstructionScript
  (CallFunction|AssemblefromData)
  (Components|Capsule|SetCapsuleSize (Variables|Default|GetCapsule) (Math|Vector|VectorLength (* (.Origin (Collision|GetComponentBounds (Variables|Default|GetShipComponent))) 0.02)) 0.5 true))

(fn AssemblefromData
  ;[0.15 0.15 0.15 0.5] Get the row that matches the ship name
  (bind (_tablerow _shipdatafound) (CallFunction|GetRowforShipinTable (Utilities|ResolveSoftReference (Variables|Default|GetTable)) (Variables|Default|GetShipName)))
  (Variables|Default|SetShipTableRow _tablerow)
  (if _shipdatafound
    ;[0.15 0.15 0.15 0.5] Add the base ship component
    (bind _returnvalue (AddComponent|AddChildActorComponent true (Transformation|GetActorTransform)))
    (Variables|Default|SetShipComponent _returnvalue)
    (ChildActorComponent|SetChildActorClass _returnvalue (Utilities|ResolveSoftReference (.PlatformBase (Utilities|Struct|BreakS_ShipConfigurations (Variables|Default|GetShipTableRow)))))
    ;[0.15 0.15 0.15 0.5] Attach Weapon Components
    (CallFunction|AttachComponentsfromData (.OffensiveWeapons (Utilities|Struct|BreakS_ShipConfigurations (Variables|Default|GetShipTableRow))) (Components|GetChildrenComponents _returnvalue true)) ; Offensive Weapons
    (CallFunction|AttachComponentsfromData (.DefensiveWeapons (Utilities|Struct|BreakS_ShipConfigurations (Variables|Default|GetShipTableRow))) (Components|GetChildrenComponents _returnvalue true)) ; Defensive Weapons
    (CallFunction|AttachComponentsfromData (.MissileSilos (Utilities|Struct|BreakS_ShipConfigurations (Variables|Default|GetShipTableRow))) (Components|GetChildrenComponents _returnvalue true)) ; Missile Silos
    (CallFunction|AttachComponentsfromData (.SensorSystems (Utilities|Struct|BreakS_ShipConfigurations (Variables|Default|GetShipTableRow))) (Components|GetChildrenComponents _returnvalue true)) ; Sensors
  ))

(fn GetRowforShipinTable
  (params (DataTable :type Data%20Table%20Soft%20Object%20Reference) (ShipName :type Name))
  (bind _output (Utilities|ResolveSoftReference DataTable))
  (bind _outrownames (DataTable|GetDataTableRowNames _output))
  (bind _array_element (Utilities|Array|ForEachLoopwithBreak _outrownames :!label _label)
    (:LoopBody
      (bind _returnvalue (Utilities|GetDataTableRow _output _array_element)
        (:then
          (Development|PrintString (Utilities|String|ToString(Name) (.PlatformName (Utilities|Struct|BreakS_ShipConfigurations _returnvalue))) true true "(R=0.000000,G=0.660000,B=1.000000,A=1.000000)" 3e+01)
          (if (== (.PlatformName (Utilities|Struct|BreakS_ShipConfigurations _returnvalue)) ShipName)
            (Utilities|FlowControl|Sequence
              (:then_0
                (bind _output_get (LocalVariables|SetShipFound true))
                (return _returnvalue _output_get))
              (:then_1
                (goto _label Break)))))))
    (:Completed
      (if (not (LocalVariables|GetShipDataFound))
        (Development|PrintString (Utilities|String|ToString(Text) (Utilities|Text|FormatText "No ship was found in the data table \"{DataTable}\" matching the name {ShipName}" _output ShipName)))))))

(fn AttachComponentsfromData
  (params (ComponentArray :type Array%20of%20S%20Ship%20Component%20Structures) (SceneComponents :type Array%20of%20Scene%20Component%20Object%20References))
  (if (Utilities|Array|IsNotEmpty ComponentArray)
    (for _array_element ComponentArray
      (bind _array_element_2 (Utilities|Array|ForEachLoopwithBreak SceneComponents :!label _label)
        (:LoopBody
          (if (Components|ComponentHasTag _array_element_2 (.AttachmentPoint (Utilities|Struct|BreakS_ShipComponent _array_element)))
            (bind _asbp_weapon_system_base_pda (Utilities|Casting|CastToBP_WeaponSystem_Base_PDA (.CurrentDataAsset (Utilities|Struct|BreakS_ShipComponent _array_element))))
            (Utilities|FlowControl|Sequence
              (:then_0
                (goto _label Break))
              (:then_1
                (bind _returnvalue (AddComponent|AddChildActorComponent false (Transformation|GetRelativeTransform _array_element_2)))
                (ChildActorComponent|SetChildActorClass _returnvalue (Utilities|ResolveSoftReference (Variables|/Game/Actors/WeaponSystems/__DataAssets/BP_WeaponSystem_Base_PDA.BP_WeaponSystem_Base_PDA_C|GetWeaponClass _asbp_weapon_system_base_pda))))))))))
  (return))