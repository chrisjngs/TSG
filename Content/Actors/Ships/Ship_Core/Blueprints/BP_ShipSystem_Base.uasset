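; Base ship actor that builds a modular ship from saved configuration or a data table row, then moves it by physics force.
; Construction spawns the hull and tag-matched weapon child actors from data assets, then saves the configuration.
; Update functions swap child actor classes by matching saved attachment points.
; Tick pushes the collision capsule forward by current acceleration, which docking zeroes; events handle active sensor pings and customization.
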(event Custom|ActivePing
  (bind _self self)
  ;[0.15 0.15 0.15 0.5] Active Ping
  ;;[0.15 0.15 0.15 0.5] Send out the active ping and get any returns
  (Default|SendPing (Variables|Default|GetBP_Ping_AC) (Variables|Default|GetPingRadius) _self 0 _self))

(event Custom|ShipDocked
  ;[0.15 0.15 0.15 0.5] Move with Force
  (Variables|Default|SetCurrentAcceleration 0.0))

(event EventTick
  (params (DeltaSeconds :type Float%20%28single-precision%29))
  (bind _currentacceleration (Variables|Default|GetCurrentAcceleration))
  ;[0.15 0.15 0.15 0.5] Move with Force
  (Variables|Default|SetDeltaSeconds (+ DeltaSeconds (Variables|Default|GetDeltaSeconds)))
  (Variables|Default|SetCurrentVelocity (Transformation|GetVelocity))
  (Variables|Default|SetShipLocation (Transformation|GetActorLocation))
  (if (Math|Boolean|ORBoolean (> (.x (Variables|Default|GetCurrentVelocity)) 0.0) (> (.y (Variables|Default|GetCurrentVelocity)) 0.0) (> (.z (Variables|Default|GetCurrentVelocity)) 0.0))
    (if (> _currentacceleration 0.1)
      (Variables|Default|SetShipAccelerating true)
      (else
        (Variables|Default|SetShipAccelerating false :!label _label)))
    (else
      (goto _label)))
  (Physics|AddForce (Variables|Default|GetShipCollisionCapsule) (* _currentacceleration (Math|Vector|GetForwardVector (Variables|Default|GetShipComponent)) 1e+03) "None" true)
  (EventDispatchers|BindEventtoDocked (Variables|Default|GetBP_Customizable_AC) (delegate Custom|ShipDocked)))

(event EventCustomize
  (params (Actor%20Being%20Customized :type Actor%20Object%20Reference) (Actor%20Interacted%20With :type Actor%20Object%20Reference))
  ;[0.15 0.15 0.15 0.5] Call events to enter customization mode for the ship
  ;;[0.15 0.15 0.15 0.5] Use the Interface to call the event dispatcher
  (Default|CallCustomizeShip Actor%20Being%20Customized Actor%20Interacted%20With))

(fn ConstructionScript
  (bind _returnvalue (Game|GetGameInstance))
  (Variables|Default|SetWeaponDataAssets (CallFunction|GetWeaponDataTable))
  (bind _savedata (Class|BPISaveGame|GetGameData(Message) _returnvalue))
  (if (!= (.shipname (Variables|/Game/Blueprints/SaveLoadSystem/BP_PlayerShipSaveData.BP_PlayerShipSaveData_C|GetShipConfiguration _savedata)) "")
    (Development|PrintString "Constructing from save data" false)
    (Class|BPISaveGame|LoadGameData(Message) _returnvalue false "PlayerShip")
    (ShipCreation|AssemblefromData true _savedata)
    (else
      (Development|PrintString "Constructing from data table" false)
      (ShipCreation|AssemblefromData false)))
  (Components|Capsule|SetCapsuleSize (Variables|Default|GetShipCollisionCapsule) (Math|Vector|VectorLength (* (.Origin (Collision|GetComponentBounds (Variables|Default|GetShipComponent))) 0.02)) 0.5 true)
  (Transformation|AttachComponentToComponent (Variables|Default|GetShipComponent) (Variables|Default|GetShipCollisionCapsule) "None" "KeepWorld" "KeepWorld" "KeepWorld" true))

(fn AttachComponentsfromData
  (params (ComponentArray :type Array%20of%20S%20Ship%20Component%20Structures) (SceneComponents :type Array%20of%20Scene%20Component%20Object%20References) (SoftDataList :type Array%20of%20Primary%20Data%20Asset%20Soft%20Object%20References))
  ;[0.15 0.15 0.15 0.5] Check to make sure that the array has information in it, then loop through it and create and assign the child actor components to the correct attachment point. Then store the newly created Actor Component Reference in the same index location.
  (if (Utilities|Array|IsNotEmpty ComponentArray)
    (for (_array_element _array_index) ComponentArray
      (bind _array_element_2 (Utilities|Array|ForEachLoopwithBreak SceneComponents :!label _label)
        (:LoopBody
          (if (Components|ComponentHasTag _array_element_2 (.AttachmentPoint (Utilities|Struct|BreakS_ShipComponent _array_element)))
            (bind _asbp_weapon_system_base_pda (Utilities|Casting|CastToBP_WeaponSystem_Base_PDA (.CurrentDataAsset (Utilities|Struct|BreakS_ShipComponent _array_element))))
            (bind _returnvalue (Utilities|LoadAssetBlocking (Utilities|Array|Get(acopy) SoftDataList (CallFunction|GetNextValidDataAssetArrayIndex (Utilities|ResolveSoftReference (.CurrentDataAsset (Utilities|Struct|BreakS_ShipComponent _array_element))) SoftDataList))))
            (bind _asbp_weapon_system_base_pda_2 (Utilities|Casting|CastToBP_WeaponSystem_Base_PDA _returnvalue))
            (Utilities|FlowControl|Sequence
              (:then_0
                (goto _label Break))
              (:then_1
                (bind _returnvalue_2 (AddComponent|AddChildActorComponent false (Transformation|GetRelativeTransform _array_element_2))) ; Returns a pointer to the child actor component, not the class that's assigned to it
                (ChildActorComponent|SetChildActorClass _returnvalue_2 (Variables|/Game/Actors/Ships/WeaponSystems/__DataAssets/BP_WeaponSystem_Base_PDA.BP_WeaponSystem_Base_PDA_C|GetWeaponClass _asbp_weapon_system_base_pda))
                (Utilities|Array|SetArrayElem (LocalVariables|GetTempArray) _array_index (Utilities|Struct|MakeS_ShipComponent (.AttachmentPoint (Utilities|Struct|BreakS_ShipComponent _array_element)) (.ComponentBaseClass (Utilities|Struct|BreakS_ShipComponent _array_element)) 0 (.CurrentDataAsset (Utilities|Struct|BreakS_ShipComponent _array_element)) _asbp_weapon_system_base_pda_2 _returnvalue_2 (.ComponentType (Utilities|Struct|BreakS_ShipComponent _array_element))) true))))))))
  (return (LocalVariables|GetTempArray)))

(fn AssemblefromData
  (params (UseSaveData :type Boolean) (Data :type BP%20Player%20Ship%20Save%20Data%20Object%20Reference))
  (bind _weapondataassets (Variables|Default|GetWeaponDataAssets))
  ;[0.15 0.15 0.15 0.5] Get the row that matches the ship name
  (if UseSaveData
    (Variables|Default|SetShipTableRow (Variables|/Game/Blueprints/SaveLoadSystem/BP_PlayerShipSaveData.BP_PlayerShipSaveData_C|GetShipConfiguration Data))
    ;[0.15 0.15 0.15 0.5] Add the base ship component
    (Variables|Default|SetStoredShipConfiguration (Variables|Default|GetShipTableRow) :!label _label)
    (bind _returnvalue (AddComponent|AddChildActorComponent true (Transformation|GetActorTransform)))
    (bind _output_get (Variables|Default|SetShipComponent _returnvalue))
    (Variables|/Script/Engine.SpringArmComponent|SetTargetArmLength (Variables|Default|GetCameraSpringArm) (.CameraDistance (Utilities|Struct|BreakS_ShipConfigurations (Variables|Default|GetShipTableRow))))
    (ChildActorComponent|SetChildActorClass _returnvalue (Utilities|ResolveSoftReference (.ShipBase (Utilities|Struct|BreakS_ShipConfigurations (Variables|Default|GetShipTableRow)))))
    ;[0.15 0.15 0.15 0.5] Attach Weapon Components
    (bind _modifiedarray (ShipCreation|AttachComponentsfromData (.OffensiveWeapons (Utilities|Struct|BreakS_ShipConfigurations (Variables|Default|GetShipTableRow))) (Components|GetChildrenComponents (Variables|Default|GetShipComponent) true) (.offensiveweapondataassets _weapondataassets))) ; Offensive Weapons
    (bind _modifiedarray_2 (ShipCreation|AttachComponentsfromData (.DefensiveWeapons (Utilities|Struct|BreakS_ShipConfigurations (Variables|Default|GetShipTableRow))) (Components|GetChildrenComponents (Variables|Default|GetShipComponent) true) (.defensiveweapondataassets _weapondataassets))) ; Defensive Weapons
    (bind _modifiedarray_3 (ShipCreation|AttachComponentsfromData (.MissileSilos (Utilities|Struct|BreakS_ShipConfigurations (Variables|Default|GetShipTableRow))) (Components|GetChildrenComponents (Variables|Default|GetShipComponent) true) (.missilesilodataassets _weapondataassets))) ; Missile Silos
    (bind _modifiedarray_4 (ShipCreation|AttachComponentsfromData (.SensorSystems (Utilities|Struct|BreakS_ShipConfigurations (Variables|Default|GetShipTableRow))) (Components|GetChildrenComponents (Variables|Default|GetShipComponent) true))) ; Sensors
    ;[0.15 0.15 0.15 0.5] Set the stored component data and then save it
    (bind _output_get_2 (Variables|Default|SetStoredShipConfiguration (Utilities|Struct|MakeS_ShipConfigurations (.shipname (Variables|Default|GetShipTableRow)) (.shiptype (Variables|Default|GetShipTableRow)) (.shipbase (Variables|Default|GetShipTableRow)) 0.0 (.shipcomponents (Variables|Default|GetShipTableRow)) _modifiedarray _modifiedarray_2 _modifiedarray_3 _modifiedarray_4)))
    (Class|BPISaveGame|SavePlayer(Message) (Game|GetGameInstance) _output_get_2 false)
    (else
      (bind (_tablerow _shipdatafound) (CallFunction|GetRowforShipinTable (Utilities|ResolveSoftReference (Variables|Default|GetTable)) (Variables|Default|GetShipName)))
      (Variables|Default|SetShipTableRow _tablerow)
      (if _shipdatafound
        (goto _label)))))

(fn UpdatedShipfromSaveData
  (params (SaveData :type BP%20Player%20Ship%20Save%20Data%20Object%20Reference) (PlayerShip :type Actor%20Object%20Reference))
  (bind _shipconfiguration (Variables|/Game/Blueprints/SaveLoadSystem/BP_PlayerShipSaveData.BP_PlayerShipSaveData_C|GetShipConfiguration SaveData))
  (bind (_shipname _shiptype _shipbase _cameradistance _shipcomponents _offensiveweapons _defensiveweapons _missilesilos _sensorsystems) (Utilities|Struct|BreakS_ShipConfigurations _shipconfiguration))
  ;[0.15 0.15 0.15 0.5] Store the player ship and get the save data
  (LocalVariables|SetLocalPlayer PlayerShip)
  (LocalVariables|SetSavedHardDataAssets (Variables|/Game/Blueprints/SaveLoadSystem/BP_PlayerShipSaveData.BP_PlayerShipSaveData_C|GetTempHardDataAssets SaveData))
  ;[0.15 0.15 0.15 0.5] Get the arrays from the saved data
  (LocalVariables|SetSavedConfiguration _shipconfiguration)
  (LocalVariables|SetShip_Saved _shipcomponents)
  (LocalVariables|SetOffensive_Saved _offensiveweapons)
  (LocalVariables|SetDefensive_Saved _defensiveweapons)
  (LocalVariables|SetMissile_Saved _missilesilos)
  (LocalVariables|SetSensor_Saved _sensorsystems)
  ;[0.15 0.15 0.15 0.5] Get the arrays from the players ship.
  (bind _asbp_ship_system_base (Utilities|Casting|CastToBP_ShipSystem_Base (LocalVariables|GetLocalPlayer)))
  (LocalVariables|SetShip_Local (.ShipComponents (Utilities|Struct|BreakS_ShipConfigurations (Variables|BP_ShipSystem_Base_C|GetStoredShipConfiguration _asbp_ship_system_base))))
  (LocalVariables|SetOffensive_Local (.OffensiveWeapons (Utilities|Struct|BreakS_ShipConfigurations (Variables|BP_ShipSystem_Base_C|GetStoredShipConfiguration _asbp_ship_system_base))))
  (LocalVariables|SetDefensive_Local (.DefensiveWeapons (Utilities|Struct|BreakS_ShipConfigurations (Variables|BP_ShipSystem_Base_C|GetStoredShipConfiguration _asbp_ship_system_base))))
  (LocalVariables|SetMissile_Local (.MissileSilos (Utilities|Struct|BreakS_ShipConfigurations (Variables|BP_ShipSystem_Base_C|GetStoredShipConfiguration _asbp_ship_system_base))))
  (LocalVariables|SetSensor_Local (.SensorSystems (Utilities|Struct|BreakS_ShipConfigurations (Variables|BP_ShipSystem_Base_C|GetStoredShipConfiguration _asbp_ship_system_base))))
  ;[0.15 0.15 0.15 0.5] Check if there are components in each array. If there are then loop through them, if not then ignore the array
  (Utilities|FlowControl|Sequence
    (:then_0
      (if (Utilities|Array|IsNotEmpty (LocalVariables|GetShip_Saved))
        (for _array_element (LocalVariables|GetShip_Saved)
          (UpdateShipData|UpdateComponentfromSaveData _array_element (LocalVariables|GetShip_Local)))
        ;[0.15 0.15 0.15 0.5] After all components are updated, save the game
        (Class|BPISaveGame|SavePlayer(Message) (Game|GetGameInstance) (LocalVariables|GetSavedConfiguration) false :!label _label)
        (Variables|Default|SetStoredShipConfiguration (Utilities|Struct|MakeS_ShipConfigurations (.shipname (LocalVariables|GetSavedConfiguration)) (.shiptype (LocalVariables|GetSavedConfiguration)) (.shipbase (LocalVariables|GetSavedConfiguration)) 0.0 (LocalVariables|GetShip_Local) (LocalVariables|GetOffensive_Local) (LocalVariables|GetDefensive_Local) (LocalVariables|GetMissile_Local) (LocalVariables|GetSensor_Local)))))
    (:then_1
      (if (Utilities|Array|IsNotEmpty (LocalVariables|GetOffensive_Saved))
        (for _array_element_2 (LocalVariables|GetOffensive_Saved)
          (UpdateShipData|UpdateComponentfromSaveData _array_element_2 (LocalVariables|GetOffensive_Local)))
        (goto _label)))
    (:then_2
      (if (Utilities|Array|IsNotEmpty (LocalVariables|GetDefensive_Saved))
        (for _array_element_3 (LocalVariables|GetDefensive_Saved)
          (UpdateShipData|UpdateComponentfromSaveData _array_element_3 (LocalVariables|GetDefensive_Local)))
        (goto _label)))
    (:then_3
      (if (Utilities|Array|IsNotEmpty (LocalVariables|GetMissile_Saved))
        (for _array_element_4 (LocalVariables|GetMissile_Saved)
          (UpdateShipData|UpdateComponentfromSaveData _array_element_4 (LocalVariables|GetMissile_Local)))
        (goto _label)))
    (:then_4
      (if (Utilities|Array|IsNotEmpty (LocalVariables|GetSensor_Saved))
        (for _array_element_5 (LocalVariables|GetSensor_Saved)
          (UpdateShipData|UpdateComponentfromSaveData _array_element_5 (LocalVariables|GetSensor_Local)))
        (goto _label)))))

(fn UpdateComponentfromSaveData
  (params (SavedArrayItem :type S%20Ship%20Component%20Structure) (LocalArray :type Array%20of%20S%20Ship%20Component%20Structures))
  (bind (_attachmentpoint _componentbaseclass _previousdataasset _currentdataasset) (Utilities|Struct|BreakS_ShipComponent SavedArrayItem))
  ;[0.15 0.15 0.15 0.5] Compair the attachment point in the local array to the one in the saved array. If they match then assume its the correct array item and update it.
  (for (_array_element _array_index) LocalArray
    (if (== _attachmentpoint (.AttachmentPoint (Utilities|Struct|BreakS_ShipComponent _array_element)))
      ;[0.15 0.15 0.15 0.5] Cast the data asset to the parent class and set the child component from the local array to the new class.
      (bind _asbp_weapon_system_base_pda (Utilities|Casting|CastToBP_WeaponSystem_Base_PDA _currentdataasset))
      (ChildActorComponent|SetChildActorClass (.ActorComponentReference (Utilities|Struct|BreakS_ShipComponent _array_element)) (Variables|/Game/Actors/Ships/WeaponSystems/__DataAssets/BP_WeaponSystem_Base_PDA.BP_WeaponSystem_Base_PDA_C|GetWeaponClass _asbp_weapon_system_base_pda))
      (CallFunction|UpdateLocalComponenttoSaved LocalArray _array_index _array_element SavedArrayItem) ; Set the local array item to match the saved one.
    )))

(fn ComponentType
  (return "NewEnumerator0"))

(fn ContactType
  (return "NewEnumerator0"))

(fn ObjectDetected
  (params (DetectedObjectHit_In :type Hit%20Result%20Structure) (SensorThatDetected_In :type Actor%20Component%20Object%20Reference))
  (return "" 0))