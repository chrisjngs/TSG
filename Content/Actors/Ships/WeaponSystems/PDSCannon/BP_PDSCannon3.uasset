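; PDS cannon ship weapon actor that supports hover inspection and click selection, apparently for ship customization.
; Cursor hover has BPWeaponSystemAC build an info widget from the DataAsset and highlight the actor, then clear both on exit.
; Clicks forward to BPCustomizableAC, while attachment-cycling logic sits unconnected.
; A local RenderInteractionWidget duplicates popup creation but is uncalled here, and the author marks the hover logic for a future weapon parent class.
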(event MouseInput|EventActorBeginCursorOver
  (bind _bp_weaponsystem_ac (Variables|Default|GetBP_WeaponSystem_AC))
  ;[0.15 0.15 0.15 0.5] All of this should go into the Weapon Parent Class for the official build, that way every weapon will be able to opporate the same without having to duplicate the logic
  ;;[0.15 0.15 0.15 0.5] Logic for creating the hover events. First create the widget, then add the information to it, and highlight the actor components
  (Default|EventGenerateWidget _bp_weaponsystem_ac (Utilities|ResolveSoftReference self) (Utilities|ResolveSoftReference (Variables|Default|GetWidget_Location)))
  (Default|RenderInteractionWidget :self _bp_weaponsystem_ac :SystemInfo (Variables|Default|GetDataAsset))
  (Default|HighlightSelectionon _bp_weaponsystem_ac self))

(event MouseInput|EventActorOnClicked
  (params (ButtonPressed :type Key%20Structure))
  (Default|ComponentClickedEvent (Variables|Default|GetBP_Customizable_AC) (Utilities|ResolveSoftReference self)))

(event MouseInput|EventActorEndCursorOver
  (bind _bp_weaponsystem_ac (Variables|Default|GetBP_WeaponSystem_AC))
  ;[0.15 0.15 0.15 0.5] All of this should go into the Weapon Parent Class for the official build, that way every weapon will be able to opporate the same without having to duplicate the logic
  ;;[0.15 0.15 0.15 0.5] Logic for creating the hover events. First create the widget, then add the information to it, and highlight the actor components
  ;;;[0.15 0.15 0.15 0.5] Remove the widget and highlight selection
  (Default|HighlightSelectionOff _bp_weaponsystem_ac self)
  (bind _widget (Variables|/Game/Actors/Ships/WeaponSystems/BP_WeaponSystem_AC.BP_WeaponSystem_AC_C|GetWidget (Variables|Default|GetBP_WeaponSystem_AC))
    (:then
      (Default|RemoveInteractionWidget _bp_weaponsystem_ac _widget))
    (:else)))

(event Collision|EventActorBeginOverlap
  (params (OtherActor :type Actor%20Object%20Reference)))

(event EventTick
  (params (DeltaSeconds :type Float%20%28single-precision%29)))

(fn ConstructionScript)

(fn RenderInteractionWidget
  (bind _widget_location (Variables|Default|GetWidget_Location))
  (bind _returnvalue (UserInterface|CreateWidget "/Game/HUD/PremadeWidgets/BPW_HoverPopup.BPW_HoverPopup_C"))
  (bind _output_get (Variables|Default|SetHoverPopup _returnvalue))
  (UserInterface|SetWidget _widget_location _output_get)
  (Transformation|SetWorldLocation _widget_location (Transformation|GetWorldLocation (Variables|Default|GetWidget_Location)) false false)
  (Rendering|Components|TextRender|SetText (Variables|/Game/HUD/PremadeWidgets/BPW_HoverPopup.BPW_HoverPopup_C|GetTitle_Text _output_get) (.name (Variables|Default|GetWeaponSystemInfo))))

(fn ComponentType
  (return "NewEnumerator1"))