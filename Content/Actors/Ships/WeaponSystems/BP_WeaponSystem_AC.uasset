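; Weapon system component (AC) that handles hover, highlight and swapping of ship weapon attachments.
; It creates a screen-space widget beside the owning actor, offset along the camera's right vector, showing weapon name and tracking range.
; Selection highlighting sets or clears an outline overlay material on static meshes.
; CycleAttachment replaces the attachment with the next class in an array, reattaches it with a hologram material, while another function resolves attachment points.
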(event Custom|Event_GenerateWidget
  (params (OwningActor :type Actor%20Soft%20Object%20Reference) (WidgetLocation :type Scene%20Component%20Soft%20Object%20Reference))
  (bind _returnvalue (Game|GetPlayerCameraManager 0))
  (bind _output (Utilities|ResolveSoftReference WidgetLocation))
  (bind _returnvalue_2 (Transformation|GetActorRightVector _returnvalue))
  (bind _output_get (Variables|Default|SetOwningActor (Utilities|ResolveSoftReference OwningActor)))
  (Transformation|SetWorldLocation _output (+ (.Origin (Collision|GetActorBounds _output_get false false)) (* _returnvalue_2 (+ (Math|Vector|DotProduct _returnvalue_2 (.BoxExtent (Collision|GetActorBounds _output_get false false))) -7.0))) false true)
  (bind _returnvalue_3 (Game|AddComponentbyClass _output_get "/Script/UMG.WidgetComponent" true (Transformation|GetWorldTransform _output)))
  (Class|WidgetComponent|SetWidgetSpace _returnvalue_3 "Screen")
  (Class|WidgetComponent|SetDrawSize _returnvalue_3 "(X=100.000000,Y=150.000000)")
  (bind _output_get_2 (Variables|Default|SetWidget _returnvalue_3))
  (Transformation|AttachComponentToComponent _output_get_2 _output "None" "SnapToTarget" "SnapToTarget" "SnapToTarget" true))

(fn RenderInteractionWidget
  (params (WidgetTransform :type Transform) (SystemInfo :type BP%20Weapon%20System%20Base%20PDA%20Object%20Reference))
  (bind _widget (Variables|Default|GetWidget))
  (bind _returnvalue (UserInterface|CreateWidget "/Game/HUD/PremadeWidgets/BPW_HoverPopup.BPW_HoverPopup_C" (Game|GetPlayerController 0)))
  (bind _output_get (Variables|Default|SetHoverPopup _returnvalue))
  (UserInterface|SetWidget _widget _output_get)
  (Transformation|SetWorldLocation _widget (Transformation|GetWorldLocation (Variables|Default|GetWidget)) false false)
  (Rendering|Components|TextRender|SetText (Variables|/Game/HUD/PremadeWidgets/BPW_HoverPopup.BPW_HoverPopup_C|GetTitle_Text _output_get) (Utilities|Text|ToText(Name) (Variables|/Game/Actors/Ships/WeaponSystems/__DataAssets/BP_WeaponSystem_Base_PDA.BP_WeaponSystem_Base_PDA_C|GetWeaponName SystemInfo)))
  (Rendering|Components|TextRender|SetText (Variables|/Game/HUD/PremadeWidgets/Text/BPW_TextBlock.BPW_TextBlock_C|GetPremadeTextBlock_TXT (Variables|/Game/HUD/PremadeWidgets/BPW_HoverPopup.BPW_HoverPopup_C|GetBPW_DetailsText_TXT _output_get)) (Utilities|Text|ToText(String) (Utilities|String|Append "Tracking Range : " (Utilities|String|ToString(Float) (Variables|/Game/Actors/Ships/WeaponSystems/__DataAssets/BP_WeaponSystem_Base_PDA.BP_WeaponSystem_Base_PDA_C|GetTrackingRange SystemInfo))))))

(fn HighlightSelectionon
  (params (Actor :type Actor%20Object%20Reference))
  (bind _owningactor (Variables|Default|GetOwningActor))
  (Utilities|IsValid _owningactor
    (:Is%20Valid
      (for _array_element (Actor|GetComponentsByClass _owningactor "/Script/Engine.StaticMeshComponent")
        (Rendering|Material|SetOverlayMaterial _array_element "/Game/Blueprints/Components/CustomizationSystem/Hologram_OutlineEnvironment_MTL.Hologram_OutlineEnvironment_MTL" :!class /Script/Engine.MeshComponent)))))

(fn HighlightSelectionOff
  (params (Actor :type Actor%20Object%20Reference))
  (Utilities|IsValid Actor
    (:Is%20Valid
      (for _array_element (Actor|GetComponentsByClass Actor "/Script/Engine.StaticMeshComponent")
        (Rendering|Material|SetOverlayMaterial _array_element 0 :!class /Script/Engine.MeshComponent)))))

(fn RemoveInteractionWidget
  (params (Widget :type Widget%20Component%20Object%20Reference))
  (Utilities|IsValid Widget
    (:Is%20Valid
      (Rendering|SetVisibility Widget false false))))

(fn SelectonClick
  (bind _owningactor (Variables|Default|GetOwningActor)
    (:then
      (if (Class|Actor|IsChildActor _owningactor)
        (return _owningactor)))
    (:else)))

(fn CycleAttachment
  (params (Attachment :type Actor%20Object%20Reference) (ParentComponent :type Scene%20Component%20Object%20Reference))
  (bind _attachmentclassarray (LocalVariables|GetAttachmentClassArray))
  (LocalVariables|GetAttachmentClass
    (:then
      _)
    (:else
      (bind _output_get (LocalVariables|SetAttachmentClass (Utilities|ResolveSoftReference (Utilities|GetClass Attachment))))))
  (Utilities|IsValid Attachment
    (:Is%20Valid
      (LocalVariables|SetArrayIndex (Utilities|Array|FindItem _attachmentclassarray _output_get))
      (if (>= (Utilities|Array|FindItem _attachmentclassarray _output_get) (- (Utilities|Array|Length _attachmentclassarray) 1))
        (LocalVariables|SetArrayIndex 0)
        (else
          (LocalVariables|SetArrayIndex (+ (LocalVariables|GetArrayIndex) 1))))
      (bind _returnvalue (Game|SpawnActorfromClass (Utilities|ResolveSoftReference (Utilities|Array|Get(acopy) (LocalVariables|GetAttachmentClassArray) (LocalVariables|GetArrayIndex))) (Transformation|GetActorTransform Attachment) "Undefined" "MultiplyWithRoot" 0 0))
      (LocalVariables|SetAttachmentClass (Utilities|ResolveSoftReference (Utilities|GetClass _returnvalue)))
      (Transformation|AttachActorToActor _returnvalue (Components|GetOwner ParentComponent) "None" "KeepWorld" "KeepWorld" "SnapToTarget" true)
      (for _array_element (Actor|GetComponentsByClass _returnvalue "/Script/Engine.StaticMeshComponent")
        (Utilities|IsValid _array_element
          (:Is%20Valid
            (Rendering|Material|SetMaterial _array_element 0 "/Game/Actors/Structures/ProxySpaceStation/Materials/Hologram_MTL_Inst.Hologram_MTL_Inst"))))
      (Actor|DestroyActor Attachment))
    (:Is%20Not%20Valid
      (Utilities|Debugging|RaiseScriptError "An error occurred: No valid parent to attach to."))))

(fn GetOwningActor
  (params (Child :type Actor%20Object%20Reference))
  (return (Components|GetOwner Child)))

(fn ValidateAttachmentPoint
  (params (AttachmentToCheck :type Actor%20Object%20Reference))
  (bind _returnvalue (Components|GetOwner AttachmentToCheck))
  (Utilities|IsValid _returnvalue
    (:Is%20Valid
      (LocalVariables|SetValidCheck true)
      (LocalVariables|SetPoint (Actor|GetComponentbyClass _returnvalue "/Script/Engine.SceneComponent")))
    (:Is%20Not%20Valid
      (bind _returnvalue_2 (Game|AddComponentbyClass (Actor|GetAttachParentActor AttachmentToCheck) "/Script/Engine.SceneComponent" true (Transformation|GetActorTransform AttachmentToCheck)))
      ;[0.15 0.15 0.15 0.5] This isn't attaching properly to include the rotation of the hologram
      (Transformation|AttachComponentToComponent _returnvalue_2 (Variables|/Script/Engine.Actor|GetRootComponent AttachmentToCheck) "None" "SnapToTarget" "SnapToTarget" "SnapToTarget" true)
      (LocalVariables|SetPoint _returnvalue_2)
      (LocalVariables|SetValidCheck true)))
  (return (LocalVariables|GetValidCheck) (LocalVariables|GetPoint)))