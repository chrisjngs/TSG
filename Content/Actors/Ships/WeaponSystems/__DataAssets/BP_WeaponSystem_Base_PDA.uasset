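; Base primary data asset for ship weapon systems, holding shared weapon state and helper functions.
; It derives its destroyed flag from whether health has run out and attaches a weapon component to a given parent using keep-relative rules.
; Reloading triggers when the passed-in ammo is empty, setting a reloading flag and returning the magazine size; nothing here clears that flag.
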(fn SetDestroyed
  (if (<= (Variables|WeaponVariables|WeaponSpecific|Private|GetHealth) 0.0)
    (Variables|WeaponVariables|WeaponSpecific|Public|SetDestroyed true)
    (else
      (Variables|WeaponVariables|WeaponSpecific|Public|SetDestroyed false))))

(fn AttachWeapon
  (params (Actor :type Actor%20Soft%20Object%20Reference) (Attachement :type Scene%20Component%20Soft%20Object%20Reference))
  (Transformation|AttachComponentToComponent (Utilities|ResolveSoftReference Actor) (Utilities|ResolveSoftReference Attachement) "None" "KeepRelative" "KeepRelative" "KeepRelative" true))

(fn ReloadWeapon
  (params (CurrentAmmo :type Integer))
  (if (<= CurrentAmmo 0)
    (Variables|WeaponVariables|WeaponSpecific|Public|SetReloading true)
    (return (Variables|WeaponVariables|WeaponSpecific|Private|GetMagazineSize))))