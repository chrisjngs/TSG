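; BP_Frigate_Protoype is a prototype frigate ship Blueprint that configures its weapon platform and thrusters.
; Its construction script sends the main battle cannon data asset to the child actor in OffensiveWeapon03 via ChangeDataAssetMessage, then runs the parent construction script.
; GetThrusters returns the two engine thrust components, and GetPlatformComponents returns OffensiveWeapon03 as the only platform.
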(fn ConstructionScript
  (Class|BPIWeaponSystem|ChangeDataAsset(Message) (Variables|/Script/Engine.ChildActorComponent|GetChildActor (Variables|Default|GetOffensiveWeapon_03)) "/Game/Actors/WeaponSystems/__DataAssets/DA_MainBattleCannon.DA_MainBattleCannon" false)
  (|CallParentFunction))

(fn GetThrusters
  (return (Utilities|Array|MakeArray (Variables|Default|GetEngineThrust_001) (Variables|Default|GetEngineThrust_002))))

(fn GetPlatformComponents
  (return (Utilities|Array|MakeArray (Variables|Default|GetOffensiveWeapon_03))))