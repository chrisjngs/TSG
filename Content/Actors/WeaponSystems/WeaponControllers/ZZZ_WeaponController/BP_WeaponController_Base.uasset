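; Base weapon controller actor that defines query functions for weapons, contacts, faction and platform components.
; Getters cover all, assigned and available offensive, defensive and missile weapons, plus contact lists per role, contact priority and assigned contact maps.
; Every function is an empty stub, except that GetFaction returns a fixed first enum entry.
; The event graph and construction script contain no logic.
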(event EventBeginPlay)

(event Collision|EventActorBeginOverlap
  (params (OtherActor :type Actor%20Object%20Reference)))

(event EventTick
  (params (DeltaSeconds :type Float%20%28single-precision%29)))

(fn ConstructionScript)

(fn GetAllDefensiveWeapons
  (return 0))

(fn GetAllMissileWeapons
  (return 0))

(fn GetAllOffensiveWeapons
  (return 0))

(fn GetAssignedContactMaps
  (return 0 0 0 0))

(fn GetAssignedDefensiveWeapons
  (return 0))

(fn GetAssignedMissileWeapons
  (return 0))

(fn GetAssignedOffensiveWeapons
  (return 0))

(fn GetAvailableDefensiveWeapons
  (return 0))

(fn GetAvailableMissileLaunchers
  (return 0))

(fn GetAvailableOffensiveWeapons
  (return 0))

(fn GetContactPriority
  (return 0 0 0 0))

(fn GetContacts
  (return 0))

(fn GetContactsforDefense
  (return 0))

(fn GetContactsforMissiles
  (return 0))

(fn GetContactsforOffensive
  (return 0))

(fn GetFaction
  (return "NewEnumerator0"))

(fn GetPlatformComponents
  (return 0 ""))

(fn ReturnWeaponController
  (return 0))