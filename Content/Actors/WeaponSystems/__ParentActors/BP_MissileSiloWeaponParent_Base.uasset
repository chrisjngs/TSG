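; Base missile silo weapon that launches pooled missiles at an assigned Contact.
; Reload picks an unused missile, spawning a magazine-sized batch from the data asset when none is free, then updates MasterAI and re-arms a DoOnce fire gate.
; Firing launches the loaded missile along the launch spot's up vector and clears the ManualFire blackboard flag.
; Contact assignment writes to the AI blackboard, notifying MasterAI when manual; faction changes propagate to pooled missiles.
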(event EventTick
  (params (DeltaSeconds :type Float%20%28single-precision%29))
  (|CallParentFunction DeltaSeconds))

(event EventSetFactionType
  (params (SetFaction :type E_FriendFoe%20Enum :default "NewEnumerator0"))
  (bind _output_get (Variables|Default|SetFaction SetFaction))
  (for _array_element (Variables|Default|GetAmmoPool)
    (Class|BPITargetable|SetFactionType(Message) _array_element _output_get)))

(event EventFireWeapon
  (bind _contact (Variables|Default|GetContact))
  (bind _ammopool (Variables|Default|GetAmmoPool))
  (bind _missileindex (Variables|Default|GetMissileIndex))
  (bind _missilelaunchspot (Variables|Default|GetMissileLaunchSpot))
  (bind _output (Utilities|Array|Get(acopy) _ammopool _missileindex))
  (Utilities|FlowControl|DoOnce false
    (:Completed
      (Variables|Default|GetMissileInTube
        (:then
          (Utilities|IsValid _output
            (:Is%20Valid
              (Utilities|IsValid _contact
                (:Is%20Valid
                  (Class|BPIProjectile|SetStartTransform(Message) _output (Transformation|GetWorldTransform _missilelaunchspot))
                  (Class|BPIProjectile|Fire(Message) _output _contact (* (Math|Vector|GetUpVector _missilelaunchspot) 1e+04) 0.0)
                  (Variables|Default|SetMissileInTube false)
                  (AI|Components|Blackboard|SetValueasBool (Variables|Default|GetAIBlackboard) (Utilities|Name|MakeLiteralName "ManualFire") false))
                (:Is%20Not%20Valid
                  (Development|PrintString "Failed in Parent Missile Silo valid check"))))))
        (:else)))))

(event EventReloadWeapon
  (bind _contact (Variables|Default|GetContact))
  (bind _missilelaunchspot (Variables|Default|GetMissileLaunchSpot))
  (bind (_array_element _array_index) (Utilities|Array|ForEachLoopwithBreak (Variables|Default|GetAmmoPool) :!label _label)
    (:LoopBody
      (bind _inuse (Class|BPIProjectile|GetinUse(Message) _array_element))
      (if (not _inuse)
        (Variables|Default|SetMissileIndex _array_index)
        (Variables|Default|SetMissileInTube true)
        (goto _label Break)))
    (:Completed
      (Variables|Default|GetMissileInTube
        (:then
          (Class|BPIWeaponController|UpdateMissileAssignments(Message) (Variables|Default|GetMaster%20AI) "NewEnumerator2" self :!label _label_2)
          (if true
            (Utilities|FlowControl|DoOnce false) ; enters at Reset
          ))
        (:else
          (bind _poolcreated (CallFunction|CreateAmmoPool))
          (if _poolcreated
            (goto _label_2)))))))

(event EventAssignContact
  (params (Contact :type Actor%20Object%20Reference) (Manual :type Boolean))
  (bind _output_get (Variables|Default|SetContact Contact))
  (AI|Components|Blackboard|SetValueasObject (Variables|Default|GetAIBlackboard) (Utilities|Name|MakeLiteralName "Contact") _output_get)
  (if Manual
    (Class|BPIWeaponController|UpdateMissileAssignments(Message) (Variables|Default|GetMaster%20AI) "NewEnumerator1" self (Variables|Default|GetContact))))

(fn ConstructionScript
  (|CallParentFunction))

(fn ResetBlackboardValues
  (bind _aiblackboard (Variables|Default|GetAIBlackboard))
  (AI|Components|Blackboard|SetValueasObject _aiblackboard (Utilities|Name|MakeLiteralName "Contact") 0)
  (AI|Components|Blackboard|SetValueasBool _aiblackboard (Utilities|Name|MakeLiteralName "AmmoCreated") false))

(fn CreateAmmoPool
  (bind _ammopool (Variables|Default|GetAmmoPool))
  (for _index (range 0 (- (Variables|/Game/Actors/WeaponSystems/__DataAssets/BP_WeaponSystem_Base_PDA.BP_WeaponSystem_Base_PDA_C|GetMagazineSize (Variables|Default|GetPrimaryDataAsset)) 1))
    (bind _returnvalue (Game|SpawnActorfromClass "/Game/Actors/WeaponSystems/Projectiles/Missiles/BP_BasicMissile_Test.BP_BasicMissile_Test_C" (Transformation|GetActorTransform) "AlwaysSpawn" "MultiplyWithRoot" 0 true (Variables|Default|GetFaction) (Variables|Default|GetAmmoDataAsset) 0))
    (Utilities|Array|AddUnique (Variables|Default|GetAmmoPool) _returnvalue))
  (for _array_element _ammopool
    (Class|BPIProjectile|SetIgnoreActors(Message) _array_element "NewEnumerator2" 0 self))
  (Variables|Default|SetMissileInTube true)
  (Variables|Default|SetMissileIndex (Utilities|Array|LastIndex _ammopool))
  (return true))