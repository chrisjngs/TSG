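; BP_WeaponChildActor_Base is a parent actor for weapon child actors, built around a BPWeaponSystemAC component that its construction script initializes.
; It exposes a set of weapon query functions, returning its DataAsset and component type and forwarding the projectile start to the component.
; The remaining queries for ammo pool, platform, meshes, positioning, range and reload are stubs returning false or nothing, and the event graph is empty.
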(event EventBeginPlay)

(event Collision|EventActorBeginOverlap
  (params (OtherActor :type Actor%20Object%20Reference)))

(event EventTick
  (params (DeltaSeconds :type Float%20%28single-precision%29)))

(fn ConstructionScript
  (Default|InitializeAC (Variables|Default|GetBP_WeaponSystem_AC)))

(fn ComponentType
  (return "NewEnumerator0"))

(fn CreateAmmoPool
  (return false))

(fn GetAttachedPlatform
  (return 0))

(fn GetDataAsset
  (return (Variables|Default|GetDataAsset)))

(fn GetMeshComponents
  (return 0 0 0))

(fn GetPlatformComponents
  (return 0 ""))

(fn GetProjectileStart
  (bind _projectilestart (Default|GetProjectileStart (Variables|Default|GetBP_WeaponSystem_AC)))
  (return _projectilestart))

(fn GetWeaponinPosition
  (return false))

(fn InRange
  (params (Contact :type Actor%20Object%20Reference))
  (return false))

(fn NeedsReload
  (return false))