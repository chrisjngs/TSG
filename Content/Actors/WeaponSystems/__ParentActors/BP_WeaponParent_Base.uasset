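; Base weapon actor for platform-mounted weapon systems that engage assigned contacts.
; A primary data asset sets its child weapon actor, stats, health and ammo type, while the child actor handles rotation and in-position checks.
; It syncs contact, burst and reload state to the AI Blackboard, firing pooled projectiles with spread and optional target prediction.
; On death it hides, notifying actors targeting it until none remain, then destroys itself.
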(event ComponentDestrroyed(BP_Health_AC)
  (Default|HideHealthBar (Variables|Default|GetBP_Health_AC))
  (Utilities|Array|RemoveItem (Variables|Default|GetActorsTargeting) self)
  (if (Utilities|Array|IsEmpty (Variables|Default|GetActorsTargeting))
    (Actor|DestroyActor)
    (else
      (Rendering|SetActorHiddenInGame true)
      (bind _returnvalue (Utilities|Time|SetTimerbyEvent (delegate Custom|Event_DeathTimer) 0.1 true))
      (Variables|Default|SetDeathTimer _returnvalue))))

(event Custom|Event_UpdateWeaponWithNewDataAssetVars
  (params (PrimaryDataAsset :type Primary%20Data%20Asset%20Object%20Reference) (UseSoftReference :type Boolean) (PrimaryDataAsset_Soft :type Primary%20Data%20Asset%20Soft%20Object%20Reference))
  ;[0.15 0.15 0.15 0.5] Update the actor with new information from the passed data asset
  (bind _primarydataasset (Initialization|WeaponCreation|UpdateDataAsset PrimaryDataAsset UseSoftReference PrimaryDataAsset_Soft))
  (Initialization|DataTableWork|SetVariablesfromDataAsset _primarydataasset)
  (Initialization|WeaponCreation|InitHealthVariables _primarydataasset))

(event Custom|Event_DeathTimer
  (bind _actorstargeting (Variables|Default|GetActorsTargeting))
  (if (Utilities|Array|IsEmpty _actorstargeting)
    (Actor|DestroyActor)
    (else
      (for _array_element _actorstargeting
        (Utilities|IsValid _array_element
          (:Is%20Valid
            (Class|BPIWeaponSystem|ContactDestroyed(Message) _array_element))
          (:Is%20Not%20Valid
            (Utilities|Array|RemoveItem (Variables|Default|GetActorsTargeting) _array_element)))))))

(event EventSetMaster/Slave
  (params (IsSlave :type Boolean) (MasterAI :type Actor%20Object%20Reference))
  (Variables|Initialization|WeaponCreation|SetIs%20Slave IsSlave)
  (Variables|AI|SetMaster%20AI MasterAI))

(event EventTakeDamage
  (params (Damage :type Float%20%28double-precision%29)))

(event EventSetFireWeapon
  (params (FireStatus :type Boolean))
  (AI|Components|Blackboard|SetValueasBool (Variables|AI|GetAIBlackboard) (Utilities|Name|MakeLiteralName "AutoFire") FireStatus))

(event EventContactDestroyed
  (bind _aiblackboard (Variables|AI|GetAIBlackboard))
  (bind _master_ai (Variables|AI|GetMaster%20AI))
  ;[0.15 0.15 0.15 0.5] Contact Destroyed
  (Class|BPITargetable|UpdateTargeting(Message) (Variables|WeaponLogic|Targets|GetAssignedContact) "NewEnumerator3" 0 self)
  (AI|Components|Blackboard|SetValueasObject _aiblackboard (Utilities|Name|MakeLiteralName "Contact") 0)
  (AI|Components|Blackboard|SetValueasBool _aiblackboard (Utilities|Name|MakeLiteralName "ContactDestroyed") true)
  (Variables|WeaponLogic|Tracking|SetPredictTarget false)
  (Variables|Initialization|WeaponCreation|GetIs%20Slave
    (:then
      (Class|BPIWeaponController|ContactDestroyed(Message) _master_ai (Variables|WeaponLogic|Targets|GetAssignedContact) self)
      (Class|BPIWeaponController|UpdateImmediateContacts(Message) _master_ai "NewEnumerator3" 0 0 (Variables|WeaponLogic|Targets|GetAssignedContact))
      (Class|BPIWeaponController|UpdateContacts(Message) _master_ai "NewEnumerator3" 0 0 (Variables|WeaponLogic|Targets|GetAssignedContact))
      (Variables|WeaponLogic|Targets|SetAssignedContact 0))
    (:else
      (Variables|WeaponLogic|Targets|SetAssignedContact 0))))

(event EventSetPlatformComponents
  (params (Platform :type Actor%20Object%20Reference) (PlatformComponents :type S%20Ship%20Child%20Components%20Structure))
  (Variables|Default|SetAttachedPlatform Platform)
  (Variables|Default|SetAttachedPlatformComponents PlatformComponents)
  (Class|BPIWeaponSystem|SetAttachedPlatform(Message) (Components|GetOwner (Components|GetChildComponent (Variables|Default|GetWeapon_ChildActor) 0)) (Variables|Default|GetAttachedPlatform)))

(event EventSetTargetable
  (params (Targetable :type Boolean))
  (Variables|Default|SetTargetable Targetable))

(event EventRotateWeapon
  (params (Rotator :type Rotator :default "0, 0, 0") (TargetLocation :type Vector :default "0, 0, 0"))
  ;[0.15 0.15 0.15 0.5] Rotate the weapon through the weapon actor
  (Class|BPIWeaponSystem|RotateWeapon(Message) (Components|GetOwner (Components|GetChildComponent (Variables|Default|GetWeapon_ChildActor) 0)) Rotator TargetLocation))

(event EventUpdateTargeting
  (params (How? :type E_ArrayModification%20Enum :default "NewEnumerator0") (AddActor :type Actor%20Object%20Reference) (RemoveTarget :type Actor%20Object%20Reference))
  (bind _actorstargeting (Variables|Default|GetActorsTargeting))
  (switch Utilities|FlowControl|Switch|SwitchonE_ArrayModification How?
    (:NewEnumerator2
      (Utilities|Array|Add _actorstargeting AddActor))
    (:NewEnumerator3
      (Utilities|Array|RemoveItem _actorstargeting RemoveTarget))))

(event EventReloadWeapon
  (bind _bp_weaponsystem_ac (Variables|Default|GetBP_WeaponSystem_AC))
  ;[0.15 0.15 0.15 0.5] Reload
  (AI|Components|Blackboard|SetValueasBool (Variables|AI|GetAIBlackboard) (Utilities|Name|MakeLiteralName "NeedsReload") false)
  (Variables|WeaponLogic|Ammo|SetShotIndex 0)
  (Class|BlackboardComponent|SetValueasInt (Variables|AI|GetAIBlackboard) (Utilities|Name|MakeLiteralName "BurstIndex"))
  (Default|EventReload _bp_weaponsystem_ac)
  (Variables|/Game/Blueprints/Components/WeaponSystem/BP_WeaponSystem_AC.BP_WeaponSystem_AC_C|SetCurrentAmmo _bp_weaponsystem_ac (Variables|/Game/Actors/WeaponSystems/__DataAssets/BP_WeaponSystem_Base_PDA.BP_WeaponSystem_Base_PDA_C|GetMagazineSize (Variables|Default|GetPrimaryDataAsset))))

(event EventStartPredicting
  (params (TargetActor :type Actor%20Object%20Reference) (PredictionTime :type Float%20%28double-precision%29))
  ;[0.15 0.15 0.15 0.5] Prediction
  (Variables|/Game/Actors/WeaponSystems/__DataAssets/BP_WeaponSystem_Base_PDA.BP_WeaponSystem_Base_PDA_C|GetUsePredictiveLocation (Variables|Default|GetPrimaryDataAsset)
    (:then
      (Variables|WeaponLogic|Tracking|SetPredictTarget true)
      (Variables|WeaponLogic|Tracking|SetPrediction%20Time (/ (CallFunction|GetDistancetoTarget self TargetActor) (Variables|/Game/Actors/WeaponSystems/Projectiles/__DataAssets/Projectile_PDA.Projectile_PDA_C|GetSpeed (Variables|Initialization|WeaponCreation|Ammo|GetAmmoDataAsset)))))
    (:else)))

(event EventAssignContact
  (params (Contact :type Actor%20Object%20Reference) (Manual :type Boolean))
  (bind _aiblackboard (Variables|AI|GetAIBlackboard))
  ;[0.15 0.15 0.15 0.5] Logic for assigning contacts to weapon
  (if (or (Variables|Initialization|WeaponCreation|GetIs%20Slave) Manual)
    (Class|BPIWeaponSystemAI|UpdateAssignment(Message) (AI|GetAIController self) Contact))
  (Variables|WeaponLogic|Targets|GetAssignedContact
    (:then
      (WeaponLogic|ClearAssignment))
    (:else
      _))
  (bind _output_get (Variables|WeaponLogic|Targets|SetAssignedContact Contact))
  (AI|Components|Blackboard|SetValueasObject _aiblackboard (Utilities|Name|MakeLiteralName "Contact") _output_get)
  (AI|Components|Blackboard|SetValueasBool _aiblackboard (Utilities|Name|MakeLiteralName "TargetDestroyed") false)
  ;;[0.15 0.15 0.15 0.5] This might cause an issue since I'm not setting any prediction time
  (Variables|WeaponLogic|Tracking|SetPredictTarget true)
  (Class|BPITargetable|UpdateTargeting(Message) (Variables|WeaponLogic|Targets|GetAssignedContact) "NewEnumerator2" self))

(event EventTick
  (params (DeltaSeconds :type Float%20%28single-precision%29))
  (Variables|Utility|SetDelta%20Seconds DeltaSeconds)
  (Variables|WeaponLogic|Tracking|GetPredictTarget
    (:then
      (Class|AISensePrediction|RequestPawnPredictionEvent self (Variables|WeaponLogic|Targets|GetAssignedContact) (Variables|WeaponLogic|Tracking|GetPrediction%20Time)))
    (:else)))

(event EventFireWeapon
  (bind _returnvalue (Transformation|GetActorTransform))
  (bind _bp_weaponsystem_ac (Variables|Default|GetBP_WeaponSystem_AC))
  (bind _shotindex (Variables|WeaponLogic|Ammo|GetShotIndex))
  (bind _ammopool (Variables|Initialization|WeaponCreation|Ammo|GetAmmoPool))
  (bind _output (Utilities|Array|Get(acopy) _ammopool _shotindex))
  ;[0.15 0.15 0.15 0.5] Fire Bullet and track the shot count to determine when to reload
  (bind _weaponinposition (Class|BPIWeaponSystem|GetWeaponinPosition(Message) (Components|GetOwner (Components|GetChildComponent (Variables|Default|GetWeapon_ChildActor) 0))))
  (if _weaponinposition
    (Variables|WeaponLogic|Ammo|SetBurstIndex (Class|BlackboardComponent|GetValueasInt (Variables|AI|GetAIBlackboard) (Utilities|Name|MakeLiteralName "BurstIndex")))
    (Utilities|IsValid _output
      (:Is%20Valid
        (Class|BPIProjectile|InUse?(Message) _output)
        (bind _assignedcontact (Variables|WeaponLogic|Targets|GetAssignedContact)
          (:then
            (Class|BPIProjectile|SetStartTransform(Message) _output _returnvalue)
            (bind (_targetvelocity _fusetime) (CallFunction|CalculateBulletSpread _returnvalue))
            (Class|BPIProjectile|Fire(Message) _output _assignedcontact _targetvelocity _fusetime)
            (Default|EventFire _bp_weaponsystem_ac)
            (Variables|/Game/Blueprints/Components/WeaponSystem/BP_WeaponSystem_AC.BP_WeaponSystem_AC_C|SetCurrentAmmo _bp_weaponsystem_ac (- (Variables|/Game/Blueprints/Components/WeaponSystem/BP_WeaponSystem_AC.BP_WeaponSystem_AC_C|GetCurrentAmmo _bp_weaponsystem_ac) 1))
            (if (>= (+ (Variables|WeaponLogic|Ammo|GetShotIndex) 1) (Variables|/Game/Actors/WeaponSystems/__DataAssets/BP_WeaponSystem_Base_PDA.BP_WeaponSystem_Base_PDA_C|GetMagazineSize (Variables|Default|GetPrimaryDataAsset)))
              (AI|Components|Blackboard|SetValueasBool (Variables|AI|GetAIBlackboard) (Utilities|Name|MakeLiteralName "NeedsReload") true)
              (else
                (Math|Integer|IncrementInt (Variables|WeaponLogic|Ammo|GetShotIndex)
                  (:%20%20
                    (bind _result (Math|Integer|IncrementInt (Variables|WeaponLogic|Ammo|GetBurstIndex))
                      (:%20%20
                        (Class|BlackboardComponent|SetValueasInt (Variables|AI|GetAIBlackboard) (Utilities|Name|MakeLiteralName "BurstIndex") _result))))))))
          (:else))))))

(event EventSetFactionType
  (params (SetFaction :type E_FriendFoe%20Enum :default "NewEnumerator0"))
  (Variables|Initialization|WeaponCreation|SetFaction SetFaction))

(event EventBeginPlay
  ;[0.15 0.15 0.15 0.5] Initialize on Begin Play
  (bind _output_get (Variables|AI|SetAIBlackboard (AI|GetBlackboard (AI|GetAIController self))))
  (Class|BlackboardComponent|SetValueasInt _output_get (Utilities|Name|MakeLiteralName "BurstSize") (Variables|/Game/Actors/WeaponSystems/__DataAssets/BP_WeaponSystem_Base_PDA.BP_WeaponSystem_Base_PDA_C|GetBurstSize (Variables|Default|GetPrimaryDataAsset)))
  (bind (_yaw _pitch _roll) (Class|BPIWeaponSystem|GetMeshComponents(Message) (Components|GetOwner (Components|GetChildComponent (Variables|Default|GetWeapon_ChildActor) 0))))
  (Variables|Debug|SetYawComponent _yaw)
  (Variables|Debug|SetPitchComponent _pitch)
  (Variables|Debug|SetRollComponent _roll))

(fn ConstructionScript
  (bind _primarydataasset (Variables|Default|GetPrimaryDataAsset)
    (:then
      (Initialization|WeaponCreation|UpdateDataAsset _primarydataasset false)
      (Initialization|DataTableWork|SetVariablesfromDataAsset _primarydataasset)
      (Initialization|WeaponCreation|InitHealthVariables _primarydataasset)
      (Default|InitializeAmmo (Variables|Default|GetBP_WeaponSystem_AC) (Variables|/Game/Actors/WeaponSystems/__DataAssets/BP_WeaponSystem_Base_PDA.BP_WeaponSystem_Base_PDA_C|GetMagazineSize _primarydataasset))
      (Components|Box|SetBoxExtent (Variables|Default|GetBox_Collision) (.BoxExtent (Collision|GetComponentBounds (Variables|Default|GetWeapon_ChildActor))) true))
    (:else)))

(fn AttachWeapontoComponent
  (params (Actor :type Actor%20Soft%20Object%20Reference) (Component :type Scene%20Component%20Soft%20Object%20Reference))
  (bind _output (Utilities|ResolveSoftReference Actor))
  (bind _output_2 (Utilities|ResolveSoftReference Component))
  ;[0.15 0.15 0.15 0.5] If both a valid actor and component are provided, then attach the actor to the component and return if it was successful. If either the actor or component was not valid then throw a script error.
  (Utilities|IsValid _output
    (:Is%20Valid
      (Utilities|IsValid _output_2
        (:Is%20Valid
          (bind _returnvalue (Transformation|AttachComponentToComponent _output _output_2 "None" "SnapToTarget" "SnapToTarget" "SnapToTarget" true))
          (return _returnvalue))
        (:Is%20Not%20Valid
          (CallFunction|ThrowScriptError "BP_WeaponParent_Base" "AttachWeaponToComponent" "No valid component was passed" "Scene Component" (Utilities|Text|ToText(Object) _output_2)))))
    (:Is%20Not%20Valid
      (CallFunction|ThrowScriptError "BP_WeaponParent_Base" "AttachWeaponToComponent" "No valid actor was passed" "Actor" (Utilities|Text|ToText(Object) _output)))))

(fn UpdateDataAssetfromTable
  (params (DataTableRow :type S%20Ship%20Configurations%20Structure) (ShipComponent :type S%20Ship%20Component%20Structure) (NewDataAsset :type Primary%20Data%20Asset%20Soft%20Object%20Reference))
  (bind _shipcomponents (Utilities|Struct|BreakS_ShipConfigurations DataTableRow))
  (bind _returnvalue (Utilities|Array|FindItem _shipcomponents ShipComponent))
  (bind _output (Utilities|Array|Get(acopy) _shipcomponents _returnvalue))
  (bind (_attachmentpoint _componentbaseclass _previousdataasset _currentdataasset _nextdataasset _actorcomponentreference _componenttype) (Utilities|Struct|BreakS_ShipComponent _output))
  ;[0.15 0.15 0.15 0.5] Take a row from a data table, find the specified component struct that needs updated and then set its data asset value to the passed one, return if the update was successful or not. If no component struct can be found on the ship, throw an error message and return False.
  (if (Utilities|Array|ContainsItem _shipcomponents ShipComponent)
    (LocalVariables|SetIndexOfComponent _returnvalue)
    (Utilities|Array|SetArrayElem _shipcomponents (LocalVariables|GetIndexOfComponent) (Utilities|Struct|MakeS_ShipComponent _attachmentpoint _componentbaseclass 0 (Utilities|ResolveSoftReference NewDataAsset) 0 0 _componenttype))
    (LocalVariables|SetUpdatedSuccessfully true)
    (else
      (CallFunction|ThrowScriptError "BP_WeaponParent_Base" "UpdateDataAssetFromTable" "The specified array struct item was not contained in the provided table row." "" "")
      (LocalVariables|SetUpdatedSuccessfully false)))
  (return (LocalVariables|GetUpdatedSuccessfully)))

(fn GetSceneComponentfromStructName
  (params (StructName :type Name))
  ;[0.15 0.15 0.15 0.5] Get the actor that owns the weapon, it should be BP_PlayerShip, and then search its components for one with the desired tag. Return the actual scene component reference instead of just its tag
  (return (Class|Actor|FindComponentbyTag (Components|GetOwner) "/Script/Engine.SceneComponent" StructName)))

(fn SetVariablesfromDataAsset
  (params (PrimaryDataAsset :type BP%20Weapon%20System%20Base%20PDA%20Object%20Reference))
  (Variables|Default|SetWeaponSystem_CoreInfo (Utilities|Struct|MakeS_WeaponSystem_CoreInfo (Variables|/Game/Actors/WeaponSystems/__DataAssets/BP_WeaponSystem_Base_PDA.BP_WeaponSystem_Base_PDA_C|GetWeaponName PrimaryDataAsset) (Variables|/Game/Actors/WeaponSystems/__DataAssets/BP_WeaponSystem_Base_PDA.BP_WeaponSystem_Base_PDA_C|GetAttachmentPoint PrimaryDataAsset) (Utilities|ResolveSoftReference (Variables|/Game/Actors/WeaponSystems/__DataAssets/BP_WeaponSystem_Base_PDA.BP_WeaponSystem_Base_PDA_C|GetWeaponClass PrimaryDataAsset)) (Variables|/Game/Actors/WeaponSystems/__DataAssets/BP_WeaponSystem_Base_PDA.BP_WeaponSystem_Base_PDA_C|GetReputationCost PrimaryDataAsset) (Variables|/Game/Actors/WeaponSystems/__DataAssets/BP_WeaponSystem_Base_PDA.BP_WeaponSystem_Base_PDA_C|GetWeaponType PrimaryDataAsset)))
  (Variables|Default|SetWeaponSystem_InfoPrivate (Utilities|Struct|MakeS_WeaponSystem_PrivateInfo (Variables|/Game/Actors/WeaponSystems/__DataAssets/BP_WeaponSystem_Base_PDA.BP_WeaponSystem_Base_PDA_C|GetProjectileType PrimaryDataAsset) (Variables|/Game/Actors/WeaponSystems/__DataAssets/BP_WeaponSystem_Base_PDA.BP_WeaponSystem_Base_PDA_C|GetEngagementType PrimaryDataAsset) (Variables|/Game/Actors/WeaponSystems/__DataAssets/BP_WeaponSystem_Base_PDA.BP_WeaponSystem_Base_PDA_C|GetTrackingSpeed PrimaryDataAsset) (Variables|/Game/Actors/WeaponSystems/__DataAssets/BP_WeaponSystem_Base_PDA.BP_WeaponSystem_Base_PDA_C|GetMagazineSize PrimaryDataAsset) (Variables|/Game/Actors/WeaponSystems/__DataAssets/BP_WeaponSystem_Base_PDA.BP_WeaponSystem_Base_PDA_C|GetReloadTime PrimaryDataAsset)))
  (Variables|Default|SetWeaponSystem_InfoPublic (Utilities|Struct|MakeS_WeaponSystem_PublicInfo (Variables|/Game/Actors/WeaponSystems/__DataAssets/BP_WeaponSystem_Base_PDA.BP_WeaponSystem_Base_PDA_C|GetTrackingRange PrimaryDataAsset) (Variables|/Game/Actors/WeaponSystems/__DataAssets/BP_WeaponSystem_Base_PDA.BP_WeaponSystem_Base_PDA_C|GetEngagementRange PrimaryDataAsset) (Variables|/Game/Actors/WeaponSystems/__DataAssets/BP_WeaponSystem_Base_PDA.BP_WeaponSystem_Base_PDA_C|GetAutoFire PrimaryDataAsset) (Variables|/Game/Actors/WeaponSystems/__DataAssets/BP_WeaponSystem_Base_PDA.BP_WeaponSystem_Base_PDA_C|GetAutoTracking PrimaryDataAsset) (Variables|/Game/Actors/WeaponSystems/__DataAssets/BP_WeaponSystem_Base_PDA.BP_WeaponSystem_Base_PDA_C|GetDestroyed PrimaryDataAsset) (Variables|/Game/Actors/WeaponSystems/__DataAssets/BP_WeaponSystem_Base_PDA.BP_WeaponSystem_Base_PDA_C|GetMaxHealth PrimaryDataAsset) (Variables|/Game/Actors/WeaponSystems/__DataAssets/BP_WeaponSystem_Base_PDA.BP_WeaponSystem_Base_PDA_C|GetDamaged PrimaryDataAsset)))
  (bind _asprojectile_pda (CallFunction|GetProjectilefromWeapon PrimaryDataAsset))
  (Variables|Initialization|WeaponCreation|Ammo|SetAmmoDataAsset _asprojectile_pda))

(fn UpdateDataAsset
  (params (HardData :type Primary%20Data%20Asset%20Object%20Reference) (UseSoftData :type Boolean) (SoftData :type Primary%20Data%20Asset%20Soft%20Object%20Reference))
  (if UseSoftData
    (bind _returnvalue (Utilities|LoadAssetBlocking SoftData))
    (bind _asbp_weapon_system_base_pda (Utilities|Casting|CastToBP_WeaponSystem_Base_PDA _returnvalue))
    (bind _returnvalue_2 (Utilities|LoadClassAssetBlocking (Variables|/Game/Actors/WeaponSystems/__DataAssets/BP_WeaponSystem_Base_PDA.BP_WeaponSystem_Base_PDA_C|GetWeaponClass _asbp_weapon_system_base_pda)))
    (bind _asactor (Utilities|Casting|CastToActorClass _returnvalue_2))
    (ChildActorComponent|SetChildActorClass (Variables|Default|GetWeapon_ChildActor) _asactor)
    (return _asbp_weapon_system_base_pda)
    (else
      (bind _asbp_weapon_system_base_pda_2 (Utilities|Casting|CastToBP_WeaponSystem_Base_PDA HardData))
      (bind _returnvalue_3 (Utilities|LoadClassAssetBlocking (Variables|/Game/Actors/WeaponSystems/__DataAssets/BP_WeaponSystem_Base_PDA.BP_WeaponSystem_Base_PDA_C|GetWeaponClass _asbp_weapon_system_base_pda_2)))
      (bind _asactor_2 (Utilities|Casting|CastToActorClass _returnvalue_3))
      (ChildActorComponent|SetChildActorClass (Variables|Default|GetWeapon_ChildActor) _asactor_2)
      (return _asbp_weapon_system_base_pda_2))))

(fn GetDataforUI
  (return (Variables|Default|GetWeaponSystem_CoreInfo) (Variables|Default|GetWeaponSystem_InfoPrivate) (Variables|Default|GetWeaponSystem_InfoPublic)))

(fn SetWeaponType
  (params (SetWeaponType :type WeaponSystem_SystemType_Enum%20Enum :default "NewEnumerator0"))
  (return SetWeaponType))

(fn GetDataAssetsBasedonType
  (switch Utilities|FlowControl|Switch|SwitchonWeaponSystem_SystemType_Enum (DataManagement|SetWeaponType "NewEnumerator0")
    (:NewEnumerator0
      (bind _returnvalue (Utilities|GetDataTableRow "/Game/Actors/WeaponSystems/__DataAssets/DT_AvailableDataAssets.DT_AvailableDataAssets" "Offensive")
        (:then
          (bind _output_get (Variables|Default|SetSoftDataAssetArray (Utilities|Struct|BreakS_AvailableDataAssets _returnvalue)))
          (bind _returnvalue_2 (Utilities|LoadAssetBlocking (Utilities|Array|Get(acopy) _output_get (Math|Integer|Clamp(Integer) (Variables|Default|GetDataAsset) 0 (Utilities|Array|LastIndex _output_get)))))
          (bind _asbp_weapon_system_base_pda (Utilities|Casting|CastToBP_WeaponSystem_Base_PDA _returnvalue_2))
          (Variables|Default|SetPrimaryDataAsset _asbp_weapon_system_base_pda))))
    (:NewEnumerator1
      (bind _returnvalue_3 (Utilities|GetDataTableRow "/Game/Actors/WeaponSystems/__DataAssets/DT_AvailableDataAssets.DT_AvailableDataAssets" "Defensive")
        (:then
          (bind _output_get_2 (Variables|Default|SetSoftDataAssetArray (Utilities|Struct|BreakS_AvailableDataAssets _returnvalue_3)))
          (bind _returnvalue_4 (Utilities|LoadAssetBlocking (Utilities|Array|Get(acopy) _output_get_2 (Math|Integer|Clamp(Integer) (Variables|Default|GetDataAsset) 0 (Utilities|Array|LastIndex _output_get_2)))))
          (bind _asbp_weapon_system_base_pda_2 (Utilities|Casting|CastToBP_WeaponSystem_Base_PDA _returnvalue_4))
          (Variables|Default|SetPrimaryDataAsset _asbp_weapon_system_base_pda_2))))
    (:NewEnumerator2
      (bind _returnvalue_5 (Utilities|GetDataTableRow "/Game/Actors/WeaponSystems/__DataAssets/DT_AvailableDataAssets.DT_AvailableDataAssets" "MissileLaunchers")
        (:then
          (bind _output_get_3 (Variables|Default|SetSoftDataAssetArray (Utilities|Struct|BreakS_AvailableDataAssets _returnvalue_5)))
          (bind _returnvalue_6 (Utilities|LoadAssetBlocking (Utilities|Array|Get(acopy) _output_get_3 (Math|Integer|Clamp(Integer) (Variables|Default|GetDataAsset) 0 (Utilities|Array|LastIndex _output_get_3)))))
          (bind _asbp_weapon_system_base_pda_3 (Utilities|Casting|CastToBP_WeaponSystem_Base_PDA _returnvalue_6))
          (Variables|Default|SetPrimaryDataAsset _asbp_weapon_system_base_pda_3))))))

(fn InitHealthVariables
  (params (Primary%20Data%20Asset :type BP%20Weapon%20System%20Base%20PDA%20Object%20Reference))
  (Default|SetStartingHealth (Variables|Default|GetBP_Health_AC) (Variables|/Game/Actors/WeaponSystems/__DataAssets/BP_WeaponSystem_Base_PDA.BP_WeaponSystem_Base_PDA_C|GetMaxHealth Primary%20Data%20Asset)))

(fn ChangeWeaponThroughDataAsset
  (params (DataAsset :type Primary%20Data%20Asset%20Object%20Reference))
  (bind _primarydataasset (Initialization|WeaponCreation|UpdateDataAsset DataAsset false))
  (Initialization|DataTableWork|SetVariablesfromDataAsset _primarydataasset)
  (Initialization|WeaponCreation|InitHealthVariables _primarydataasset))

(fn ClearAssignment
  (bind _aiblackboard (Variables|AI|GetAIBlackboard))
  (Variables|WeaponLogic|Targets|SetAssignedContact 0)
  (AI|Components|Blackboard|SetValueasObject _aiblackboard (Utilities|Name|MakeLiteralName "TargetActor") 0)
  (AI|Components|Blackboard|SetValueasBool _aiblackboard (Utilities|Name|MakeLiteralName "TargetDestroyed") false))

(fn CalculateBulletSpread
  (params (StartingTransform :type Transform%20%28by%20ref%29))
  (bind _returnvalue (Utilities|Name|MakeLiteralName "PredictedTargetLocation"))
  (bind _aiblackboard (Variables|AI|GetAIBlackboard))
  (bind _ammodataasset (Variables|Initialization|WeaponCreation|Ammo|GetAmmoDataAsset))
  (bind _returnvalue_2 (AI|Components|Blackboard|GetValueasVector _aiblackboard _returnvalue))
  (bind _speed (Variables|/Game/Actors/WeaponSystems/Projectiles/__DataAssets/Projectile_PDA.Projectile_PDA_C|GetSpeed _ammodataasset))
  (Variables|/Game/Actors/WeaponSystems/__DataAssets/BP_WeaponSystem_Base_PDA.BP_WeaponSystem_Base_PDA_C|GetUsePredictiveLocation (Variables|Default|GetPrimaryDataAsset)
    (:then
      ;[0.15 0.15 0.15 0.5] Fire at the predicted location of the target
      (if (> (Math|Vector|VectorLength _returnvalue_2) 1.0)
        (LocalVariables|SetTargetVector _returnvalue_2)
        (else
          (LocalVariables|SetTargetVector (- (Transformation|GetActorLocation (Variables|WeaponLogic|Targets|GetAssignedContact)) (Transformation|GetActorLocation self)))))
      (Development|PrintString (Utilities|String|ToString(Vector) (+ (LocalVariables|GetTargetVector) (Transformation|GetVelocity (Variables|Default|GetAttachedPlatform)))))
      (return (CallFunction|MakeBulletSpread (+ (LocalVariables|GetTargetVector) (Transformation|GetVelocity (Variables|Default|GetAttachedPlatform))) (Variables|/Game/Actors/WeaponSystems/__DataAssets/BP_WeaponSystem_Base_PDA.BP_WeaponSystem_Base_PDA_C|GetWeaponSpread (Variables|Default|GetPrimaryDataAsset))) (+ (/ (Math|Vector|Distance(Vector) (.Location (Math|Transform|BreakTransform StartingTransform)) (Transformation|GetActorLocation (Variables|WeaponLogic|Targets|GetAssignedContact))) (Variables|/Game/Actors/WeaponSystems/Projectiles/__DataAssets/Projectile_PDA.Projectile_PDA_C|GetSpeed (Variables|Initialization|WeaponCreation|Ammo|GetAmmoDataAsset))) (Math|Random|RandomFloatinRange 0.0 0.2))))
    (:else
      (bind _pitch (Class|BPIWeaponSystem|GetMeshComponents(Message) (Components|GetOwner (Components|GetChildComponent (Variables|Default|GetWeapon_ChildActor) 0))))
      ;[0.15 0.15 0.15 0.5] Get Velocity from the current location of the target
      (return (CallFunction|MakeBulletSpread (+ (Transformation|GetVelocity (Variables|Default|GetAttachedPlatform)) (* (Math|Vector|GetForwardVector _pitch) _speed)) (Variables|/Game/Actors/WeaponSystems/__DataAssets/BP_WeaponSystem_Base_PDA.BP_WeaponSystem_Base_PDA_C|GetWeaponSpread (Variables|Default|GetPrimaryDataAsset))) (+ (/ (Math|Vector|Distance(Vector) (.Location (Math|Transform|BreakTransform StartingTransform)) (Transformation|GetActorLocation (Variables|WeaponLogic|Targets|GetAssignedContact))) _speed) (Math|Random|RandomFloatinRange 0.0 0.2))))))

(fn CalculateTargetVelocity
  (params (StartingTransform :type Transform%20%28by%20ref%29) (AssignedContact :type Actor%20Object%20Reference))
  (bind _ammodataasset (Variables|Initialization|WeaponCreation|Ammo|GetAmmoDataAsset))
  (bind _speed (Variables|/Game/Actors/WeaponSystems/Projectiles/__DataAssets/Projectile_PDA.Projectile_PDA_C|GetSpeed _ammodataasset))
  (bind _pitch (Class|BPIWeaponSystem|GetMeshComponents(Message) (Components|GetOwner (Components|GetChildComponent (Variables|Default|GetWeapon_ChildActor) 0))))
  (return (* (Math|Vector|GetUpVector _pitch) _speed) (+ (/ (Math|Vector|Distance(Vector) (.Location (Math|Transform|BreakTransform StartingTransform)) (Transformation|GetActorLocation AssignedContact)) _speed) (Math|Random|RandomFloatinRange 0.0 0.2))))

(fn CreateAmmoPool
  (bind _tempignorearray (LocalVariables|GetTempIgnoreArray))
  (for _index (range 0 (- (Variables|/Game/Actors/WeaponSystems/__DataAssets/BP_WeaponSystem_Base_PDA.BP_WeaponSystem_Base_PDA_C|GetMagazineSize (Variables|Default|GetPrimaryDataAsset)) 1))
    (bind _returnvalue (Game|SpawnActorfromClass "/Game/Actors/WeaponSystems/Projectiles/BP_Projectile_Base.BP_Projectile_Base_C" (Transformation|GetActorTransform) "AlwaysSpawn" "MultiplyWithRoot" 0 (Variables|Initialization|WeaponCreation|Ammo|GetAmmoDataAsset) 0))
    (Utilities|Array|AddUnique (Variables|Initialization|WeaponCreation|Ammo|GetAmmoPool) _returnvalue))
  (bind _master_ai (Variables|AI|GetMaster%20AI)
    (:then
      (bind _defensiveweapons (Class|BPIWeaponController|GetAllDefensiveWeapons(Message) _master_ai))
      (Utilities|Array|AppendArray (LocalVariables|GetTempIgnoreArray) _defensiveweapons)
      (bind _offensiveweapons (Class|BPIWeaponController|GetAllOffensiveWeapons(Message) _master_ai))
      (Utilities|Array|AppendArray (LocalVariables|GetTempIgnoreArray) _offensiveweapons)
      (bind _missileweapons (Class|BPIWeaponController|GetAllMissileWeapons(Message) _master_ai))
      (Utilities|Array|AppendArray _tempignorearray _missileweapons))
    (:else
      _))
  (Utilities|Array|AddUnique _tempignorearray self)
  (for _array_element (Variables|Initialization|WeaponCreation|Ammo|GetAmmoPool)
    (Class|BPIProjectile|SetIgnoreActors(Message) _array_element "NewEnumerator0" (LocalVariables|GetTempIgnoreArray)))
  (return true))

(fn GetFactionType
  (return (Variables|Initialization|WeaponCreation|GetFaction)))

(fn GetMeshComponents
  (return 0 0 0))

(fn GetPlatformComponents
  (return (Variables|Default|GetAttachedPlatform) (Variables|Default|GetAttachedPlatformComponents)))

(fn GetProjectileStart
  (return ""))

(fn GetTargetable
  (return (Variables|Default|GetTargetable)))

(fn GetTargetableType
  (return "NewEnumerator3"))

(fn GetWeaponinPosition
  (return false))

(fn InRange
  (params (Contact :type Actor%20Object%20Reference))
  (return false))

(fn NeedsReload
  (if (>= (Variables|Initialization|WeaponCreation|Ammo|GetCurrentShotIndex) (Variables|Initialization|WeaponCreation|Ammo|GetMagazineSize))
    (return true)))