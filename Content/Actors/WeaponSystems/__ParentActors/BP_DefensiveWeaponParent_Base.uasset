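; Base Blueprint for defensive weapon systems, extending a parent weapon class and overriding its weapon type with a fixed value.
; When a contact is destroyed, it runs the parent logic, then, if IsSlave is valid, notifies MasterAI to update defensive assignments and clears its assigned contact.
; Target sorting, priority selection and target-map calls remain in the event graph as unconnected, never-executed nodes.
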(event EventContactDestroyed
  (|CallParentFunction)
  (Variables|Default|GetIs%20Slave
    (:then
      (Class|BPIWeaponController|UpdateDefensiveAssignments(Message) (Variables|Default|GetMaster%20AI) "NewEnumerator2" self)
      (Variables|Default|SetAssignedContact 0))
    (:else)))

(fn ConstructionScript
  (|CallParentFunction))

(fn SetWeaponType
  (params (SetWeaponType :type WeaponSystem_SystemType_Enum%20Enum :default "NewEnumerator0"))
  (return (|CallParentFunction "NewEnumerator1")))