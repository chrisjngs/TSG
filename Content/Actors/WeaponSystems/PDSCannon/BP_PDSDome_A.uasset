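; BP_PDSDome_A is the A variant of the PDS cannon dome actor among the game's weapon systems.
; It is a thin child Blueprint whose BeginPlay only calls the parent.
; Its construction script runs the parent's, then calls UpdateDataAsset with its primary data asset as a hard reference rather than soft data.
; Unwired debug nodes for printing and drawing the spawn location remain in the graph.
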(event EventBeginPlay
  (|CallParentFunction))

(fn ConstructionScript
  (|CallParentFunction)
  (CallFunction|UpdateDataAsset (Variables|Default|GetPrimaryDataAsset) false))