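; Test flak cannon weapon actor that supports hover inspection and click customization, with logic intended to move into a weapon parent class.
; Cursor hover has BPWeaponSystemAC show a data-asset-driven popup and highlight the weapon, while clicks forward to BPCustomizableAC.
; The construction script hardcodes weapon stats, read only by a local popup function the hover events bypass.
; CycleDataAsset only prints attachment-hierarchy debug names, and PauseRotate is an empty stub.
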(event MouseInput|EventActorBeginCursorOver
  (bind _bp_weaponsystem_ac (Variables|Default|GetBP_WeaponSystem_AC))
  ;[0.15 0.15 0.15 0.5] All of this should go into the Weapon Parent Class for the official build, that way every weapon will be able to opporate the same without having to duplicate the logic
  ;;[0.15 0.15 0.15 0.5] Logic for creating the hover events. First create the widget, then add the information to it, and highlight the actor components
  (Default|EventGenerateWidget _bp_weaponsystem_ac (Utilities|ResolveSoftReference self) (Utilities|ResolveSoftReference (Variables|Default|GetWidget_Location)))
  (Default|RenderInteractionWidget :self _bp_weaponsystem_ac :SystemInfo (Variables|Default|GetDataAsset))
  (Default|HighlightSelectionon _bp_weaponsystem_ac self))

(event MouseInput|EventActorOnClicked
  (params (ButtonPressed :type Key%20Structure))
  (Default|ComponentClickedEvent (Variables|Default|GetBP_Customizable_AC) (Utilities|ResolveSoftReference self)))

(event MouseInput|EventActorEndCursorOver
  (bind _bp_weaponsystem_ac (Variables|Default|GetBP_WeaponSystem_AC))
  ;[0.15 0.15 0.15 0.5] All of this should go into the Weapon Parent Class for the official build, that way every weapon will be able to opporate the same without having to duplicate the logic
  ;;[0.15 0.15 0.15 0.5] Logic for creating the hover events. First create the widget, then add the information to it, and highlight the actor components
  ;;;[0.15 0.15 0.15 0.5] Remove the widget and highlight selection
  (Default|HighlightSelectionOff _bp_weaponsystem_ac self)
  (bind _widget (Variables|/Game/Blueprints/Components/WeaponSystem/BP_WeaponSystem_AC.BP_WeaponSystem_AC_C|GetWidget (Variables|Default|GetBP_WeaponSystem_AC))
    (:then
      (Default|RemoveInteractionWidget _bp_weaponsystem_ac _widget))
    (:else)))

(fn ConstructionScript
  (Variables|Default|SetWeaponSystemInfo (Utilities|Struct|MakeWeaponSystem_Base_Struct "Flack Cannon" "None" "NewEnumerator0" "NewEnumerator0" 1000 true 500 3e+01 false 5e+02 7.5e+02)))

(fn RenderInteractionWidget
  (bind _widget_location (Variables|Default|GetWidget_Location))
  (bind _returnvalue (UserInterface|CreateWidget "/Game/HUD/PremadeWidgets/BPW_HoverPopup.BPW_HoverPopup_C"))
  (bind _output_get (Variables|Default|SetHoverPopup _returnvalue))
  (UserInterface|SetWidget _widget_location _output_get)
  (Transformation|SetWorldLocation _widget_location (Transformation|GetWorldLocation (Variables|Default|GetWidget_Location)) false false)
  (Rendering|Components|TextRender|SetText (Variables|/Game/HUD/PremadeWidgets/BPW_HoverPopup.BPW_HoverPopup_C|GetTitle_Text _output_get) (.name (Variables|Default|GetWeaponSystemInfo))))

(fn CycleDataAsset
  (params (DataTable :type Primary%20Data%20Asset%20Object%20Reference) (ClickedComponent :type Boolean))
  (bind _self self)
  (bind _returnvalue (Class|Actor|GetParentComponent _self))
  (Development|PrintString (Utilities|GetDisplayName (Transformation|GetAttachParent _returnvalue)) true true "(R=0.000000,G=0.660000,B=1.000000,A=1.000000)" 3e+01)
  (Development|PrintString (Utilities|GetDisplayName _returnvalue) true true "(R=1.000000,G=0.223055,B=0.524958,A=1.000000)" 3e+01)
  (Development|PrintString (Utilities|GetDisplayName (Actor|GetAttachParentActor _self)) true true "(R=0.014920,G=1.000000,B=0.576665,A=1.000000)" 3e+01)
  (Development|PrintString (Utilities|GetDisplayName _self) true true "(R=1.000000,G=0.570051,B=0.000000,A=1.000000)" 3e+01))

(fn ComponentType
  (return "NewEnumerator0"))

(fn PauseRotate
  (params (Rotate :type Boolean))
  (return))