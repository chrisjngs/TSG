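; Test missile actor that is launched by physics force, can home on a target, and explodes on overlap to deal radial damage.
; When Tracking is valid, a looping timer turns the missile toward TrackingTarget and pushes it that way.
; Overlaps ignore ping spheres and ProxyEnemyShip-tagged actors with their children.
; An impact spawns a proxy explosion, damages nearby health-interface actors, destroys the missile if any are found, and calls MissileExplode.
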(event Custom|Event_UpdateTargetTracking
  (CallFunction|UpdateTracking))

(event Collision|EventActorBeginOverlap
  (params (OtherActor :type Actor%20Object%20Reference))
  (bind _missile (Variables|Default|GetMissile))
  (bind _damageradius (Variables|Default|GetDamageRadius))
  (if (not (== (Utilities|GetClass OtherActor) "/Game/Blueprints/Components/PingSystem/BP_PingSphere.BP_PingSphere_C"))
    (if (not (Utilities|Array|ContainsItem (Variables|Default|GetActorsToIgnore) OtherActor))
      (Development|PrintString (Utilities|String|ToString(Text) (Utilities|Text|FormatText "Collided with actor \"{actor}\"" OtherActor)))
      (Game|SpawnActorfromClass "/Game/Actors/WeaponSystems/Missiles/BP_ProxyExplosion.BP_ProxyExplosion_C" (Transformation|GetWorldTransform _missile) "AlwaysSpawn" "MultiplyWithRoot" 0 _damageradius 0)
      (bind _outactors (Collision|SphereOverlapActors (Transformation|GetWorldLocation _missile) _damageradius (Variables|Default|GetValidObjectTypes) 0 (Variables|Default|GetActorsToIgnore)))
      (for _array_element _outactors
        (if (Utilities|DoesObjectImplementInterface _array_element "/Game/Blueprints/Components/HealthSystem/BPI_HealthInterface.BPI_HealthInterface_C")
          (Class|BPIHealthInterface|TakeDamage(Message) _array_element (Variables|Default|GetDamageAmount))
          (Actor|DestroyActor)))
      (Default|CallMissileExplode))))

(event EventBeginPlay
  (bind _outactors (Actor|GetAllActorswithTag "ProxyEnemyShip"))
  (Utilities|Array|AppendArray (Variables|Default|GetActorsToIgnore) _outactors)
  (for _array_element _outactors
    (Utilities|Array|AppendArray (Variables|Default|GetActorsToIgnore) (Actor|GetAllChildActors _array_element true)))
  (Variables|Default|GetTracking
    (:then
      (Utilities|Time|SetTimerbyEvent (delegate Custom|Event_UpdateTargetTracking) 0.5 true))
    (:else)))

(fn ConstructionScript
  (Transformation|AttachComponentToComponent (Variables|Default|GetCollision) (Variables|Default|GetMissile) "None" "KeepWorld" "KeepWorld" "KeepWorld" true))

(fn LaunchMissileFunc
  (params (Force%20Vector :type Vector) (Force%20Amount :type Float%20%28double-precision%29))
  (Physics|AddForce (Variables|Default|GetMissile) (* Force%20Vector Force%20Amount) "None" true))

(fn UpdateTracking
  (bind _missile (Variables|Default|GetMissile))
  (bind _trackingtarget (Variables|Default|GetTrackingTarget))
  (bind _returnvalue (Transformation|GetWorldTransform _trackingtarget))
  (bind _returnvalue_2 (Transformation|GetWorldLocation _missile))
  (bind _returnvalue_3 (Math|Rotator|FindLookatRotation _returnvalue_2 (.location _returnvalue)))
  (bind _missile_2 (Variables|Default|GetMissile)
    (:then
      (Transformation|SetWorldRotation _missile_2 _returnvalue_3 false false)
      (bind _missile_3 (Variables|Default|GetMissile)
        (:then
          (Physics|AddForce _missile_3 (* (Math|Vector|GetForwardVector _returnvalue_3) 5e+05) "None" true)
          (Collision|LineTraceByChannel _returnvalue_2 (.location _returnvalue) "TraceTypeQuery1" false 0 "ForOneFrame"))
        (:else
          (Development|PrintString "Missile is not valid"))))
    (:else)))