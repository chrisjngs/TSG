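; Placeholder-style explosion visual for the missile weapon system, built from three spheres and a point light.
; The construction script sets the light's attenuation radius to ExplosionRadius and scales each sphere from it by slightly different divisors, so the spheres differ in relative scale.
; The actor destroys itself half a second after BeginPlay and applies no damage or other gameplay effect in its graphs.
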(event EventBeginPlay
  (Utilities|FlowControl|Delay 0.5)
  (Actor|DestroyActor))

(fn ConstructionScript
  (bind _explosionsphere_002 (Variables|Default|GetExplosionSphere_002))
  (bind _explosionsphere_003 (Variables|Default|GetExplosionSphere_003))
  (bind _explosionsphere_001 (Variables|Default|GetExplosionSphere_001))
  (Rendering|Lighting|SetAttenuationRadius (Variables|Default|GetPointLight) (Variables|Default|GetExplosionRadius))
  (Transformation|SetWorldScale3D _explosionsphere_001 (* (Transformation|GetWorldScale _explosionsphere_001) (/ (Variables|Default|GetExplosionRadius) 5e+01)))
  (Transformation|SetWorldScale3D _explosionsphere_002 (* (Transformation|GetWorldScale _explosionsphere_002) (/ (Variables|Default|GetExplosionRadius) 55.0)))
  (Transformation|SetWorldScale3D _explosionsphere_003 (* (Transformation|GetWorldScale _explosionsphere_003) (/ (Variables|Default|GetExplosionRadius) 49.0))))