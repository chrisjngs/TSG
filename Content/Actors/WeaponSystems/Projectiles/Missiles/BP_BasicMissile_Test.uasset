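; Test homing missile actor, apparently reusable through an InUse state, that can itself be targeted.
; Fire launches it at a given velocity, then after a short delay enables collision, faces the target and starts homing.
; A looping timer re-aims velocity with random spread until within range, alongside safe-distance and lifetime timers.
; Detonation spawns a proxy explosion and damages health-interface actors in a sphere; unarmed contact deals only reduced direct damage.
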(event OnComponentBeginOverlap(Capsule_Collision)
  (params (OverlappedComponent :type Primitive%20Component%20Object%20Reference) (OtherActor :type Actor%20Object%20Reference) (OtherComp :type Primitive%20Component%20Object%20Reference) (OtherBodyIndex :type Integer) (bFromSweep :type Boolean) (SweepResult :type Hit%20Result%20Structure%20%28by%20ref%29))
  (bind _ammodataasset (Variables|Default|GetAmmoDataAsset))
  (bind _proximityradius (Variables|/Game/Actors/WeaponSystems/Projectiles/__DataAssets/Projectile_PDA.Projectile_PDA_C|GetProximityRadius _ammodataasset))
  ;[0.15 0.15 0.15 0.5] Explosion on Contact
  (if (not (== OtherActor self))
    (Variables|Default|GetSafeDistance
      (:then
        (Game|SpawnActorfromClass "/Game/Actors/WeaponSystems/Projectiles/Missiles/BP_ProxyExplosion.BP_ProxyExplosion_C" (Transformation|GetActorTransform) "Undefined" "MultiplyWithRoot" 0 _proximityradius 0)
        (bind _outactors (Collision|SphereOverlapActors (Transformation|GetActorLocation) _proximityradius (Utilities|Array|MakeArray "ObjectTypeQuery2" "ObjectTypeQuery1" "ObjectTypeQuery3") 0))
        (for _array_element _outactors
          (if (Utilities|DoesObjectImplementInterface _array_element "/Game/Blueprints/Components/HealthSystem/BPI_HealthInterface.BPI_HealthInterface_C")
            (Class|BPIHealthInterface|TakeDamage(Message) _array_element (Variables|/Game/Actors/WeaponSystems/Projectiles/__DataAssets/Projectile_PDA.Projectile_PDA_C|GetDamage (Variables|Default|GetAmmoDataAsset))))
          (CallFunction|InUse?)
          (CallFunction|SetTargetable false)))
      (:else
        (Class|BPIHealthInterface|TakeDamage(Message) OtherActor (/ (Variables|/Game/Actors/WeaponSystems/Projectiles/__DataAssets/Projectile_PDA.Projectile_PDA_C|GetDamage (Variables|Default|GetAmmoDataAsset)) 1e+01))
        (CallFunction|InUse?)
        (CallFunction|SetTargetable false)))))

(event Custom|Event_DistanceBurn
  (bind _returnvalue (Transformation|GetActorLocation))
  (bind _target_actor (Variables|Default|GetTarget%20Actor))
  (bind _projectilemovement (Variables|Default|GetProjectileMovement))
  (bind _target_actor_2 (Variables|Default|GetTarget%20Actor))
  (bind _returnvalue_2 (Transformation|GetVelocity _target_actor))
  (bind _returnvalue_3 (Transformation|GetActorLocation _target_actor_2))
  (bind _predictedlocation (CallFunction|MakeBulletSpread _returnvalue_3 4e+03))
  (bind _returnvalue_4 (+ _returnvalue_2 _returnvalue))
  (bind _returnvalue_5 (- _predictedlocation _returnvalue_4))
  ;[0.15 0.15 0.15 0.5] Homing
  (if (<= (CallFunction|GetDistancetoTarget self (Variables|Default|GetTarget%20Actor)) (Variables|Default|GetDesiredRange))
    (Variables|/Script/Engine.MovementComponent|SetVelocity _projectilemovement _returnvalue_5)
    (Utilities|Time|ClearandInvalidateTimerbyHandle (Variables|Projectile|Targeting|GetDistanceBurnTimer))
    (else
      (Variables|/Script/Engine.MovementComponent|SetVelocity _projectilemovement (/ _returnvalue_5 1e+01)))))

(event Custom|Event_ExplodeMissile
  (bind _ammodataasset (Variables|Default|GetAmmoDataAsset))
  (bind _proximityradius (Variables|/Game/Actors/WeaponSystems/Projectiles/__DataAssets/Projectile_PDA.Projectile_PDA_C|GetProximityRadius _ammodataasset))
  ;[0.15 0.15 0.15 0.5] Explosion on Contact
  (Utilities|Time|ClearandInvalidateTimerbyHandle (Variables|Default|GetTimedMissileDeathTimer))
  (Game|SpawnActorfromClass "/Game/Actors/WeaponSystems/Projectiles/Missiles/BP_ProxyExplosion.BP_ProxyExplosion_C" (Transformation|GetActorTransform) "Undefined" "MultiplyWithRoot" 0 _proximityradius 0)
  (bind _outactors (Collision|SphereOverlapActors (Transformation|GetActorLocation) _proximityradius (Utilities|Array|MakeArray "ObjectTypeQuery2" "ObjectTypeQuery1" "ObjectTypeQuery3") 0))
  (for _array_element _outactors
    (if (Utilities|DoesObjectImplementInterface _array_element "/Game/Blueprints/Components/HealthSystem/BPI_HealthInterface.BPI_HealthInterface_C")
      (Class|BPIHealthInterface|TakeDamage(Message) _array_element (Variables|/Game/Actors/WeaponSystems/Projectiles/__DataAssets/Projectile_PDA.Projectile_PDA_C|GetDamage (Variables|Default|GetAmmoDataAsset))))
    (CallFunction|InUse?)
    (CallFunction|SetTargetable false)))

(event EventFire
  (params (TargetActor :type Actor%20Object%20Reference) (TargetVelocity :type Vector :default "0, 0, 0") (FuseTime :type Float%20%28double-precision%29))
  (bind _projectilemovement (Variables|Default|GetProjectileMovement))
  (bind _projectilemovement_2 (Variables|Default|GetProjectileMovement))
  ;[0.15 0.15 0.15 0.5] Launch Missile
  (Variables|Default|SetTarget%20Actor TargetActor)
  (Utilities|FlowControl|Sequence
    (:then_0
      (Variables|Default|SetInUse true)
      (Utilities|Time|ClearandInvalidateTimerbyHandle (Variables|Default|GetSafeDistanceTimer))
      (bind _returnvalue (Utilities|Time|SetTimerbyEvent (EventDispatchers|CreateEvent :!event EventSetSafeDistance) (Variables|/Game/Actors/WeaponSystems/Projectiles/__DataAssets/Projectile_PDA.Projectile_PDA_C|GetMinimumSafeTime (Variables|Default|GetAmmoDataAsset))))
      (Variables|Default|SetSafeDistanceTimer _returnvalue)
      (Transformation|SetActorTransform (Variables|Default|GetStartTransform))
      (Components|Activation|Activate (Variables|Default|GetProjectileMovement) true)
      (Utilities|IsValid (Variables|Default|GetTarget%20Actor)
        (:Is%20Valid
          (Utilities|IsValid _projectilemovement_2
            (:Is%20Valid
              (Variables|/Script/Engine.MovementComponent|SetVelocity _projectilemovement_2 TargetVelocity)
              (Development|SetHiddeninGame (Variables|Character|GetMesh) false true)
              (Utilities|FlowControl|Delay 0.5)
              (Collision|SetCollisionEnabled (Variables|Default|GetCapsule_Collision) "QueryAndPhysics")
              (Variables|/Script/Engine.PrimitiveComponent|SetbGenerateOverlapEvents (Variables|Default|GetCapsule_Collision) true)
              (CallFunction|SetTargetable true)
              (Utilities|IsValid self
                (:Is%20Valid
                  (Utilities|IsValid (Variables|Default|GetTarget%20Actor)
                    (:Is%20Valid
                      (Transformation|SetActorRotation (Math|Rotator|FindLookatRotation (Transformation|GetActorLocation) (Transformation|GetActorLocation (Variables|Default|GetTarget%20Actor))))
                      (CallFunction|DelayedHoming (Variables|Default|GetTarget%20Actor))
                      (bind _returnvalue_2 (Utilities|Time|SetTimerbyEvent (EventDispatchers|CreateEvent :!event Custom|Event_ExplodeMissile) 6e+01))
                      (Variables|Default|SetTimedMissileDeathTimer _returnvalue_2))))))))))
    (:then_1
      ;[0.15 0.15 0.15 0.5] Homing
      (Utilities|FlowControl|DoOnce false) ; enters at Reset
    )))

(event EventBeginPlay
  (Components|Activation|Deactivate (Variables|Default|GetProjectileMovement))
  (Collision|SetCollisionEnabled (Variables|Default|GetCapsule_Collision) "NoCollision"))

(event EventUpdateTargeting
  (params (How? :type E_ArrayModification%20Enum :default "NewEnumerator0") (AddActor :type Actor%20Object%20Reference) (RemoveTarget :type Actor%20Object%20Reference))
  (bind _actorstargeting (Variables|Default|GetActorsTargeting))
  (switch Utilities|FlowControl|Switch|SwitchonE_ArrayModification How?
    (:NewEnumerator2
      (Utilities|Array|Add _actorstargeting AddActor))
    (:NewEnumerator3
      (Utilities|Array|RemoveItem _actorstargeting RemoveTarget))))

(event EventDelayedHoming
  (params (HomingTarget :type Actor%20Object%20Reference))
  (bind _projectilemovement (Variables|Default|GetProjectileMovement))
  ;[0.15 0.15 0.15 0.5] Homing
  (Utilities|IsValid HomingTarget
    (:Is%20Valid
      (Utilities|FlowControl|DoOnce false
        (:Completed
          (Variables|/Script/Engine.ProjectileMovementComponent|SetHomingTargetComponent _projectilemovement (Variables|/Script/Engine.Actor|GetRootComponent HomingTarget))
          (Variables|/Script/Engine.ProjectileMovementComponent|SetbIsHomingProjectile _projectilemovement true)
          (Variables|/Script/Engine.ProjectileMovementComponent|SetHomingAccelerationMagnitude _projectilemovement 7.5e+03)
          (Class|BPITargetable|UpdateTargeting(Message) HomingTarget "NewEnumerator0" self)
          (bind _returnvalue (Utilities|Time|SetTimerbyEvent (delegate Custom|Event_DistanceBurn) 0.1 true))
          (Variables|Projectile|Targeting|SetDistanceBurnTimer _returnvalue))))))

(event EventSetTargetable
  (params (Targetable :type Boolean))
  (Variables|Default|SetTargetable Targetable))

(fn ConstructionScript
  (|CallParentFunction)
  (Variables|/Script/Engine.ProjectileMovementComponent|SetMaxSpeed (Variables|Default|GetProjectileMovement) (* (Variables|/Game/Actors/WeaponSystems/Projectiles/__DataAssets/Projectile_PDA.Projectile_PDA_C|GetSpeed (Variables|Default|GetAmmoDataAsset)) 5e+01)))

(fn GetFactionType
  (return (Variables|Default|GetFaction)))

(fn GetTargetable
  (return (Variables|Default|GetTargetable)))

(fn GetTargetableType
  (return "NewEnumerator2"))