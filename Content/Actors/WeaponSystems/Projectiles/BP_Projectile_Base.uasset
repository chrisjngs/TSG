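; Pooled base projectile for weapon systems, configured by an ammo data asset for speed, mesh, damage, proximity radius and optional health.
; Fire launches it from a stored transform, delays collision and arms a safety timer and fuse.
; Valid capsule hits deal direct damage, while proximity or fuse triggers spawn an explosion with radial damage.
; InUse? resets it for reuse; when health is destroyed, targeting actors are notified first.
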(event OnComponentBeginOverlap(ProximityDetination_Collision)
  (params (OverlappedComponent :type Primitive%20Component%20Object%20Reference) (OtherActor :type Actor%20Object%20Reference) (OtherComp :type Primitive%20Component%20Object%20Reference) (OtherBodyIndex :type Integer) (bFromSweep :type Boolean) (SweepResult :type Hit%20Result%20Structure%20%28by%20ref%29))
  (bind _ammodataasset (Variables|Projectile|Initialize|GetAmmoDataAsset))
  (bind _proximityradius (Variables|/Game/Actors/WeaponSystems/Projectiles/__DataAssets/Projectile_PDA.Projectile_PDA_C|GetProximityRadius _ammodataasset))
  (Variables|Projectile|Update|GetInUse
    (:then
      (bind _validcontact (CallFunction|ValidHit OtherActor))
      (if _validcontact
        (Utilities|FlowControl|Delay (Math|Random|RandomFloatinRange 0.0 0.1))
        (Variables|Default|GetSafeDistance
          (:then
            (Utilities|Time|ClearandInvalidateTimerbyHandle (Variables|Default|GetDelayedExplosionTimer))
            (Game|SpawnActorfromClass "/Game/Actors/WeaponSystems/Projectiles/Missiles/BP_ProxyExplosion.BP_ProxyExplosion_C" (Transformation|GetActorTransform) "Undefined" "MultiplyWithRoot" 0 _proximityradius 0)
            (bind _outactors (Collision|SphereOverlapActors (Transformation|GetActorLocation) _proximityradius (Utilities|Array|MakeArray "ObjectTypeQuery1" "ObjectTypeQuery2" "ObjectTypeQuery3" "ObjectTypeQuery4" "ObjectTypeQuery5" "ObjectTypeQuery6") 0))
            (for _array_element _outactors
              (Class|BPIHealthInterface|TakeDamage(Message) _array_element (Variables|/Game/Actors/WeaponSystems/Projectiles/__DataAssets/Projectile_PDA.Projectile_PDA_C|GetDamage (Variables|Projectile|Initialize|GetAmmoDataAsset)))
              (CallFunction|InUse?)))
          (:else
            (Utilities|Time|ClearandInvalidateTimerbyHandle (Variables|Default|GetSafeToDetinateTimer))
            (CallFunction|InUse?)))))
    (:else)))

(event OnComponentBeginOverlap(Capsule_Collision)
  (params (OverlappedComponent :type Primitive%20Component%20Object%20Reference) (OtherActor :type Actor%20Object%20Reference) (OtherComp :type Primitive%20Component%20Object%20Reference) (OtherBodyIndex :type Integer) (bFromSweep :type Boolean) (SweepResult :type Hit%20Result%20Structure%20%28by%20ref%29))
  (bind _validcontact (CallFunction|ValidHit OtherActor))
  (if _validcontact
    (Utilities|Time|ClearandInvalidateTimerbyHandle (Variables|Default|GetDelayedExplosionTimer))
    (if (Utilities|DoesObjectImplementInterface OtherActor "/Game/Blueprints/Components/HealthSystem/BPI_HealthInterface.BPI_HealthInterface_C")
      (Class|BPIHealthInterface|TakeDamage(Message) OtherActor (Variables|/Game/Actors/WeaponSystems/Projectiles/__DataAssets/Projectile_PDA.Projectile_PDA_C|GetDamage (Variables|Projectile|Initialize|GetAmmoDataAsset))))
    (CallFunction|InUse?)))

(event ComponentDestrroyed(HealthAC)
  (Default|HideHealthBar (Variables|Default|GetHealthAC))
  (Utilities|Array|RemoveItem (Variables|Health|UpdateOnDeath|GetActorsTargeting) self)
  (if (Utilities|Array|IsEmpty (Variables|Health|UpdateOnDeath|GetActorsTargeting))
    (CallFunction|InUse?)
    (else
      (Rendering|SetActorHiddenInGame true)
      (bind _returnvalue (Utilities|Time|SetTimerbyEvent (delegate Custom|Event_DeathTimer) 0.1 true))
      (Variables|Health|UpdateOnDeath|SetDeathTimer _returnvalue))))

(event Custom|Event_DelayedFusedExplosion
  (bind _ammodataasset (Variables|Projectile|Initialize|GetAmmoDataAsset))
  (bind _proximityradius (Variables|/Game/Actors/WeaponSystems/Projectiles/__DataAssets/Projectile_PDA.Projectile_PDA_C|GetProximityRadius _ammodataasset))
  (Variables|Projectile|Update|GetInUse
    (:then
      (Variables|Default|GetSafeDistance
        (:then
          (Utilities|Time|ClearandInvalidateTimerbyHandle (Variables|Default|GetDelayedExplosionTimer))
          (Game|SpawnActorfromClass "/Game/Actors/WeaponSystems/Projectiles/Missiles/BP_ProxyExplosion.BP_ProxyExplosion_C" (Transformation|GetActorTransform) "Undefined" "MultiplyWithRoot" 0 _proximityradius 0)
          (bind _outactors (Collision|SphereOverlapActors (Transformation|GetActorLocation) _proximityradius (Utilities|Array|MakeArray "ObjectTypeQuery1" "ObjectTypeQuery2" "ObjectTypeQuery3" "ObjectTypeQuery4" "ObjectTypeQuery5" "ObjectTypeQuery6") 0))
          (for _array_element _outactors
            (Class|BPIHealthInterface|TakeDamage(Message) _array_element (Variables|/Game/Actors/WeaponSystems/Projectiles/__DataAssets/Projectile_PDA.Projectile_PDA_C|GetDamage (Variables|Projectile|Initialize|GetAmmoDataAsset)))
            (CallFunction|InUse?)))
        (:else
          (Utilities|Time|ClearandInvalidateTimerbyHandle (Variables|Default|GetSafeToDetinateTimer))
          (CallFunction|InUse?))))
    (:else)))

(event Custom|Event_SetSafeDistance
  (Variables|Default|SetSafeDistance true)
  (Utilities|Time|ClearandInvalidateTimerbyHandle (Variables|Default|GetSafeToDetinateTimer)))

(event Custom|Event_ReuseTargetable
  (Default|HideHealthBar (Variables|Default|GetHealthAC))
  (Utilities|Array|RemoveItem (Variables|Health|UpdateOnDeath|GetActorsTargeting) self)
  (if (Utilities|Array|IsEmpty (Variables|Health|UpdateOnDeath|GetActorsTargeting))
    (CallFunction|InUse?)
    (else
      (Rendering|SetActorHiddenInGame true)
      (bind _returnvalue (Utilities|Time|SetTimerbyEvent (delegate Custom|Event_DeathTimer) 0.1 true))
      (Variables|Health|UpdateOnDeath|SetDeathTimer _returnvalue))))

(event Custom|Event_DeathTimer
  (bind _actorstargeting (Variables|Health|UpdateOnDeath|GetActorsTargeting))
  (if (Utilities|Array|IsEmpty _actorstargeting)
    (CallFunction|InUse?)
    (else
      (for _array_element _actorstargeting
        (Utilities|IsValid _array_element
          (:Is%20Valid
            (Class|BPIWeaponSystem|ContactDestroyed(Message) _array_element))
          (:Is%20Not%20Valid
            (Utilities|Array|RemoveItem (Variables|Health|UpdateOnDeath|GetActorsTargeting) _array_element)))))))

(event EventSetIgnoreActors
  (params (How? :type E_ArrayModification%20Enum :default "NewEnumerator0") (Array :type Array%20of%20Actor%20Object%20References) (Add :type Actor%20Object%20Reference) (Remove :type Actor%20Object%20Reference))
  (bind (_arraytoset _arrayneedsset) (CallFunction|UpdateArray How? (Variables|Default|GetActorsToIgnore) Array Add Remove))
  (if _arrayneedsset
    (Variables|Default|SetActorsToIgnore _arraytoset)))

(event EventFire
  (params (TargetActor :type Actor%20Object%20Reference) (TargetVelocity :type Vector :default "0, 0, 0") (FuseTime :type Float%20%28double-precision%29))
  (bind _projectilemovement (Variables|Default|GetProjectileMovement))
  (bind _ammodataasset (Variables|Projectile|Initialize|GetAmmoDataAsset))
  (bind _capsule_collision (Variables|Default|GetCapsule_Collision))
  (bind _proximitydetination_collision (Variables|Default|GetProximityDetination_Collision))
  (Variables|Default|SetTarget%20Actor TargetActor)
  (bind _returnvalue (Utilities|Time|SetTimerbyEvent (delegate Custom|Event_SetSafeDistance) (Variables|/Game/Actors/WeaponSystems/Projectiles/__DataAssets/Projectile_PDA.Projectile_PDA_C|GetMinimumSafeTime (Variables|Projectile|Initialize|GetAmmoDataAsset)) false true))
  (Variables|Default|SetSafeToDetinateTimer _returnvalue)
  (Variables|Projectile|Update|SetInUse true)
  (Transformation|SetActorTransform (Variables|Projectile|Update|GetStartTransform) false true)
  (Components|Activation|Activate _projectilemovement true)
  (Variables|/Script/Engine.MovementComponent|SetVelocity _projectilemovement TargetVelocity)
  (Development|SetHiddeninGame (Variables|Default|GetMesh) false true)
  (Utilities|FlowControl|Delay 0.5)
  (Variables|/Script/Engine.PrimitiveComponent|SetbGenerateOverlapEvents _capsule_collision true)
  (Collision|SetCollisionEnabled _capsule_collision "QueryAndPhysics")
  (Collision|SetCollisionEnabled _proximitydetination_collision "QueryAndPhysics")
  (Variables|/Script/Engine.PrimitiveComponent|SetbGenerateOverlapEvents _proximitydetination_collision true)
  (Variables|/Game/Actors/WeaponSystems/Projectiles/__DataAssets/Projectile_PDA.Projectile_PDA_C|GetUseAsShieldWall _ammodataasset
    (:then
      (Variables|Default|SetDelayedExplosionTime (Variables|/Game/Actors/WeaponSystems/Projectiles/__DataAssets/Projectile_PDA.Projectile_PDA_C|GetLifetime _ammodataasset))
      (Variables|Default|SetSafeDistance true))
    (:else
      (Variables|Default|SetDelayedExplosionTime FuseTime)))
  (bind _returnvalue_2 (Utilities|Time|SetTimerbyEvent (EventDispatchers|CreateEvent :!event Custom|Event_DelayedFusedExplosion) (Variables|Default|GetDelayedExplosionTime) false true))
  (Variables|Default|SetDelayedExplosionTimer _returnvalue_2))

(event EventInUse?
  (bind _projectilemovement (Variables|Default|GetProjectileMovement))
  (bind _proximitydetination_collision (Variables|Default|GetProximityDetination_Collision))
  (bind _capsule_collision (Variables|Default|GetCapsule_Collision))
  (Variables|Default|SetSafeDistance false)
  (Variables|Projectile|Update|SetInUse false)
  (Components|Activation|Deactivate _projectilemovement)
  (Variables|/Script/Engine.MovementComponent|SetVelocity _projectilemovement "0, 0, 0")
  (Variables|/Script/Engine.PrimitiveComponent|SetbGenerateOverlapEvents _capsule_collision false)
  (Collision|SetCollisionEnabled _capsule_collision "NoCollision")
  (Variables|/Script/Engine.PrimitiveComponent|SetbGenerateOverlapEvents _proximitydetination_collision false)
  (Collision|SetCollisionEnabled _proximitydetination_collision "NoCollision")
  (Development|SetHiddeninGame (Variables|Default|GetMesh) true false)
  (Transformation|SetActorTransform (Variables|Projectile|Update|GetStartTransform) false true))

(event EventTakeDamage
  (params (Damage :type Float%20%28double-precision%29))
  (bind _healthac (Variables|Default|GetHealthAC)
    (:then
      (Default|TakeDamage _healthac Damage))
    (:else)))

(event EventSetStartTransform
  (params (StartingTransform :type Transform))
  (Variables|Projectile|Update|SetStartTransform StartingTransform))

(event EventBeginPlay
  (Variables|Projectile|Update|SetInUse false)
  (Components|Activation|Deactivate (Variables|Default|GetProjectileMovement))
  (Collision|SetCollisionEnabled (Variables|Default|GetCapsule_Collision) "NoCollision")
  (Collision|SetCollisionEnabled (Variables|Default|GetProximityDetination_Collision) "NoCollision"))

(fn ConstructionScript
  (bind _projectilemovement (Variables|Default|GetProjectileMovement))
  (bind _mesh (Variables|Default|GetMesh))
  (bind _ammodataasset (Variables|Projectile|Initialize|GetAmmoDataAsset))
  (bind _ammodataasset_2 (Variables|Projectile|Initialize|GetAmmoDataAsset))
  (bind _ammodataasset_3 (Variables|Projectile|Initialize|GetAmmoDataAsset))
  (bind _proximitydetination_collision (Variables|Default|GetProximityDetination_Collision))
  (bind (_min _max) (Components|StaticMesh|GetLocalBounds _mesh))
  (bind _speed (Variables|/Game/Actors/WeaponSystems/Projectiles/__DataAssets/Projectile_PDA.Projectile_PDA_C|GetSpeed _ammodataasset))
  (bind _health (Variables|/Game/Actors/WeaponSystems/Projectiles/__DataAssets/Projectile_PDA.Projectile_PDA_C|GetHealth _ammodataasset_3))
  (Variables|/Script/Engine.ProjectileMovementComponent|SetInitialSpeed _projectilemovement _speed)
  (Variables|/Script/Engine.ProjectileMovementComponent|SetMaxSpeed _projectilemovement _speed)
  (Variables|/Game/Actors/WeaponSystems/Projectiles/__DataAssets/Projectile_PDA.Projectile_PDA_C|GetUseStaticMesh _ammodataasset
    (:then
      (Components|StaticMesh|SetStaticMesh (Variables|Default|GetMesh) (Variables|/Game/Actors/WeaponSystems/Projectiles/__DataAssets/Projectile_PDA.Projectile_PDA_C|GetStaticMesh _ammodataasset)))
    (:else
      (Development|SetHiddeninGame (Variables|Default|GetMesh) true true)))
  (Variables|/Game/Actors/WeaponSystems/Projectiles/__DataAssets/Projectile_PDA.Projectile_PDA_C|GetProximityDetination _ammodataasset_2
    (:then
      (Components|Sphere|SetSphereRadius _proximitydetination_collision (Variables|/Game/Actors/WeaponSystems/Projectiles/__DataAssets/Projectile_PDA.Projectile_PDA_C|GetProximityRadius _ammodataasset_2) true))
    (:else
      (Components|Activation|SetAutoActivate _proximitydetination_collision false)
      (Collision|SetCollisionEnabled _proximitydetination_collision "NoCollision")))
  (Components|Capsule|SetCapsuleHalfHeight (Variables|Default|GetCapsule_Collision) (.x (+ _min _max)) true)
  (Variables|/Game/Actors/WeaponSystems/Projectiles/__DataAssets/Projectile_PDA.Projectile_PDA_C|GetIncludeHealth _ammodataasset_3
    (:then
      (bind _returnvalue (AddComponent|AddBPHealthAC _health))
      (bind _output_get (Variables|Default|SetHealthAC _returnvalue))
      (Default|SetStartingHealth _output_get _health))
    (:else)))

(fn ValidHit
  (params (HitActor :type Actor%20Object%20Reference%20%28by%20ref%29))
  (bind _returnvalue (Utilities|GetClass HitActor))
  (if (not (Utilities|Array|ContainsItem (Variables|Default|GetActorsToIgnore) HitActor))
    (if (Math|Boolean|ANDBoolean (!= _returnvalue "BP_Projectile_Base_C") (!= _returnvalue "/Game/Blueprints/Debug/BP_TargetingRange.BP_TargetingRange_C") (!= _returnvalue "/Game/Blueprints/Components/PingSystem/BP_PingSphere.BP_PingSphere_C") (not (Actor|ActorHasTag HitActor "IgnoreCollision")))
      (return true)
      (else
        (return false)))))

(fn GetinUse
  (return (Variables|Projectile|Update|GetInUse)))