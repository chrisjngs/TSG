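; Base pooled projectile actor, configured by an ammo data asset for speed, mesh, optional homing, optional health and capsule size.
; Fire launches it at a given velocity, enabling collision and visibility after a brief delay.
; A hit deals damage through BPI_HealthInterface; a hit or lifetime expiry hides it and teleports it to its stored start transform for reuse.
; AI blackboard targeting logic exists but is never run.
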(event OnComponentHit(Capsule_Collision)
  (params (HitComponent :type Primitive%20Component%20Object%20Reference) (OtherActor :type Actor%20Object%20Reference) (OtherComp :type Primitive%20Component%20Object%20Reference) (NormalImpulse :type Vector :default "0, 0, 0") (Hit :type Hit%20Result%20Structure%20%28by%20ref%29))
  (if (Utilities|DoesObjectImplementInterface OtherActor "/Game/Blueprints/Components/HealthSystem/BPI_HealthInterface.BPI_HealthInterface_C")
    (Class|BPIHealthInterface|TakeDamage(Message) OtherActor (Variables|/Game/Actors/WeaponSystems/Projectiles/__DataAssets/Projectile_PDA.Projectile_PDA_C|GetDamage (Variables|Projectile|GetAmmoDataAsset))))
  (CallFunction|InUse?))

(event EventFire
  (params (TargetActor :type Actor%20Object%20Reference) (TargetVelocity :type Vector :default "0, 0, 0"))
  (bind _projectilemovement (Variables|Default|GetProjectileMovement))
  (Variables|Projectile|Update|SetInUse true)
  (Components|Activation|Activate _projectilemovement true)
  (Variables|/Script/Engine.MovementComponent|SetVelocity _projectilemovement TargetVelocity)
  (Utilities|FlowControl|Delay 0.1)
  (Collision|SetCollisionEnabled (Variables|Default|GetCapsule_Collision) "QueryAndPhysics")
  (Development|SetHiddeninGame (Variables|Default|GetMesh) false true)
  (Utilities|FlowControl|Delay (Variables|/Game/Actors/WeaponSystems/Projectiles/__DataAssets/Projectile_PDA.Projectile_PDA_C|GetLifetime (Variables|Projectile|GetAmmoDataAsset)))
  (CallFunction|InUse?))

(event EventInUse?
  (bind _projectilemovement (Variables|Default|GetProjectileMovement))
  (Variables|Projectile|Update|SetInUse false)
  (Components|Activation|Deactivate _projectilemovement)
  (Variables|/Script/Engine.MovementComponent|SetVelocity _projectilemovement "0, 0, 0")
  (Collision|SetCollisionEnabled (Variables|Default|GetCapsule_Collision) "NoCollision")
  (Development|SetHiddeninGame (Variables|Default|GetMesh) true false)
  (Transformation|SetActorTransform (Variables|Projectile|GetStartTransform) false true))

(event EventTakeDamage
  (params (Damage :type Float%20%28double-precision%29))
  (bind _healthac (Variables|Default|GetHealthAC)
    (:then
      (Default|TakeDamage _healthac Damage))
    (:else)))

(event EventSetStartTransform
  (params (StartingTransform :type Transform))
  (Variables|Projectile|SetStartTransform StartingTransform))

(event EventBeginPlay
  (Variables|Projectile|Update|SetInUse false)
  (Components|Activation|Deactivate (Variables|Default|GetProjectileMovement))
  (Collision|IgnoreActorwhenMoving (Variables|Default|GetCapsule_Collision) (Components|GetOwner) true))

(fn ConstructionScript
  (bind _projectilemovement (Variables|Default|GetProjectileMovement))
  (bind _mesh (Variables|Default|GetMesh))
  (bind _ammodataasset (Variables|Projectile|GetAmmoDataAsset))
  (bind _ammodataasset_2 (Variables|Projectile|GetAmmoDataAsset))
  (bind (_min _max) (Components|StaticMesh|GetLocalBounds _mesh))
  (bind _speed (Variables|/Game/Actors/WeaponSystems/Projectiles/__DataAssets/Projectile_PDA.Projectile_PDA_C|GetSpeed _ammodataasset))
  (bind _health (Variables|/Game/Actors/WeaponSystems/Projectiles/__DataAssets/Projectile_PDA.Projectile_PDA_C|GetHealth _ammodataasset_2))
  (Variables|/Script/Engine.ProjectileMovementComponent|SetInitialSpeed _projectilemovement _speed)
  (Variables|/Script/Engine.ProjectileMovementComponent|SetMaxSpeed _projectilemovement _speed)
  (Variables|/Game/Actors/WeaponSystems/Projectiles/__DataAssets/Projectile_PDA.Projectile_PDA_C|GetUseStaticMesh _ammodataasset
    (:then
      (Components|StaticMesh|SetStaticMesh (Variables|Default|GetMesh) (Variables|/Game/Actors/WeaponSystems/Projectiles/__DataAssets/Projectile_PDA.Projectile_PDA_C|GetStaticMesh _ammodataasset)))
    (:else
      (Development|SetHiddeninGame (Variables|Default|GetMesh) true true)))
  (Variables|/Game/Actors/WeaponSystems/Projectiles/__DataAssets/Projectile_PDA.Projectile_PDA_C|GetIsHoming (Variables|Projectile|GetAmmoDataAsset)
    (:then
      (Variables|/Script/Engine.ProjectileMovementComponent|SetbIsHomingProjectile _projectilemovement true)
      (Variables|/Script/Engine.ProjectileMovementComponent|SetHomingTargetComponent _projectilemovement (Variables|/Script/Engine.Actor|GetRootComponent (Variables|Projectile|Homing|GetHomingTarget))))
    (:else
      _))
  (Components|Capsule|SetCapsuleHalfHeight (Variables|Default|GetCapsule_Collision) (.x (+ _min _max)) true)
  (Variables|/Game/Actors/WeaponSystems/Projectiles/__DataAssets/Projectile_PDA.Projectile_PDA_C|GetIncludeHealth _ammodataasset_2
    (:then
      (bind _returnvalue (AddComponent|AddBPHealthAC _health))
      (bind _output_get (Variables|Default|SetHealthAC _returnvalue))
      (Default|SetStartingHealth _output_get _health))
    (:else)))