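; In-mission HUD that creates the layered overlay UI layout on BeginPlay and starts the selected game mode.
; It forwards layer register, push, pop and clear calls to that primary layout widget.
; Level options from the game instance select the mode: Skirmish messages the player controller to play on the chosen platform and initializes the pawn's reputation and commander rank.
; Career handling is an empty stub.
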(event EventBeginPlay
  (bind _returnvalue (UserInterface|CreateWidget "/Game/HUD/WBP_OverlayUILayout.WBP_OverlayUILayout_C" (Game|GetPlayerController 0) (Variables|Default|GetInitialScreensInGame)))
  (bind _output_get (Variables|State|SetPrimaryLayout _returnvalue))
  (UserInterface|Viewport|AddtoViewport _output_get 0)
  (Development|PrintString "Begin play in InMission HUD" true true "(R=0.000000,G=0.660000,B=1.000000,A=1.000000)" 15.0)
  (CallFunction|HandleGameModes))

(event EventPopContentfromLayer
  (params (LayerName :type Gameplay%20Tag%20Structure))
  (Default|PopContentfromLayer (CallFunction|GetPrimaryLayout) LayerName))

(event EventClearAllLayersExcept
  (params (ExecptionLayerName :type Gameplay%20Tag%20Structure))
  (Default|ClearAllLayersExcept (CallFunction|GetPrimaryLayout) ExecptionLayerName))

(event EventClearAllLayers
  (Default|ClearAllLayers (CallFunction|GetPrimaryLayout)))

(event EventClearLayer
  (params (LayerName :type Gameplay%20Tag%20Structure))
  (Default|ClearLayer (CallFunction|GetPrimaryLayout) LayerName))

(fn ConstructionScript)

(fn GetPrimaryLayout
  (return (Variables|State|GetPrimaryLayout)))

(fn InitializeSkirmishReputation
  (params (PlayerPawn :type Pawn%20Object%20Reference))
  (bind _leveloptionstruct (Variables|Default|GetLevelOptionStruct))
  (bind (_rank _reputation) (Utilities|Struct|BreakS_LevelOptions _leveloptionstruct))
  (Class|BPIPlayer|InitializeSkirmishReputation(Message) PlayerPawn (Math|Float|Truncate _reputation) (+ (Utilities|Array|FindItem (LocalVariables|GetRankArray) _rank) 2)))

(fn HandleGameModes
  (bind _leveloptionstruct (Class|BPISaveGame|GetLevelOptions(Message) (Game|GetGameInstance)))
  (bind _output_get (Variables|Default|SetLevelOptionStruct _leveloptionstruct))
  (switch Utilities|FlowControl|Switch|SwitchonE_GameMode (Utilities|Struct|BreakS_LevelOptions _output_get)
    (:NewEnumerator0
      (CallFunction|HandleCareerMode))
    (:NewEnumerator1
      (CallFunction|HandleSkirmishMode))))

(fn HandleSkirmishMode
  (bind _returnvalue (Game|GetPlayerController 0))
  (Class|BPIInitiliazeGame|PlayGame(Message) _returnvalue false (Utilities|Array|MakeArray (Utilities|String|StringToName (Utilities|Struct|BreakS_LevelOptions (Variables|Default|GetLevelOptionStruct)))))
  (bind _playerpawn (Class|BPIInitiliazeGame|GetPlayerPawn(Message) _returnvalue))
  (CallFunction|InitializeSkirmishReputation _playerpawn))

(fn HandleCareerMode)

(fn PushContenttoLayer
  (params (LayerName :type Gameplay%20Tag%20Structure) (WidgetClass :type User%20Widget%20Soft%20Class%20Reference))
  (bind _widget (Default|PushContenttoLayer (CallFunction|GetPrimaryLayout) LayerName WidgetClass))
  (return _widget))

(fn RegisterLayer
  (params (LayoutName :type Gameplay%20Tag%20Structure) (LayerWidget :type WBP%20Layer%20Object%20Reference))
  (bind _success (Default|RegisterLayer (CallFunction|GetPrimaryLayout) LayoutName LayerWidget))
  (return _success))