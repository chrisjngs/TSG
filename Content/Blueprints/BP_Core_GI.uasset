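; Game instance that owns the player ship save data, loading it synchronously on Init and exposing it through GetGameData.
; Loading reads the slot or creates a fresh BP_PlayerShipSaveData if none exists; only a completed async load fires OnGameLoaded.
; Ship configurations save, optionally async, to a fixed player slot or a temporary customization slot, both overwriting the current SaveSlot and shared SavedData.
; Helpers delete slots and debug-print loadouts.
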(event EventInit
  ;[0.15 0.15 0.15 0.5] First thing that's run when the game starts. Load any saved game data
  (CallFunction|LoadGameData false (Variables|Default|GetSaveSlot) (Variables|Default|GetSaveSlotIndex)))

(event EventLoadGameData
  (params (Async :type Boolean) (Slot%20Name :type String) (User%20Index :type Integer))
  ;[0.15 0.15 0.15 0.5] Load Game
  (Variables|Default|SetSaveSlot Slot%20Name)
  (Variables|Default|SetSaveSlotIndex User%20Index)
  (bind _returnvalue (SaveGame|DoesSaveGameExist (Variables|Default|GetSaveSlot) (Variables|Default|GetSaveSlotIndex)))
  (if _returnvalue
    (if Async
      (bind _savegame (|AsyncLoadGamefromSlot (Variables|Default|GetSaveSlot) (Variables|Default|GetSaveSlotIndex))
        (:Completed
          (bind _asbp_player_ship_save_data (Utilities|Casting|CastToBP_PlayerShipSaveData _savegame))
          (Variables|Default|SetSavedData _asbp_player_ship_save_data)
          (Default|CallOnGameLoaded)))
      (else
        (bind _returnvalue_2 (SaveGame|LoadGamefromSlot (Variables|Default|GetSaveSlot) (Variables|Default|GetSaveSlotIndex)))
        (bind _asbp_player_ship_save_data_2 (Utilities|Casting|CastToBP_PlayerShipSaveData _returnvalue_2))
        (Variables|Default|SetSavedData _asbp_player_ship_save_data_2)))
    (else
      (bind _returnvalue_3 (SaveGame|CreateSaveGameObject "/Game/Blueprints/SaveLoadSystem/BP_PlayerShipSaveData.BP_PlayerShipSaveData_C"))
      (Variables|Default|SetSavedData _returnvalue_3))))

(event EventSaveGameData
  (params (Async :type Boolean) (TempSave :type Boolean))
  (bind _saveddata (Variables|Default|GetSavedData))
  (bind _saveslot (Variables|Default|GetSaveSlot))
  (bind _saveslotindex (Variables|Default|GetSaveSlotIndex))
  (bind _result (Utilities|Text|FormatText "Saved data \"{data}\" to slot \"{slot}\" under user \"{user}\"" _saveddata _saveslot _saveslotindex))
  ;[0.15 0.15 0.15 0.5] Save Game
  (if Async
    (|AsyncSaveGametoSlot (Variables|Default|GetSavedData) (Variables|Default|GetSaveSlot) (Variables|Default|GetSaveSlotIndex)
      (:Completed
        (Development|PrintString (Utilities|String|ToString(Text) _result) false)))
    (else
      (SaveGame|SaveGametoSlot (Variables|Default|GetSavedData) (Variables|Default|GetSaveSlot) (Variables|Default|GetSaveSlotIndex))
      (Development|PrintString (Utilities|String|ToString(Text) _result) false))))

(event EventStoreTempPlayerData
  (params (TempPlayerData :type S%20Ship%20Configurations%20Structure) (Async :type Boolean))
  ;[0.15 0.15 0.15 0.5] Save a temp file for customizing the players ship
  (Variables|/Game/Blueprints/SaveLoadSystem/BP_PlayerShipSaveData.BP_PlayerShipSaveData_C|SetShipConfiguration (Variables|Default|GetSavedData) TempPlayerData)
  (Variables|Default|SetSaveSlot "TEMPSHIPCONFIG")
  (CallFunction|SaveGameData Async false))

(event EventDeleteSave
  (params (SaveSlot :type String) (UserIndex :type Integer))
  ;[0.15 0.15 0.15 0.5] Delete a specific save file
  (bind _returnvalue (SaveGame|DoesSaveGameExist SaveSlot UserIndex))
  (if _returnvalue
    (SaveGame|DeleteGameinSlot SaveSlot UserIndex)))

(event EventSavePlayer
  (params (PlayerShipInformation :type S%20Ship%20Configurations%20Structure) (Async :type Boolean))
  ;[0.15 0.15 0.15 0.5] Save the player's ship configuration
  (bind _output_get (Variables|/Game/Blueprints/SaveLoadSystem/BP_PlayerShipSaveData.BP_PlayerShipSaveData_C|SetShipConfiguration (Variables|Default|GetSavedData) PlayerShipInformation))
  (Variables|Default|SetSaveSlot "TestPlayerShip")
  (CallFunction|SaveGameData Async false))

(fn TempPrintSaveData
  (params (save%20data :type S%20Loaded%20Soft%20Data%20Assets%20Structure))
  (bind (_offensive _defensive _missiles) (Utilities|Struct|BreakS_LoadedSoftDataAssets save%20data))
  (Development|PrintString (Utilities|String|ToString(Text) (Utilities|Text|FormatText "The loaded data that was saved is:")) true true "(R=0.000000,G=0.701102,B=0.000000,A=1.000000)")
  (for _array_element _offensive
    (Development|PrintString (Utilities|String|ToString(Text) (Utilities|Text|FormatText "Offensive: \"{array}\"" (Utilities|ResolveSoftReference _array_element))) true true "(R=0.000000,G=0.701102,B=0.000000,A=1.000000)"))
  (for _array_element_2 _defensive
    (Development|PrintString (Utilities|String|ToString(Text) (Utilities|Text|FormatText "Defensive: \"{array}\"" (Utilities|ResolveSoftReference _array_element_2))) true true "(R=0.000000,G=0.701102,B=0.000000,A=1.000000)"))
  (for _array_element_3 _missiles
    (Development|PrintString (Utilities|String|ToString(Text) (Utilities|Text|FormatText "Missiles: \"{array}\"" (Utilities|ResolveSoftReference _array_element_3))) true true "(R=0.000000,G=0.701102,B=0.000000,A=1.000000)"))
  (return save%20data))

(fn GetGameData
  (return (Variables|Default|GetSavedData)))