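; Attack/Defend game mode that registers BP_Core_PC controllers on login or controller swap and spawns player pawns and ship platforms.
; Spawn events place BP_Core_Pawn and named BP_ShipSystem_Base actors at random PlayerStarts, storing the pawn and mapping each platform to its Faction.
; A separate SpawnPlayer function replaces a controller's pawn and adds a platform, re-rolling the random start on each lookup.
; Getters expose pawn and platforms, while GetPMSInitialized always returns false.
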(event EventBeginPlay
  (Development|PrintString "Begin play in Game Mode" true true "(R=0.000000,G=0.660000,B=1.000000,A=1.000000)" 15.0))

(event EventPostLogin
  (params (NewPlayer :type Player%20Controller%20Object%20Reference))
  (bind _asbp_core_pc (Utilities|Casting|CastToBP_Core_PC NewPlayer))
  (Utilities|Array|Add (Variables|Default|GetPlayerController) _asbp_core_pc))

(event EventOnSwapPlayerControllers
  (params (OldPC :type Player%20Controller%20Object%20Reference) (NewPC :type Player%20Controller%20Object%20Reference))
  (bind _asbp_core_pc (Utilities|Casting|CastToBP_Core_PC NewPC))
  (Utilities|Array|Add (Variables|Default|GetPlayerController) _asbp_core_pc))

(event EventSpawnPlatform
  (params (PlatformName :type Name :default "None") (Faction :type E_FriendFoe%20Enum :default "NewEnumerator0"))
  (bind _spawnedplatform (CallFunction|HandlePlatformSpawning PlatformName Faction))
  (Utilities|Map|Add (Variables|Default|GetSpawnedPlatforms) _spawnedplatform Faction))

(event EventSpawnPlayer
  (bind _spawnedpawn (CallFunction|HandleSpawnPlayer))
  (Variables|Default|SetPlayerPawn _spawnedpawn))

(fn ConstructionScript)

(fn FindPlayerStart
  (bind _outactors (Actor|GetAllActorsOfClass "/Script/Engine.PlayerStart"))
  (return (Transformation|GetActorTransform (Utilities|Array|Get(acopy) _outactors (Math|Random|RandomIntegerinRange 0 (- (Utilities|Array|Length _outactors) 1))))))

(fn SpawnPlayer
  (params (Player%20Controller :type Player%20Controller%20Object%20Reference))
  (bind _returnvalue (Pawn|GetControlledPawn Player%20Controller))
  (bind _player_start_transform (Spawning|FindPlayerStart))
  (Utilities|IsValid _returnvalue
    (:Is%20Valid
      (Actor|DestroyActor _returnvalue))
    (:Is%20Not%20Valid
      _))
  (bind _returnvalue_2 (Game|SpawnActorfromClass "/Game/Blueprints/Player/BP_Core_Pawn.BP_Core_Pawn_C" _player_start_transform "Undefined" "MultiplyWithRoot" 0 0))
  (bind _returnvalue_3 (Game|SpawnActorfromClass "/Game/Actors/Ships/Ship_Core/Blueprints/BP_ShipSystem_Base.BP_ShipSystem_Base_C" _player_start_transform "Undefined" "MultiplyWithRoot" 0 "Test Frigate" "NewEnumerator0" 0))
  (return _returnvalue_2 _returnvalue_3 _player_start_transform))

(fn HandlePlatformSpawning
  (params (PlatformName :type Name) (Faction :type E_FriendFoe%20Enum :default "NewEnumerator0"))
  (bind _returnvalue (Game|SpawnActorfromClass "/Game/Actors/Ships/Ship_Core/Blueprints/BP_ShipSystem_Base.BP_ShipSystem_Base_C" (Spawning|FindPlayerStart) "Undefined" "MultiplyWithRoot" 0 PlatformName Faction 0))
  (return _returnvalue))

(fn HandleSpawnPlayer
  (bind _returnvalue (Game|SpawnActorfromClass "/Game/Blueprints/Player/BP_Core_Pawn.BP_Core_Pawn_C" (Spawning|FindPlayerStart) "Undefined" "MultiplyWithRoot" 0 0))
  (return _returnvalue))

(fn GetPlayerPawn
  (return (Variables|Default|GetPlayerPawn)))

(fn GetPMSInitialized
  (return false))

(fn GetSpawnedPlatforms
  (return (Variables|Default|GetSpawnedPlatforms)))