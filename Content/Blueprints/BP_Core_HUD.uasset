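; Core HUD that creates the game's root layered UI and serves as the access point for managing its layers.
; On BeginPlay it builds WBP_OverlayUILayout for the first player controller, seeded with the in-game initial screens, stores it as PrimaryLayout and adds it to the viewport.
; Thin wrappers forward layer registration and content push, pop and clear calls to that layout, keeping layer logic in the widget.
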(event EventBeginPlay
  (bind _returnvalue (UserInterface|CreateWidget "/Game/HUD/WBP_OverlayUILayout.WBP_OverlayUILayout_C" (Game|GetPlayerController 0) (Variables|Default|GetInitialScreensInGame)))
  (bind _output_get (Variables|State|SetPrimaryLayout _returnvalue))
  (UserInterface|Viewport|AddtoViewport _output_get 0)
  (bind _playerpawn (Class|BPIInitiliazeGame|GetPlayerPawn(Message) (Game|GetPlayerController 0))))

(event EventPopContentfromLayer
  (params (LayerName :type Gameplay%20Tag%20Structure))
  (Default|PopContentfromLayer (CallFunction|GetPrimaryLayout) LayerName))

(event EventClearAllLayersExcept
  (params (ExecptionLayerName :type Gameplay%20Tag%20Structure))
  (Default|ClearAllLayersExcept (CallFunction|GetPrimaryLayout) ExecptionLayerName))

(event EventClearAllLayers
  (Default|ClearAllLayers (CallFunction|GetPrimaryLayout)))

(event EventClearLayer
  (params (LayerName :type Gameplay%20Tag%20Structure))
  (Default|ClearLayer (CallFunction|GetPrimaryLayout) LayerName))

(fn ConstructionScript)

(fn GetPrimaryLayout
  (return (Variables|State|GetPrimaryLayout)))

(fn PushContenttoLayer
  (params (LayerName :type Gameplay%20Tag%20Structure) (WidgetClass :type User%20Widget%20Soft%20Class%20Reference))
  (bind _widget (Default|PushContenttoLayer (CallFunction|GetPrimaryLayout) LayerName WidgetClass))
  (return _widget))

(fn RegisterLayer
  (params (LayoutName :type Gameplay%20Tag%20Structure) (LayerWidget :type WBP%20Layer%20Object%20Reference))
  (bind _success (Default|RegisterLayer (CallFunction|GetPrimaryLayout) LayoutName LayerWidget))
  (return _success))