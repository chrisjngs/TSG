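; Blueprint function library for working with modular ships and platforms built from nested child actors.
; Finds the "ShipBase" child actor, reads a platform's stored configuration, and looks up or updates component entries by attachment point and type.
; OrganizePlatformConfig flattens component categories into one array with socket-keyed actor and index maps.
; Also casts weapon data assets and extracts positions from PCG JSON exports; GetPlayerShipComponentsToUpdate is an unwired stub.
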(fn GetShipBase
  (params (Actor :type Actor%20Object%20Reference))
  ;[0.15 0.15 0.15 0.5] Returns the base component of the ship that has the tag "ShipBase"
  (Utilities|IsValid Actor
    (:Is%20Valid
      (bind _array_element (Utilities|Array|ForEachLoopwithBreak (Actor|GetAllChildActors Actor true) :!label _label)
        (:LoopBody
          (if (Actor|ActorHasTag _array_element "ShipBase")
            (Utilities|FlowControl|Sequence
              (:then_0
                (goto _label Break))
              (:then_1
                (return _array_element)))))))
    (:Is%20Not%20Valid
      (Development|PrintText 0 (Utilities|Text|FormatText "The passed actor is not valid as an actor to get ShipBase from. Got {actor}" Actor) true true "(R=1.000000,G=0.194653,B=0.179850,A=1.000000)" 5.0))))

(fn UpdateLocalComponenttoSaved
  (params (LocalArray :type Array%20of%20S%20Ship%20Component%20Structures) (ArrayIndex :type Integer) (LocalComponent :type S%20Ship%20Component%20Structure) (SavedComponent :type S%20Ship%20Component%20Structure))
  (bind (_attachmentpoint _componentbaseclass _previousdataasset _currentdataasset _nextdataasset _actorcomponentreference) (Utilities|Struct|BreakS_ShipComponent LocalComponent))
  (bind (_attachmentpoint_2 _componentbaseclass_2 _previousdataasset_2 _currentdataasset_2 _nextdataasset_2 _actorcomponentreference_2 _componenttype) (Utilities|Struct|BreakS_ShipComponent SavedComponent))
  (Utilities|Array|SetArrayElem LocalArray ArrayIndex (Utilities|Struct|MakeS_ShipComponent _attachmentpoint _componentbaseclass_2 0 _currentdataasset_2 0 _actorcomponentreference _componenttype)))

(fn GetDataAssetVariables
  (params (DataAsset :type Primary%20Data%20Asset%20Object%20Reference))
  ;[0.15 0.15 0.15 0.5] A simple cast function to get the variables from the given data asset.
  (bind _asbp_weapon_system_base_pda (Utilities|Casting|CastToBP_WeaponSystem_Base_PDA DataAsset)
    (:then
      (return _asbp_weapon_system_base_pda))
    (:CastFailed
      (CallFunction|ThrowScriptError "BFL_NestedChildren_Functions" "GetDataAssetVariables" "The cast failed." "A data asset that inherits from BP_WeaponSystem_Base_PDA" (Utilities|Text|ToText(String) (Utilities|GetClassDisplayName (Utilities|GetClass DataAsset)))))))

(fn GetPilotedPlatformInfo
  (params (Platform :type Actor%20Object%20Reference))
  (bind _asplatformparent_base (Utilities|Casting|CastTo___BP_PlatformParent_BASE Platform)
    (:then
      (return (Variables|/Game/Actors/Platforms/__ParentActors/___BP_PlatformParent_BASE.___BP_PlatformParent_BASE_C|GetShipConfig _asplatformparent_base) (Variables|/Game/Actors/Platforms/__ParentActors/___BP_PlatformParent_BASE.___BP_PlatformParent_BASE_C|GetStoredPlatformComponents _asplatformparent_base)))
    (:CastFailed
      (CallFunction|ThrowScriptError "BFL_NestedChildren_Functions" "GetPilotedPlatformInfo" "Cast failed" "BP_PlatformParent_Ship" (Utilities|Text|ToText(Object) Platform)))))

(fn ReadPCGJsonExport
  (params (JsonFile :type File%20Path%20Structure%20%28by%20ref%29))
  ;[0.15 0.15 0.15 0.5] This works with the default Json file that is created by the PCG graph.
  (bind (_outjsonobject _returnvalue) (Class|JsonBlueprintFunctionLibrary|FromFile JsonFile))
  (if _returnvalue
    (bind _fieldnames (Class|JsonBlueprintFunctionLibrary|GetFieldNames _outjsonobject))
    (for _array_element _fieldnames
      (bind _outvalue (|GetJsonField _outjsonobject _array_element))
      (bind _fieldnames_2 (Class|JsonBlueprintFunctionLibrary|GetFieldNames _outvalue))
      (for _array_element_2 _fieldnames_2
        (bind _outvalue_2 (|GetJsonField _outvalue "$Position"))
        (if (Utilities|Array|IsNotEmpty _outvalue_2)
          (Utilities|Array|Add (LocalVariables|GetLocalPointVector) (Math|Vector|MakeVector (Math|Conversions|ToFloat(Integer) (Utilities|Array|Get(acopy) _outvalue_2)) (Math|Conversions|ToFloat(Integer) (Utilities|Array|Get(acopy) _outvalue_2 1)) (Math|Conversions|ToFloat(Integer) (Utilities|Array|Get(acopy) _outvalue_2 2)))))))
    (return (LocalVariables|GetLocalPointVector))))

(fn GetPlayerShipComponentstoUpdate
  (params (ComponentArray :type Array%20of%20S%20Ship%20Component%20Structures) (ShipComponent :type Scene%20Component%20Object%20Reference)))

(fn GetComponentsfromAttachmentPoints
  (params (AttachmentPoints :type Scene%20Component%20Object%20Reference) (Array :type Array%20of%20S%20Ship%20Component%20Structures) (Index :type Integer))
  (bind _output (Utilities|Array|Get(acopy) Array Index))
  (bind (_attachmentpoint _currentdataasset _actorcomponentreference) (Utilities|Struct|BreakS_ShipComponent _output))
  (if (== (Utilities|String|StringToName (Utilities|GetObjectName AttachmentPoints)) _attachmentpoint)
    (return _currentdataasset _actorcomponentreference)))

(fn GetComponentEntrybyAttachmentPointName
  (params (AttachmentPoint :type Name) (ShipConfiguration :type S%20Ship%20Configs%20Structure) (ComponentType :type ShipSystem_ComponentType_Enum%20Enum :default "NewEnumerator0"))
  (bind (_shipcost _shipmesh _shiptype _armortype _engines _shipcomponents _offensiveweapons _defensiveweapons _missilesilos _sensorsystems) (Utilities|Struct|BreakS_ShipConfigs ShipConfiguration))
  (switch Utilities|FlowControl|Switch|SwitchonShipSystem_ComponentType_Enum ComponentType
    (:NewEnumerator0
      (for _array_element _shipcomponents
        (if (== AttachmentPoint (Utilities|Struct|BreakS_PlatformAttachmentInformation _array_element))
          (return _array_element))))
    (:NewEnumerator1
      (for _array_element_2 _offensiveweapons
        (if (== AttachmentPoint (Utilities|Struct|BreakS_PlatformAttachmentInformation _array_element_2))
          (return _array_element_2))))
    (:NewEnumerator2
      (for _array_element_3 _defensiveweapons
        (if (== AttachmentPoint (Utilities|Struct|BreakS_PlatformAttachmentInformation _array_element_3))
          (return _array_element_3))))
    (:NewEnumerator3
      (for _array_element_4 _missilesilos
        (if (== AttachmentPoint (Utilities|Struct|BreakS_PlatformAttachmentInformation _array_element_4))
          (return _array_element_4))))
    (:NewEnumerator4
      (for _array_element_5 _sensorsystems
        (if (== AttachmentPoint (Utilities|Struct|BreakS_PlatformAttachmentInformation _array_element_5))
          (return _array_element_5))))))

(fn GetPlayerShip
  (return (.AsBP%20Core%20PC (Utilities|Casting|CastToBP_Core_PC (Game|GetPlayerController 0)))))

(fn OrganizePlatformConfig
  (params (Configuration :type S%20Ship%20Configs%20Structure))
  (bind (_shipcost _shipcomponents _offensiveweapons _defensiveweapons _missilesilos _sensorsystems) (Utilities|Struct|BreakS_ShipConfigs Configuration))
  (bind _alllocalcomponents (LocalVariables|GetAllLocalComponents))
  (Utilities|Array|AppendArray _alllocalcomponents _shipcomponents)
  (Utilities|Array|AppendArray _alllocalcomponents _offensiveweapons)
  (Utilities|Array|AppendArray _alllocalcomponents _defensiveweapons)
  (Utilities|Array|AppendArray _alllocalcomponents _missilesilos)
  (Utilities|Array|AppendArray _alllocalcomponents _sensorsystems)
  (for (_array_element _array_index) (LocalVariables|GetAllLocalComponents)
    (Utilities|Map|Add (LocalVariables|GetLocalActorMap) (.AttachmentSocket (Utilities|Struct|BreakS_PlatformAttachmentInformation _array_element)) (.ActorComponentReference (Utilities|Struct|BreakS_PlatformAttachmentInformation _array_element)))
    (Utilities|Map|Add (LocalVariables|GetLocalIndexMap) (.AttachmentSocket (Utilities|Struct|BreakS_PlatformAttachmentInformation _array_element)) _array_index))
  (return (LocalVariables|GetAllLocalComponents) (LocalVariables|GetLocalActorMap) (LocalVariables|GetLocalIndexMap)))