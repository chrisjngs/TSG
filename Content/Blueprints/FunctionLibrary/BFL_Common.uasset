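; BFL_Common is a function library of shared helpers for input type, mouse line traces, container updates and actor motion math.
; Array and map updaters switch on an operation and flag when the caller must set the result, with a weapon variant syncing assigned contacts and available weapons.
; The angle helper compares world-origin position vectors.
; The towards/away check dots relative velocity, estimated from position samples, with the offset between actors.
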(fn GetInputType
  (return (Class|CommonInputSubsystem|GetCurrentInputType (PlayerController|LocalPlayerSubsystems|GetCommonInputSubsystem (Game|GetPlayerController 0)))))

(fn LineTracefromMouse
  (params (LineTraceDistance :type Float%20%28single-precision%29) (PlayerController :type Player%20Controller%20Object%20Reference) (TraceChannel :type ETraceTypeQuery%20Enum :default "TraceTypeQuery1"))
  (bind (_worldlocation _worlddirection) (Game|Player|ConvertMouseLocationToWorldSpace PlayerController))
  (bind _outhit (Collision|LineTraceByChannel 0 _worldlocation (+ _worldlocation (* _worlddirection LineTraceDistance)) TraceChannel false 0 "None" true "(R=1.000000,G=0.000000,B=0.000000,A=1.000000)" "(R=0.000000,G=1.000000,B=0.000000,A=1.000000)" 0.5))
  (return _outhit))

(fn UpdateArray
  (params (How? :type E_ArrayModification%20Enum :default "NewEnumerator0") (ArrayBeingModified :type Array%20of%20Actor%20Object%20References) (NewArray :type Array%20of%20Actor%20Object%20References) (AddItem :type Actor%20Object%20Reference) (RemoveItem :type Actor%20Object%20Reference))
  (switch Utilities|FlowControl|Switch|SwitchonE_ArrayModification How?
    (:NewEnumerator0
      (return NewArray true))
    (:NewEnumerator1
      (Utilities|Array|AppendArray ArrayBeingModified NewArray)
      (return ArrayBeingModified false))
    (:NewEnumerator2
      (Utilities|Array|AddUnique ArrayBeingModified AddItem)
      (return ArrayBeingModified false))
    (:NewEnumerator3
      (Utilities|Array|RemoveItem ArrayBeingModified RemoveItem)
      (return ArrayBeingModified false))))

(fn UpdateMap
  (params (How? :type E_MapModification%20Enum :default "NewEnumerator0") (MapBeingModified :type Map%20of%20Actor%20Object%20References%20to%20Integers) (NewMap :type Map%20of%20Actor%20Object%20References%20to%20Integers) (ItemKey :type Actor%20Object%20Reference) (ItemValue :type Integer) (RemoveKey :type Actor%20Object%20Reference))
  (switch Utilities|FlowControl|Switch|SwitchonE_MapModification How?
    (:NewEnumerator0
      (return NewMap true))
    (:NewEnumerator1
      (Utilities|Map|Add MapBeingModified ItemKey ItemValue)
      (return MapBeingModified false))
    (:NewEnumerator2
      (Utilities|Map|Remove MapBeingModified RemoveKey)
      (return MapBeingModified false))))

(fn UpdateWeaponAvailability
  (params (How? :type E_MapModification%20Enum :default "NewEnumerator0") (AssignedMap :type Map%20of%20Actor%20Object%20References%20to%20Objects) (AvailableArray :type Array%20of%20Actor%20Object%20References) (Weapon :type Actor%20Object%20Reference) (Contact :type Actor%20Object%20Reference))
  (switch Utilities|FlowControl|Switch|SwitchonE_MapModification How?
    (:NewEnumerator0
      (return AssignedMap true))
    (:NewEnumerator1
      (Utilities|Map|Add AssignedMap Weapon Contact)
      (Utilities|Array|RemoveItem AvailableArray Weapon)
      (return AssignedMap false))
    (:NewEnumerator2
      (Utilities|Map|Remove AssignedMap Weapon)
      (Utilities|Array|AddUnique AvailableArray Weapon)
      (return AssignedMap false))))

(fn GetAngleTowardsTarget
  (params (Source :type Actor%20Object%20Reference) (Contact :type Actor%20Object%20Reference))
  (bind _returnvalue (Transformation|GetActorLocation Contact))
  (bind _returnvalue_2 (Transformation|GetActorLocation Source))
  (bind (_x _y _z) (Math|Vector|BreakVector _returnvalue_2))
  (bind (_x_2 _y_2 _z_2) (Math|Vector|BreakVector _returnvalue))
  (return (Class|KismetMathLibrary|DegAcos (/ (Math|Vector|DotProduct _returnvalue_2 _returnvalue) (* (Math|Float|Sqrt (+ (Math|Float|Square _x) (Math|Float|Square _y) (Math|Float|Square _z))) (Math|Float|Sqrt (+ (Math|Float|Square _x_2) (Math|Float|Square _y_2) (Math|Float|Square _z_2))))))))

(fn IsObjectMovingAwayorTowards
  (params (Source :type Actor%20Object%20Reference) (Object :type Actor%20Object%20Reference) (DeltaTime :type Float%20%28double-precision%29))
  (Utilities|IsValid Source
    (:Is%20Valid
      (Utilities|IsValid Object
        (:Is%20Valid
          (LocalVariables|SetD (- (Transformation|GetActorLocation Object) (Transformation|GetActorLocation Source)))
          (bind _velocity (CallFunction|GetActorVelocity Source DeltaTime))
          (LocalVariables|SetU _velocity)
          (LocalVariables|SetU_Set true)
          (bind _velocity_2 (CallFunction|GetActorVelocity Object DeltaTime))
          (LocalVariables|SetV _velocity_2)
          (LocalVariables|SetV_Set true)
          (if (and (LocalVariables|GetU_Set) (LocalVariables|GetV_Set))
            (LocalVariables|SetFinalDirection (Math|Vector|DotProduct (- (LocalVariables|GetU) (LocalVariables|GetV)) (LocalVariables|GetD)))
            (if (< (Math|Vector|DotProduct (- (LocalVariables|GetU) (LocalVariables|GetV)) (LocalVariables|GetD)) 0.0)
              (return (LocalVariables|GetFinalDirection) true)
              (else
                (return (LocalVariables|GetFinalDirection) false)))))))))

(fn GetActorVelocity
  (params (Actor :type Actor%20Object%20Reference) (Time :type Float%20%28double-precision%29))
  (bind _returnvalue (Transformation|GetActorLocation Actor))
  (LocalVariables|GetHaveU_P1
    (:then
      (LocalVariables|GetHaveU_P2
        (:then
          (LocalVariables|SetV_P1 _returnvalue)
          (LocalVariables|SetHaveU_P2 false))
        (:else
          (LocalVariables|SetV_P2 _returnvalue)
          (LocalVariables|SetHaveU_P2 true)))
      (if (and (LocalVariables|GetHaveU_P1) (LocalVariables|GetHaveU_P2))
        (return (/ (- (LocalVariables|GetV_P1) (LocalVariables|GetV_P2)) Time) (LocalVariables|GetV_P1) (LocalVariables|GetV_P2))))
    (:else
      (LocalVariables|SetV_P1 _returnvalue)
      (LocalVariables|SetHaveU_P1 true))))