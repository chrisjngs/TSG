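; Blueprint function library for the weapon system, covering target validation, target selection, component lookup and weapon aiming.
; Contacts are validated by line trace, and priority goes to the first untracked target, falling back to a distance-sorted list.
; Interface checks locate sensor controllers and other platform components.
; RotateWeapon converts the target into weapon-local yaw and pitch, drives limited rotation through PID controllers, and reports whether aim is within firing tolerance.
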(fn ContactValidation
  (params (Source :type Actor%20Object%20Reference) (Contact :type Actor%20Object%20Reference) (IgnoredActors :type Array%20of%20Actor%20Object%20References))
  (bind _returnvalue (Transformation|GetActorLocation Contact))
  (bind _returnvalue_2 (Transformation|GetActorLocation Source))
  ;[0.15 0.15 0.15 0.5] Run a line trace from the source of the ping to the contact. If the line trace hits the object it's expecting, it returns its hit information.
  (Utilities|IsValid Source
    (:Is%20Valid
      (Utilities|IsValid Contact
        (:Is%20Valid
          (if (Utilities|Array|IsNotEmpty IgnoredActors)
            (bind _outhit (Collision|LineTraceByChannel 0 (Transformation|GetActorLocation Source) _returnvalue "TraceTypeQuery2" true IgnoredActors "None" true "(R=1.000000,G=0.000000,B=0.000000,A=1.000000)" "(R=0.000000,G=1.000000,B=0.000000,A=1.000000)" 0.0))
            (if (== (.HitActor (Collision|BreakHitResult _outhit)) Contact)
              (return _outhit _returnvalue (== (.HitActor (Collision|BreakHitResult _outhit)) Contact)))
            (else
              (bind _outhit_2 (Collision|LineTraceByChannel 0 _returnvalue_2 (Transformation|GetActorLocation Contact) "TraceTypeQuery2" true 0 "None" true "(R=1.000000,G=0.000000,B=0.000000,A=1.000000)" "(R=0.000000,G=1.000000,B=0.000000,A=1.000000)" 0.0))
              (if (== (.HitActor (Collision|BreakHitResult _outhit_2)) Contact)
                (return _outhit_2 _returnvalue_2 (== (.HitActor (Collision|BreakHitResult _outhit_2)) Contact))))))))))

(fn GetDistancetoTarget
  (params (Source :type Actor%20Object%20Reference) (Target :type Actor%20Object%20Reference))
  (Utilities|IsValid Source
    (:Is%20Valid
      (Utilities|IsValid Target
        (:Is%20Valid
          (return (Math|Vector|Distance(Vector) (Transformation|GetActorLocation Source) (Transformation|GetActorLocation Target))))))))

(fn SortTrackedTargets
  (params (ActorsInRange :type Array%20of%20Actor%20Object%20References) (Source :type Actor%20Object%20Reference))
  (for _index (range 0 (- (Utilities|Array|Length ActorsInRange) 1))
    ;[0.15 0.15 0.15 0.5] First make a temp array with all of the distance values.
    (LocalVariables|SetIndex _index)
    (Utilities|Array|SetArrayElem (LocalVariables|GetTempDistanceArray) (LocalVariables|GetIndex) (Math|Vector|Distance(Vector) (Transformation|GetActorLocation Source) (Transformation|GetActorLocation (Utilities|Array|Get(acopy) ActorsInRange (LocalVariables|GetIndex)))) true))
  ;[0.15 0.15 0.15 0.5] Sort the temp array and return how the indexed changed, then use those changed index to change the actor array.
  (bind _changedindex (CallFunction|SortFloatArray-Shell (LocalVariables|GetTempDistanceArray)))
  (bind (_keypin _valuepin) (Utilities|Map|ForEachLoop(Map) _changedindex)
    (:then
      (Utilities|Array|Swap ActorsInRange _keypin _valuepin))
    (:CompletedPin
      (return ActorsInRange))))

(fn GetPriorityTarget
  (params (Targets :type Map%20of%20Actor%20Object%20References%20to%20Booleans) (Source :type Actor%20Object%20Reference) (StatusToCheck :type E_TargetedStatus%20Enum :default "NewEnumerator0"))
  ;[0.15 0.15 0.15 0.5] Get a target that is not currently tracked. If there are no targets that aren't being tracked, then get the clostest one.
  (bind (_keypin _valuepin) (Utilities|Map|ForEachLoop(Map) Targets)
    (:then
      (Utilities|Array|Add (LocalVariables|GetTempTargetArray) _keypin)
      (if (not _valuepin)
        (return _keypin)))
    (:CompletedPin
      (bind _sortedarray (TargetSorting|SortTrackedTargets (LocalVariables|GetTempTargetArray) Source))
      (return (Utilities|Array|Get(acopy) _sortedarray)))))

(fn GetSensorController
  (params (AttachedPlatform :type Actor%20Object%20Reference))
  (bind _platformcomponents (Class|BPIPSC|GetPlatformComponents(Message) AttachedPlatform))
  (bind _array_element (Utilities|Array|ForEachLoopwithBreak _platformcomponents :!label _label)
    (:LoopBody
      (if (Utilities|DoesObjectImplementInterface _array_element "/Game/Blueprints/Components/SensorSystem/BPI_SensorController.BPI_SensorController_C")
        (LocalVariables|SetController _array_element)
        (LocalVariables|SetControllerFound true)
        (goto _label Break)))
    (:Completed
      (return (LocalVariables|GetController) (LocalVariables|GetControllerFound)))))

(fn GetInterfaceComponent
  (params (PlatformComponents :type S%20Ship%20Child%20Components%20Structure) (Interface :type Interface%20Class%20Reference))
  (bind _array_element (Utilities|Array|ForEachLoopwithBreak (.Ship (Utilities|Struct|BreakS_ShipChildComponents PlatformComponents)) :!label _label)
    (:LoopBody
      (if (Utilities|DoesObjectImplementInterface _array_element Interface)
        (LocalVariables|SetController _array_element)
        (LocalVariables|SetControllerFound true)
        (goto _label Break)))
    (:Completed
      (return (LocalVariables|GetController) (LocalVariables|GetControllerFound)))))

(fn MakeBulletSpread
  (params (TargetLocation :type Vector) (SpreadAmount :type Float%20%28double-precision%29) (__WorldContext :type Object%20Object%20Reference))
  (bind _returnvalue (/ SpreadAmount 2.0))
  (return (+ TargetLocation (Math|Random|RandomFloatinRange (* _returnvalue -1.0) (Math|Float|Absolute(Float) _returnvalue)))))

(fn LimitWeaponRotation
  (params (Min :type Float%20%28double-precision%29) (Max :type Float%20%28double-precision%29) (Current :type Float%20%28double-precision%29) (Change :type Float%20%28double-precision%29))
  (bind _returnvalue (+ Current Change))
  (return (and (<= _returnvalue Max) (>= _returnvalue Min))))

(fn FindTargetPitch
  (params (TargetLocation :type Vector) (PitchComponent :type Static%20Mesh%20Component%20Object%20Reference) (Weapon :type Actor%20Object%20Reference))
  (bind _returnvalue (Transformation|GetWorldLocation PitchComponent))
  (bind _returnvalue_2 (Transformation|GetActorTransform Weapon))
  (bind _returnvalue_3 (- TargetLocation _returnvalue))
  (bind _returnvalue_4 (Math|Transform|InverseTransformDirection _returnvalue_2 _returnvalue_3))
  (bind (_x _y _z) (Math|Vector|BreakVector _returnvalue_4))
  (return (Math|Rotator|MakeRotator 0.0 (.pitch (Class|KismetMathLibrary|NegateRotator (Math|Rotator|MakeRotator 0.0 (- (Class|KismetMathLibrary|DegAtan2 (Math|Float|Sqrt (+ (Math|Float|Square _x) (Math|Float|Square _y))) _z) 9e+01) 0.0))) 0.0)))

(fn FindTargetYaw
  (params (TargetLocation :type Vector) (YawComponent :type Static%20Mesh%20Component%20Object%20Reference) (Weapon :type Actor%20Object%20Reference))
  (bind _returnvalue (Transformation|GetWorldLocation YawComponent))
  (bind _returnvalue_2 (Transformation|GetActorTransform Weapon))
  (bind _returnvalue_3 (- TargetLocation _returnvalue))
  (bind _returnvalue_4 (Math|Transform|InverseTransformDirection _returnvalue_2 _returnvalue_3))
  (bind (_x _y) (Math|Vector|BreakVector _returnvalue_4))
  (return (Math|Rotator|MakeRotator 0.0 0.0 (Class|KismetMathLibrary|DegAtan2 _y _x))))

(fn RotateWeapon
  (params (YawComponent :type Static%20Mesh%20Component%20Object%20Reference) (PitchComponent :type Static%20Mesh%20Component%20Object%20Reference) (RollComponent :type Static%20Mesh%20Component%20Object%20Reference) (UseYaw :type Boolean) (UsePitch :type Boolean) (UseRoll :type Boolean) (TargetLocation :type Vector) (WeaponData :type BP%20Weapon%20System%20Base%20PDA%20Object%20Reference) (DeltaSeconds :type Float%20%28double-precision%29) (AttachedPlatform :type Actor%20Object%20Reference) (WeaponActor :type Actor%20Object%20Reference))
  (bind _relativerotation (Variables|/Script/Engine.SceneComponent|GetRelativeRotation YawComponent))
  (bind _relativerotation_2 (Variables|/Script/Engine.SceneComponent|GetRelativeRotation PitchComponent))
  (Utilities|FlowControl|Sequence
    (:then_0
      ;[0.15 0.15 0.15 0.5] Rotate Yaw
      (LocalVariables|GetUseYaw
        (:then
          (bind _errorquaternion (CallFunction|PIDErrorEulertoQuat _relativerotation (WeaponControl|FindTargetYaw TargetLocation YawComponent WeaponActor)))
          (LocalVariables|SetYawError (.z _errorquaternion))
          (if (Validation|LimitWeaponRotation (Variables|/Game/Actors/WeaponSystems/__DataAssets/BP_WeaponSystem_Base_PDA.BP_WeaponSystem_Base_PDA_C|GetYawMin WeaponData) (Variables|/Game/Actors/WeaponSystems/__DataAssets/BP_WeaponSystem_Base_PDA.BP_WeaponSystem_Base_PDA_C|GetYawMax WeaponData) (.Yaw (Math|Rotator|BreakRotator _relativerotation)) (.z _errorquaternion))
            (bind _output (CallFunction|UpdatePID (Variables|/Game/Actors/WeaponSystems/__DataAssets/BP_WeaponSystem_Base_PDA.BP_WeaponSystem_Base_PDA_C|GetYawPIDConfig WeaponData) (Variables|/Game/Actors/WeaponSystems/__DataAssets/BP_WeaponSystem_Base_PDA.BP_WeaponSystem_Base_PDA_C|GetYawPIDState WeaponData) (.z _errorquaternion) DeltaSeconds))
            (Class|TSGQuaternionLibrary|AddLocalRotationQuat YawComponent (Class|KismetMathLibrary|MakeQuat 0.0 0.0 (* _output (Class|GameplayStatics|GetGlobalTimeDilation)) (* (.w _errorquaternion) -1.0)))))
        (:else)))
    (:then_1
      ;[0.15 0.15 0.15 0.5] Rotate Pitch
      (LocalVariables|GetUsePitch
        (:then
          (bind _errorrotator (CallFunction|PIDErrorEuler _relativerotation_2 (WeaponControl|FindTargetPitch TargetLocation PitchComponent WeaponActor)))
          (LocalVariables|SetPitchError (.pitch _errorrotator))
          (if (Validation|LimitWeaponRotation (Variables|/Game/Actors/WeaponSystems/__DataAssets/BP_WeaponSystem_Base_PDA.BP_WeaponSystem_Base_PDA_C|GetPitchMin WeaponData) (Variables|/Game/Actors/WeaponSystems/__DataAssets/BP_WeaponSystem_Base_PDA.BP_WeaponSystem_Base_PDA_C|GetPitchMax WeaponData) (.Pitch (Math|Rotator|BreakRotator _relativerotation_2)) (.pitch _errorrotator))
            (bind _output_2 (CallFunction|UpdatePID (Variables|/Game/Actors/WeaponSystems/__DataAssets/BP_WeaponSystem_Base_PDA.BP_WeaponSystem_Base_PDA_C|GetPitchPIDConfig WeaponData) (Variables|/Game/Actors/WeaponSystems/__DataAssets/BP_WeaponSystem_Base_PDA.BP_WeaponSystem_Base_PDA_C|GetPitchPIDState WeaponData) (.pitch _errorrotator) DeltaSeconds))
            (Transformation|AddRelativeRotation PitchComponent (Math|Rotator|MakeRotator 0.0 (* _output_2 (Class|GameplayStatics|GetGlobalTimeDilation)) 0.0) false false)))
        (:else)))
    (:then_2
      ;[0.15 0.15 0.15 0.5] Confirm that the weapon is within a firing angle
      (return (Math|Boolean|ANDBoolean (< (LocalVariables|GetYawError) (Variables|/Game/Actors/WeaponSystems/__DataAssets/BP_WeaponSystem_Base_PDA.BP_WeaponSystem_Base_PDA_C|GetYawError WeaponData)) (> (LocalVariables|GetYawError) (* (Variables|/Game/Actors/WeaponSystems/__DataAssets/BP_WeaponSystem_Base_PDA.BP_WeaponSystem_Base_PDA_C|GetYawError WeaponData) -1.0)) (> (LocalVariables|GetPitchError) (* (Variables|/Game/Actors/WeaponSystems/__DataAssets/BP_WeaponSystem_Base_PDA.BP_WeaponSystem_Base_PDA_C|GetPitchError WeaponData) -1.0)) (< (LocalVariables|GetPitchError) (Variables|/Game/Actors/WeaponSystems/__DataAssets/BP_WeaponSystem_Base_PDA.BP_WeaponSystem_Base_PDA_C|GetPitchError WeaponData)))))))