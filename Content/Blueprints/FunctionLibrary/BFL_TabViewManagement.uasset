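; BFL_TabViewManagement is a Blueprint function library for adding labeled tabs to a tab list in the UI.
; Each function registers a content widget under a name ID and index, using either the focusable or non-focus tab button class.
; It then fetches the created button by ID, sets its text and returns it cast to that class.
; The non-focusable variant also passes a change-on-hover setting to the button.
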(fn RegisterFocusableTabwithButtonName
  (params (TabList :type Common%20Tab%20List%20Widget%20Base%20Object%20Reference) (TabContent :type Widget%20Object%20Reference) (TabIndex :type Integer) (TabNameID :type Name) (TabName :type Text))
  (bind _returnvalue (Class|CommonTabListWidgetBase|GetTabButtonBasebyID TabList TabNameID))
  (bind _asbpw_tab_view_button_focusable (Utilities|Casting|CastToBPW_TabViewButtonFocusable _returnvalue))
  (Class|CommonTabListWidgetBase|RegisterTab TabList TabNameID "/Game/HUD/PremadeWidgets/Buttons/BPW_TabViewButtonFocusable.BPW_TabViewButtonFocusable_C" TabContent TabIndex)
  (Default|EventSetButtonText _asbpw_tab_view_button_focusable TabName)
  (return _asbpw_tab_view_button_focusable))

(fn RegisterNonFocusableTabwithButtonName
  (params (TabList :type Common%20Tab%20List%20Widget%20Base%20Object%20Reference) (TabContent :type Widget%20Object%20Reference) (TabIndex :type Integer) (TabNameID :type Name) (TabName :type Text) (ChangeOnHover :type Boolean))
  (bind _returnvalue (Class|CommonTabListWidgetBase|GetTabButtonBasebyID TabList TabNameID))
  (bind _asbpw_tab_view_button_non_focus (Utilities|Casting|CastToBPW_TabViewButtonNonFocus _returnvalue))
  (Class|CommonTabListWidgetBase|RegisterTab TabList TabNameID "/Game/HUD/PremadeWidgets/Buttons/BPW_TabViewButtonNonFocus.BPW_TabViewButtonNonFocus_C" TabContent TabIndex)
  (Default|EventChangeonHover _asbpw_tab_view_button_non_focus ChangeOnHover)
  (Default|EventSetButtonText _asbpw_tab_view_button_non_focus TabName)
  (return _asbpw_tab_view_button_non_focus))