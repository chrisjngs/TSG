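; Blueprint function library of shared data helpers for a ship combat game with weapons, missions and factions.
; Table helpers find a ship's row by name with a script error on failure, fetch the first weapon row, or pick a random mission.
; Other helpers step data asset indices, read weapon UI info, filter actors to other factions and blocking-load projectile assets.
; A Shell sort orders float arrays, returning a map of swapped indices.
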(fn GetRowforShipinTable
  (params (DataTable :type Data%20Table%20Soft%20Object%20Reference) (ShipName :type Name))
  (bind _output (Utilities|ResolveSoftReference DataTable))
  ;[0.15 0.15 0.15 0.5] Find the row in the data table that the given ship name is on. If a row was found, return it and a true boolean. If no row was found with the ship name, throw a script error.
  (bind _outrownames (DataTable|GetDataTableRowNames _output))
  (bind _array_element (Utilities|Array|ForEachLoopwithBreak _outrownames :!label _label)
    (:LoopBody
      (bind _returnvalue (Utilities|GetDataTableRow _output _array_element)
        (:then
          (if (== (.PlatformName (Utilities|Struct|BreakS_ShipConfigurations _returnvalue)) ShipName)
            (Utilities|FlowControl|Sequence
              (:then_0
                (bind _output_get (LocalVariables|SetShipFound true))
                (return _returnvalue _output_get))
              (:then_1
                (goto _label Break)))))))
    (:Completed
      (if (not (LocalVariables|GetShipFound))
        (CallFunction|ThrowScriptError "BFL_DataTableFunctions" "GetRowForShipInTable" "No ship row was found for the given name. Check spelling and confirm row exists." (Utilities|Text|FormatText "The name of a ship in data table \"{DataTable}\"" _output) (Utilities|Text|FormatText "Data table variable \"{table}\" /n Ship name variable \"{ship}\"" _output ShipName))))))

(fn GetNextValidDataAssetArrayIndex
  (params (CurrentDataAsset :type Primary%20Data%20Asset%20Soft%20Object%20Reference) (Array :type Array%20of%20Primary%20Data%20Asset%20Soft%20Object%20References))
  (bind _returnvalue (Utilities|Array|FindItem Array CurrentDataAsset))
  (bind _returnvalue_2 (+ _returnvalue 1))
  ;[0.15 0.15 0.15 0.5] First check that the current item index is greater than 0, if it is then check that it isn't greater than or equal to the last index, if both those pass then add 1 to the current index, otherwise set it to 0.
  (if (< _returnvalue 0)
    (LocalVariables|SetValidIndex 0 :!label _label)
    (elif (<= _returnvalue_2 (Utilities|Array|LastIndex Array))
      (LocalVariables|SetValidIndex _returnvalue_2)
      (else
        (goto _label))))
  (return (LocalVariables|GetValidIndex)))

(fn GetPreviusValidDataAssetArrayIndex
  (params (CurrentDataAsset :type Primary%20Data%20Asset%20Soft%20Object%20Reference) (Array :type Array%20of%20Primary%20Data%20Asset%20Soft%20Object%20References))
  (if (== (Utilities|Array|FindItem Array CurrentDataAsset) 0)
    (LocalVariables|SetValidIndex (Utilities|Array|LastIndex Array))
    (else
      (LocalVariables|SetValidIndex 0)))
  (return (LocalVariables|GetValidIndex)))

(fn GetWeaponDataTable
  (bind _weapondatatable (LocalVariables|GetWeaponDataTable))
  (bind _outrownames (DataTable|GetDataTableRowNames _weapondatatable))
  (for _array_element _outrownames
    (bind _returnvalue (Utilities|GetDataTableRow _weapondatatable _array_element)
      (:then
        (return _returnvalue (.OffensiveWeaponDataAssets (Utilities|Struct|BreakS_WeaponDataAssets _returnvalue)) (.DefensiveWeaponDataAssets (Utilities|Struct|BreakS_WeaponDataAssets _returnvalue)) (.MissileSiloDataAssets (Utilities|Struct|BreakS_WeaponDataAssets _returnvalue)))))))

(fn GetRandomMission
  (bind _outrownames (DataTable|GetDataTableRowNames (LocalVariables|GetMissionDataTable)))
  (bind _returnvalue (Utilities|GetDataTableRow (LocalVariables|GetMissionDataTable) (Utilities|Array|Get(acopy) _outrownames (Math|Random|RandomIntegerinRange 0 (- (Utilities|Array|Length _outrownames) 1))))
    (:then
      (return _returnvalue))))

(fn GetWeaponInfofromChildActorComponent
  (params (Weapon :type Actor%20Object%20Reference))
  (bind _asbp_weapon_parent_base (Utilities|Casting|CastToBP_WeaponParent_Base Weapon)
    (:then
      (bind (_weaponsystem_coreinfo _weaponsystem_infoprivate _weaponsystem_infopublic) (Default|GetDataforUI _asbp_weapon_parent_base))
      (return true _weaponsystem_coreinfo _weaponsystem_infoprivate _weaponsystem_infopublic (Variables|/Game/Blueprints/Components/HealthSystem/BP_Health_AC.BP_Health_AC_C|GetCurrentHealth (Variables|/Game/Actors/WeaponSystems/__ParentActors/BP_WeaponParent_Base.BP_WeaponParent_Base_C|GetBP_Health_AC _asbp_weapon_parent_base))))
    (:CastFailed
      (Development|PrintString 0 "Failed to cast component to BP_WeaponParent_Base" true true "(R=0.739130,G=0.002563,B=0.000000,A=1.000000)")
      (return false "" "" "" 0.0))))

(fn SortFloatArray-Shell
  (params (FloatArray :type Array%20of%20Floats%20%28double-precision%29))
  (bind _output_get (LocalVariables|SetSize (Utilities|Array|Length FloatArray)))
  (LocalVariables|SetS (/ _output_get 2))
  (while (> (LocalVariables|GetS) 0)
    (for _index (range (LocalVariables|GetS) (- (LocalVariables|GetSize) 1))
      (LocalVariables|SetJ (- _index (LocalVariables|GetS)))
      (while (and (>= (LocalVariables|GetJ) 0) (> (Utilities|Array|Get(acopy) FloatArray (Math|Integer|Absolute(Integer) (LocalVariables|GetJ))) (Utilities|Array|Get(acopy) FloatArray (+ (LocalVariables|GetJ) (LocalVariables|GetS)))))
        (Utilities|Array|Swap FloatArray (LocalVariables|GetJ) (+ (LocalVariables|GetJ) (LocalVariables|GetS)))
        (Utilities|Map|Add (LocalVariables|GetIndexChangeMap) (LocalVariables|GetJ) (+ (LocalVariables|GetJ) (LocalVariables|GetS)))
        (LocalVariables|SetJ (- (LocalVariables|GetJ) (LocalVariables|GetS)))))
    (LocalVariables|SetS (/ (LocalVariables|GetS) 2)))
  (return (LocalVariables|GetIndexChangeMap)))

(fn ValidateActorArrayItems
  (params (ActorArray :type Array%20of%20Actor%20Object%20References) (ControllingPawn :type Actor%20Object%20Reference))
  (for _array_element ActorArray
    (Utilities|IsValid _array_element
      (:Is%20Valid
        (bind _validcontact (Arrays|Validation|ContactIsDifferentFaction ControllingPawn _array_element))
        (if _validcontact
          (Utilities|Array|AddUnique (LocalVariables|GetTempArray) _array_element)))))
  (return (LocalVariables|GetTempArray)))

(fn ContactIsDifferentFaction
  (params (Ship :type Actor%20Object%20Reference) (Contact :type Actor%20Object%20Reference))
  (bind _faction (Class|BPIWeaponController|GetFaction(Message) Ship))
  (bind _factiontype (Class|BPITargetable|GetFactionType(Message) Contact))
  (return (Utilities|Enum|NotEqual(Enum) _factiontype _faction)))

(fn GetProjectilefromWeapon
  (params (Target :type BP%20Weapon%20System%20Base%20PDA%20Object%20Reference))
  (bind _projectiledataasset (Variables|/Game/Actors/WeaponSystems/__DataAssets/BP_WeaponSystem_Base_PDA.BP_WeaponSystem_Base_PDA_C|GetProjectileDataAsset Target))
  (if (Utilities|IsValidSoftObjectReference _projectiledataasset)
    (bind _returnvalue (Utilities|LoadAssetBlocking _projectiledataasset))
    (bind _asprojectile_pda (Utilities|Casting|CastToProjectile_PDA _returnvalue))
    (return _asprojectile_pda)))