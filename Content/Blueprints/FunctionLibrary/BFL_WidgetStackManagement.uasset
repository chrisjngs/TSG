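; Blueprint function library that gives a single entry point for managing layered UI widget stacks and input focus per player.
; Layer functions register layers, push or pop content, and clear layers by forwarding message calls to the player's HUD, mostly after validating the owning player.
; Focus functions cast the player controller to BP_Core_PC to switch between game focus and modal UI focus with pause, cursor and input options.
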(fn RegisterLayer
  (params (OwningPlayer :type Actor%20Object%20Reference) (LayerName :type Gameplay%20Tag%20Structure) (LayerWidget :type WBP%20Layer%20Object%20Reference) (Target :type Player%20Controller%20Object%20Reference))
  (Utilities|IsValid OwningPlayer
    (:Is%20Valid
      (bind _success (Class|BPIUIManager|RegisterLayer(Message) (HUD|GetHUD Target) LayerName LayerWidget))
      (return _success))))

(fn PushContenttoLayer
  (params (OwningPlayer :type Player%20Controller%20Object%20Reference) (LayerName :type Gameplay%20Tag%20Structure) (WidgetClass :type User%20Widget%20Soft%20Class%20Reference))
  (Utilities|IsValid OwningPlayer
    (:Is%20Valid
      (bind _widget (Class|BPIUIManager|PushContenttoLayer(Message) (HUD|GetHUD OwningPlayer) LayerName WidgetClass))
      (return _widget))))

(fn PopContentfromLayer
  (params (OwningPlayer :type Player%20Controller%20Object%20Reference) (LayerName :type Gameplay%20Tag%20Structure%20%28by%20ref%29))
  (Utilities|IsValid OwningPlayer
    (:Is%20Valid
      (Class|BPIUIManager|PopContentfromLayer(Message) (HUD|GetHUD OwningPlayer) LayerName))))

(fn ClearAllLayers
  (params (OwningPlayer :type Player%20Controller%20Object%20Reference))
  (Utilities|IsValid OwningPlayer
    (:Is%20Valid
      (Class|BPIUIManager|ClearAllLayers(Message) (HUD|GetHUD OwningPlayer)))))

(fn ClearLayer
  (params (OwningPlayer :type Player%20Controller%20Object%20Reference) (LayerName :type Gameplay%20Tag%20Structure%20%28by%20ref%29))
  (Utilities|IsValid OwningPlayer
    (:Is%20Valid
      (Class|BPIUIManager|ClearLayer(Message) (HUD|GetHUD OwningPlayer) LayerName))))

(fn FocusGame
  (params (OwningPlayer :type Player%20Controller%20Object%20Reference))
  (bind _asbp_core_pc (Utilities|Casting|CastToBP_Core_PC OwningPlayer))
  (Default|FocusGame _asbp_core_pc))

(fn ClearAllLayersExcept
  (params (OwningPlayer :type Player%20Controller%20Object%20Reference) (ExecptionLayerName :type Gameplay%20Tag%20Structure))
  (Utilities|IsValid OwningPlayer
    (:Is%20Valid
      (Class|BPIUIManager|ClearAllLayersExcept(Message) (HUD|GetHUD OwningPlayer) ExecptionLayerName))))

(fn FocusModal
  (params (OwningPlayer :type Player%20Controller%20Object%20Reference) (WidgetToFocus :type Widget%20Object%20Reference) (bPauseGame :type Boolean) (bShowMouseCursor :type Boolean) (bUIOnlyInput :type Boolean))
  (bind _asbp_core_pc (Utilities|Casting|CastToBP_Core_PC OwningPlayer))
  (Default|FocusModal _asbp_core_pc WidgetToFocus bPauseGame bShowMouseCursor bUIOnlyInput))