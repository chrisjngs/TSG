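; Blueprint function library for data table lookups, with a function that finds a ship's row by its name.
; GetRowForShipInTable loops over the table's row names, compares each row's ShipName field to the given name, and returns the first match with a found flag.
; When nothing matches, it throws a script error reporting the table and the name searched for.
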(fn GetRowforShipinTable
  (params (DataTable :type Data%20Table%20Soft%20Object%20Reference) (ShipName :type Name))
  (bind _output (Utilities|ResolveSoftReference DataTable))
  ;[0.15 0.15 0.15 0.5] Find the row in the data table that the given ship name is on. If a row was found, return it and a true boolean. If no row was found with the ship name, throw a script error.
  (bind _outrownames (DataTable|GetDataTableRowNames _output))
  (bind _array_element (Utilities|Array|ForEachLoopwithBreak _outrownames :!label _label)
    (:LoopBody
      (bind _returnvalue (Utilities|GetDataTableRow _output _array_element)
        (:then
          (if (== (.ShipName (Utilities|Struct|BreakS_ShipConfigurations _returnvalue)) ShipName)
            (Utilities|FlowControl|Sequence
              (:then_0
                (bind _output_get (LocalVariables|SetShipFound true))
                (return _returnvalue _output_get))
              (:then_1
                (goto _label Break)))))))
    (:Completed
      (if (not (LocalVariables|GetShipFound))
        (CallFunction|ThrowScriptError "BFL_DataTableFunctions" "GetRowForShipInTable" "No ship row was found for the given name. Check spelling and confirm row exists." (Utilities|Text|FormatText "The name of a ship in data table \"{DataTable}\"" _output) (Utilities|Text|FormatText "Data table variable \"{table}\" /n Ship name variable \"{ship}\"" _output ShipName))))))