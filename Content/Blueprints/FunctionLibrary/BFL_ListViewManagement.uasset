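; Blueprint function library that adds entries to list views showing ship component details and component overviews.
; Each function constructs a data entry object with the list view as outer, initializes it and adds it as an item.
; Detail entries carry text, color, an optional icon and a single or split current/max value.
; Overview entries carry a component name, preview image and data asset.
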(fn AddItemtoShipCompListView
  (params (ListView :type List%20View%20Object%20Reference) (List%20View%20Struct%20Text :type Text) (TextColor :type Slate%20Color%20Structure) (UseIcon :type Boolean) (WidgetIcon :type Texture%202D%20Object%20Reference) (UseSplitValue :type Boolean) (Value :type Float%20%28double-precision%29) (CurrentValue :type Float%20%28double-precision%29) (MaxValue :type Float%20%28double-precision%29))
  (bind _returnvalue (Game|ConstructObjectfromClass ListView "/Game/HUD/PremadeWidgets/ListViews/BP_ListViewShipCompDataEntry.BP_ListViewShipCompDataEntry_C"))
  (bind _output_get (LocalVariables|SetListViewDataEntry _returnvalue))
  (Default|Init _output_get List%20View%20Struct%20Text false TextColor UseIcon WidgetIcon UseSplitValue Value CurrentValue MaxValue)
  (Class|ListView|AddItem ListView _output_get))

(fn AddItemtoShipCompOverviewListView
  (params (ListView :type List%20View%20Object%20Reference) (ComponentName :type Text) (PreviewImage :type Texture%202D%20Object%20Reference) (ComponentData :type Primary%20Data%20Asset%20Soft%20Object%20Reference))
  (bind _returnvalue (Game|ConstructObjectfromClass ListView "/Game/HUD/PremadeWidgets/ListViews/BP_ListViewComponentOverviewDataEntry.BP_ListViewComponentOverviewDataEntry_C"))
  (bind _output_get (LocalVariables|SetListViewDataEntry _returnvalue))
  (Default|Init _output_get ComponentName PreviewImage ComponentData)
  (Class|ListView|AddItem ListView _output_get))