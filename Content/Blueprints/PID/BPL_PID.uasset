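; Blueprint function library for a generic scalar PID controller with helpers for computing rotation error.
; UpdatePID accumulates the integral and derives the error rate in a by-ref state struct, then returns the gain-weighted sum clamped to the config's output limits.
; ResetPID overwrites that state with given values.
; Error helpers give either a per-axis rotator difference, without angle wrapping, or a quaternion error from the target's conjugate times the current rotation.
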(fn UpdatePID
  (params (PIDConfig :type BPS%20PID%20Config%20Structure) (PIDState :type BPS%20PID%20State%20Structure%20%28by%20ref%29) (e :type Float%20%28double-precision%29%20%28by%20ref%29) (DeltaSeconds :type Float%20%28double-precision%29%20%28by%20ref%29))
  (bind _returnvalue (* e DeltaSeconds))
  (bind _returnvalue_2 (+ (.e_accumulator PIDState) _returnvalue))
  (Utilities|FlowControl|Sequence
    (:then_0
      ;[0.15 0.15 0.15 0.5] Update Integral, by summing error over time... and save new value to the State accumulator
      (LocalVariables|SetIntegral _returnvalue_2)
      (|SetBy-RefVar (.e_accumulator PIDState) _returnvalue_2))
    (:then_1
      ;[0.15 0.15 0.15 0.5] Compute Derivative, and save error as LastError in State Structure
      (LocalVariables|SetDerivative (/ (- e (.lasterror PIDState)) DeltaSeconds))
      (|SetBy-RefVar (.lasterror PIDState) e))
    (:then_2
      ;[0.15 0.15 0.15 0.5] Sum the Error, Inegral, and Derivative times their PID constans, sum them, and clamp the output
      (return (Math|Float|Clamp(Float) (+ (* (.kp PIDConfig) e) (* (.ki PIDConfig) (LocalVariables|GetIntegral)) (* (.kd PIDConfig) (LocalVariables|GetDerivative))) (.minoutput PIDConfig) (.maxoutput PIDConfig))))))

(fn ResetPID
  (params (PIDState :type BPS%20PID%20State%20Structure%20%28by%20ref%29) (New%20Error%20Value :type Float%20%28double-precision%29%20%28by%20ref%29) (New%20Accumulator%20Value :type Float%20%28double-precision%29%20%28by%20ref%29))
  (|SetBy-RefVar PIDState (Utilities|Struct|MakeBPS_PIDState New%20Error%20Value New%20Accumulator%20Value)))

(fn PIDErrorEuler
  (params (CurrentRotator :type Rotator) (TargetRotator :type Rotator))
  (bind (_roll _pitch _yaw) (Math|Rotator|BreakRotator TargetRotator))
  (bind (_roll_2 _pitch_2 _yaw_2) (Math|Rotator|BreakRotator CurrentRotator))
  (return (Math|Rotator|MakeRotator (- _roll _roll_2) (- _pitch _pitch_2) (- _yaw _yaw_2))))

(fn PIDErrorEulertoQuat
  (params (CurrentRotator :type Rotator) (TargetRotator :type Rotator))
  (bind _returnvalue (Class|TSGQuaternionLibrary|EulertoQuaternion CurrentRotator))
  (LocalVariables|SetCurrentQuat _returnvalue)
  (bind _returnvalue_2 (Class|TSGQuaternionLibrary|EulertoQuaternion TargetRotator))
  (LocalVariables|SetTargetQuat _returnvalue_2)
  (return (* (Class|KismetMathLibrary|MakeQuat (* (.x (LocalVariables|GetTargetQuat)) -1.0) (* (.y (LocalVariables|GetTargetQuat)) -1.0) (* (.z (LocalVariables|GetTargetQuat)) -1.0) (.w (LocalVariables|GetTargetQuat))) (LocalVariables|GetCurrentQuat))))