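; BP_Core_GM is a Game Mode that tracks core player controllers and provides player spawning.
; Post-login and controller-swap events append each BP_Core_PC to a controller array.
; SpawnPlayer destroys any controlled pawn, then spawns and returns a core pawn and a ship-system command platform, without possessing either.
; Spawn transforms come from randomly chosen PlayerStarts, re-rolled separately for pawn, platform and returned transform.
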(event EventBeginPlay)

(event EventTick
  (params (DeltaSeconds :type Float%20%28single-precision%29)))

(event EventPostLogin
  (params (NewPlayer :type Player%20Controller%20Object%20Reference))
  (bind _asbp_core_pc (Utilities|Casting|CastToBP_Core_PC NewPlayer))
  (Utilities|Array|Add (Variables|Default|GetPlayerController) _asbp_core_pc))

(event EventOnSwapPlayerControllers
  (params (OldPC :type Player%20Controller%20Object%20Reference) (NewPC :type Player%20Controller%20Object%20Reference))
  (bind _asbp_core_pc (Utilities|Casting|CastToBP_Core_PC NewPC))
  (Utilities|Array|Add (Variables|Default|GetPlayerController) _asbp_core_pc))

(fn ConstructionScript)

(fn FindPlayerStart
  (bind _outactors (Actor|GetAllActorsOfClass "/Script/Engine.PlayerStart"))
  (return (Transformation|GetActorTransform (Utilities|Array|Get(acopy) _outactors (Math|Random|RandomIntegerinRange 0 (- (Utilities|Array|Length _outactors) 1))))))

(fn SpawnPlayer
  (params (Player%20Controller :type Player%20Controller%20Object%20Reference))
  (bind _returnvalue (Pawn|GetControlledPawn Player%20Controller))
  (bind _player_start_transform (Spawning|FindPlayerStart))
  (Utilities|IsValid _returnvalue
    (:Is%20Valid
      (Actor|DestroyActor _returnvalue))
    (:Is%20Not%20Valid
      _))
  (bind _returnvalue_2 (Game|SpawnActorfromClass "/Game/Blueprints/Player/BP_Core_Pawn.BP_Core_Pawn_C" _player_start_transform "Undefined" "MultiplyWithRoot" 0 0))
  (bind _returnvalue_3 (Game|SpawnActorfromClass :Class "/Game/Actors/Ships/Ship_Core/Blueprints/BP_ShipSystem_Base.BP_ShipSystem_Base_C" :SpawnTransform _player_start_transform :CollisionHandlingOverride "Undefined" :TransformScaleMethod "MultiplyWithRoot" :Instigator 0))
  (return _returnvalue_2 _returnvalue_3 _player_start_transform))