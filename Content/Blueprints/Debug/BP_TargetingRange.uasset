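; BP_TargetingRange is a debug volume that populates a target range with ships when the player pawn enters its box.
; A one-time overlap sends its Faction to the space station, then spawns BP_ShipSystem_Base targets of that faction with random position, rotation and scale within the actor's bounds.
; Debug spheres re-roll the random location, so they do not mark actual spawns.
; The construction script sizes the box from BoxSize; ActorToSpawn is unused.
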(event OnComponentBeginOverlap(Box)
  (params (OverlappedComponent :type Primitive%20Component%20Object%20Reference) (OtherActor :type Actor%20Object%20Reference) (OtherComp :type Primitive%20Component%20Object%20Reference) (OtherBodyIndex :type Integer) (bFromSweep :type Boolean) (SweepResult :type Hit%20Result%20Structure%20%28by%20ref%29))
  (bind (_origin _boxextent) (Collision|GetActorBounds false false))
  (bind _returnvalue (Math|Random|RandomFloatinRange -3.6e+02 3.6e+02))
  (bind _spawnedscalemin (Variables|Default|GetSpawnedScaleMin))
  (bind _spawnedscalemax (Variables|Default|GetSpawnedScaleMax))
  (bind _returnvalue_2 (Math|Random|RandomPointinBoundingBox _origin _boxextent))
  (bind _returnvalue_3 (Math|Random|RandomFloatinRange _spawnedscalemin _spawnedscalemax))
  (bind _returnvalue_4 (Math|Conversions|ToVector(Float) _returnvalue_3))
  (bind _returnvalue_5 (Math|Transform|MakeTransform _returnvalue_2 (Math|Rotator|MakeRotator _returnvalue _returnvalue _returnvalue) _returnvalue_4))
  (Utilities|FlowControl|DoOnce false
    (:Completed
      (if (== (Game|Player|GetPlayerPawn 0) OtherActor)
        (bind _returnvalue_6 (Actor|GetActorOfClass "/Game/Actors/Structures/ProxySpaceStation/Blueprints/BP_SpaceStation.BP_SpaceStation_C"))
        (Class|BPITargetable|SetFactionType(Message) _returnvalue_6 (Variables|Default|GetFaction))
        (for _index (range 0 (- (Variables|Default|GetNumberOfTargets) 1))
          (Game|SpawnActorfromClass :Class "/Game/Actors/Ships/Ship_Core/Blueprints/BP_ShipSystem_Base.BP_ShipSystem_Base_C" :SpawnTransform _returnvalue_5 :CollisionHandlingOverride "AlwaysSpawn" :TransformScaleMethod "MultiplyWithRoot" :Faction (Variables|Default|GetFaction) :Instigator 0)
          (Rendering|Debug|DrawDebugSphere (.Location (Math|Transform|BreakTransform _returnvalue_5)) 1e+04 12 "(R=1.000000,G=0.002286,B=0.822059,A=1.000000)" 5.0 2e+02))))))

(event EventBeginPlay)

(fn ConstructionScript
  (Components|Box|SetBoxExtent (Variables|Default|GetBox) (Math|Conversions|ToVector(Float) (Variables|Default|GetBoxSize)) true))