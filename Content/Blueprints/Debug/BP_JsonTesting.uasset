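; Debug Blueprint that tests reading point positions from a JSON file created by a PCG graph.
; On BeginPlay it loads the file, walks the top-level fields and appends each non-empty "$Position" to VectorOfPoint as a vector.
; The inner loop ignores its element, so a position is added once per sub-field.
; An unconnected alternative parses a modified layout under "Test Points" and prints the vectors.
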(event EventBeginPlay
  ;[0.15 0.15 0.15 0.5] This works with the default Json file that is created by the PCG graph.
  (bind (_outjsonobject _returnvalue) (Class|JsonBlueprintFunctionLibrary|FromFile (Variables|Default|GetFile)))
  (if _returnvalue
    (bind _fieldnames (Class|JsonBlueprintFunctionLibrary|GetFieldNames _outjsonobject))
    (for _array_element _fieldnames
      (bind _outvalue (|GetJsonField _outjsonobject _array_element))
      (bind _fieldnames_2 (Class|JsonBlueprintFunctionLibrary|GetFieldNames _outvalue))
      (for _array_element_2 _fieldnames_2
        (bind _outvalue_2 (|GetJsonField _outvalue "$Position"))
        (if (Utilities|Array|IsNotEmpty _outvalue_2)
          (Utilities|Array|Add (Variables|Default|GetVectorOfPoint) (Math|Vector|MakeVector (Math|Conversions|ToFloat(Integer) (Utilities|Array|Get(acopy) _outvalue_2)) (Math|Conversions|ToFloat(Integer) (Utilities|Array|Get(acopy) _outvalue_2 1)) (Math|Conversions|ToFloat(Integer) (Utilities|Array|Get(acopy) _outvalue_2 2)))))))))

(fn ConstructionScript)