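; Debug actor that shows a colored sphere as a visual indicator in the game.
; On BeginPlay it creates a dynamic instance of MI_DebugVisualIndicator and assigns it to the sphere.
; Events set the material's Color parameter to green, red, yellow or a custom color.
; ShowDebug passes its Hidden argument straight to SetActorHiddenInGame, so true hides the indicator despite the event's name.
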(event Custom|SetGreen
  (Rendering|Material|SetVectorParameterValue (Variables|Default|GetDebugMaterial) "Color" "(R=0.000000,G=1.000000,B=0.000000,A=1.000000)" :!class /Script/Engine.MaterialInstanceDynamic))

(event Custom|SetRed
  (Rendering|Material|SetVectorParameterValue (Variables|Default|GetDebugMaterial) "Color" "(R=1.000000,G=0.000000,B=0.000000,A=1.000000)" :!class /Script/Engine.MaterialInstanceDynamic))

(event Custom|SetYellow
  (Rendering|Material|SetVectorParameterValue (Variables|Default|GetDebugMaterial) "Color" "(R=1.000000,G=1.000000,B=0.000000,A=1.000000)" :!class /Script/Engine.MaterialInstanceDynamic))

(event Custom|ShowDebug
  (params (Hidden? :type Boolean))
  (Rendering|SetActorHiddenInGame Hidden?))

(event Custom|SetCustom
  (params (CustomColor :type Linear%20Color%20Structure))
  (Rendering|Material|SetVectorParameterValue (Variables|Default|GetDebugMaterial) "Color" CustomColor :!class /Script/Engine.MaterialInstanceDynamic))

(event EventBeginPlay
  (bind _returnvalue (Rendering|Material|CreateDynamicMaterialInstance (Variables|Default|GetSphere) 0 "/Game/Blueprints/Debug/Materials/MI_DebugVisualIndicator.MI_DebugVisualIndicator" "None" :!class /Script/Engine.PrimitiveComponent))
  (bind _output_get (Variables|Default|SetDebugMaterial _returnvalue))
  (Rendering|Material|SetMaterial (Variables|Default|GetSphere) 0 _output_get))

(fn ConstructionScript)