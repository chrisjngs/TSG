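; BF_Debug is a Blueprint function library of independent debug helpers.
; Print helpers report focused widgets with the current CommonUI input type, active Enhanced Input mapping contexts with priorities, the player controller transform, and quaternion components.
; Other helpers draw RGB axis lines for an actor or static mesh component and fetch a BP_DebugVisualIndicator from a child actor.
; It also supplies lorem ipsum placeholder text and raises formatted script errors.
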(fn PrintActiveFocusWidget
  (params (WidgetClass :type Array%20of%20User%20Widget%20Class%20References))
  (LocalVariables|SetHasUserFocus false)
  (Utilities|Array|Clear (LocalVariables|GetWidgetsInFocus))
  (if (Utilities|Array|IsEmpty WidgetClass)
    _
    (else
      (LocalVariables|SetWidgetsToCheck WidgetClass)))
  (for _array_element (LocalVariables|GetWidgetsToCheck)
    (bind _foundwidgets (Widget|GetAllWidgetsOfClass 0 _array_element false))
    (for _array_element_2 _foundwidgets
      (if (or (Class|Widget|HasFocusedDescendants _array_element_2) (Class|Widget|HasAnyUserFocus _array_element_2))
        (Utilities|Array|Add (LocalVariables|GetWidgetsInFocus) (Utilities|GetDisplayName _array_element_2))
        (LocalVariables|SetHasUserFocus true)))
    (if (LocalVariables|GetHasUserFocus)
      (for _array_element_3 (LocalVariables|GetWidgetsInFocus)
        (Development|PrintString 0 (Utilities|String|Append "The focused Widgets are: " _array_element_3) true false "(R=0.000000,G=0.660000,B=1.000000,A=1.000000)" 0.0))
      (Development|PrintString 0 (Utilities|String|Append "The Current input method is: " (Utilities|String|EnumtoString (Class|CommonInputSubsystem|GetCurrentInputType (PlayerController|LocalPlayerSubsystems|GetCommonInputSubsystem (Game|GetPlayerController 0))))) true true "(R=1.000000,G=0.793355,B=0.089685,A=1.000000)" 0.0))))

(fn LoremIpsumGenerator
  (return (Utilities|Text|FormatText "Lorem ipsum dolor sit amet, consectetur adipiscing elit. Maecenas tristique, nunc at semper eleifend, nulla tortor fermentum nisl, non tempus nisi nisi sed leo. Nullam libero tellus, luctus nec dolor non, iaculis sagittis dui. Aliquam accumsan pharetra est nec bibendum. Mauris ut augue purus. Pellentesque aliquet venenatis est eu cursus. Aliquam nibh mi, scelerisque et libero in, tincidunt ultrices justo. Donec viverra, sapien vitae tristique iaculis, ex massa aliquam est, et porttitor justo ligula at ante. Nunc accumsan tellus felis, vel auctor nisi lacinia vel. Vestibulum aliquet nisi sed nisi auctor maximus. Etiam sed orci ligula. Fusce sed ullamcorper felis. Curabitur iaculis turpis felis, et placerat neque fermentum sit amet. Nam tempus gravida diam id fermentum. Donec tortor ante, congue eu sapien vitae, facilisis ornare ante. Nullam condimentum, leo mattis suscipit rhoncus, libero erat aliquet massa, eu fermentum ligula metus id dolor. 
 
Pellentesque consectetur convallis mi in varius. Cras ut nulla consequat augue vulputate iaculis eget nec augue. Phasellus ultrices urna massa, at pellentesque ex tristique vitae. Nunc maximus nunc sit amet neque luctus, et sagittis ligula molestie. Integer lobortis est sed leo ultricies, quis sollicitudin tortor facilisis. Fusce sollicitudin ipsum eu ante facilisis, id sollicitudin turpis posuere. Vestibulum euismod quam at pellentesque porttitor. Maecenas nec tempor mauris. Quisque facilisis iaculis placerat. Donec sagittis ac tellus non euismod. Duis accumsan ligula vitae turpis semper scelerisque. Etiam hendrerit laoreet risus, id faucibus tortor molestie quis. Sed enim leo, aliquam at neque eu, sollicitudin porta dolor. Aliquam at pellentesque turpis. Duis in hendrerit nisi, at tincidunt libero. 
 
Phasellus viverra ligula et finibus mattis. Quisque vel fringilla dui. Suspendisse fermentum, libero scelerisque mattis lacinia, leo lectus mollis est, sed porttitor nibh ipsum at ex. Aliquam mattis mauris a rutrum finibus. Sed sollicitudin sollicitudin massa, id lacinia lectus elementum sit amet. Proin vulputate vulputate venenatis. Interdum et malesuada fames ac ante ipsum primis in faucibus. Phasellus tincidunt urna sed eros convallis, non vulputate nulla maximus. Mauris commodo odio eu condimentum placerat.")))

(fn DebugActor/ComponentAxis
  (params (Actor :type Actor%20Object%20Reference) (DebugStaticMesh :type Boolean) (StaticMeshComp :type Static%20Mesh%20Component%20Object%20Reference))
  (bind _returnvalue (Transformation|GetWorldLocation StaticMeshComp))
  (bind _returnvalue_2 (Transformation|GetActorLocation Actor))
  (if DebugStaticMesh
    ;[0.15 0.15 0.15 0.5] Debug Static Mesh
    (Rendering|Debug|DrawDebugLine 0 _returnvalue (+ _returnvalue (* (Math|Vector|GetForwardVector StaticMeshComp) 7.5e+02)) "(R=1.000000,G=0.000000,B=0.000000,A=1.000000)" 0.0 5e+01)
    (Rendering|Debug|DrawDebugLine 0 _returnvalue (+ _returnvalue (* (Math|Vector|GetRightVector StaticMeshComp) 7.5e+02)) "(R=0.000000,G=1.000000,B=0.000000,A=1.000000)" 0.0 5e+01)
    (Rendering|Debug|DrawDebugLine 0 _returnvalue (+ _returnvalue (* (Math|Vector|GetUpVector StaticMeshComp) 7.5e+02)) "(R=0.000000,G=0.000000,B=1.000000,A=1.000000)" 0.0 5e+01)
    (else
      ;[0.15 0.15 0.15 0.5] Debug Actor
      (Rendering|Debug|DrawDebugLine 0 _returnvalue_2 (+ _returnvalue_2 (* (Transformation|GetActorForwardVector Actor) 7.5e+02)) "(R=1.000000,G=0.000000,B=0.000000,A=1.000000)" 0.0 5e+01)
      (Rendering|Debug|DrawDebugLine 0 _returnvalue_2 (+ _returnvalue_2 (* (Transformation|GetActorRightVector Actor) 7.5e+02)) "(R=0.000000,G=1.000000,B=0.000000,A=1.000000)" 0.0 5e+01)
      (Rendering|Debug|DrawDebugLine 0 _returnvalue_2 (+ _returnvalue_2 (* (Transformation|GetActorUpVector Actor) 7.5e+02)) "(R=0.000000,G=0.000000,B=1.000000,A=1.000000)" 0.0 5e+01))))

(fn DebugActiveInputMappingContext
  (for _array_element (LocalVariables|GetInputContext)
    (if (.ReturnValue (Class|EnhancedInputSubsystemInterface|HasMappingContext (PlayerController|LocalPlayerSubsystems|GetEnhancedInputLocalPlayerSubsystem (Game|GetPlayerController 0)) _array_element))
      (Development|PrintString 0 (Utilities|String|ToString(Text) (Utilities|Text|FormatText "{context} active at priority {priority}" _array_element (.OutFoundPriority (Class|EnhancedInputSubsystemInterface|HasMappingContext (PlayerController|LocalPlayerSubsystems|GetEnhancedInputLocalPlayerSubsystem (Game|GetPlayerController 0)) _array_element)))) true false "(R=0.000000,G=0.750000,B=0.000000,A=1.000000)" 0.0)
      (else
        (Development|PrintString 0 (Utilities|String|ToString(Text) (Utilities|Text|FormatText "{context} NOT active" _array_element)) true false "(R=0.750000,G=0.000000,B=0.000000,A=1.000000)" 0.0)))))

(fn DebugPlayerCamera
  (params (PlayerShip :type BP%20Ship%20System%20Base%20Object%20Reference))
  (Development|PrintString 0 (Utilities|String|ToString(Transform) (Transformation|GetActorTransform (Game|GetPlayerController 0))) true false "(R=1.000000,G=0.156748,B=0.081841,A=1.000000)" 0.0))

(fn DebugQuaternion
  (params (Quaternion :type Quat%20Structure))
  (bind (_x _y _z _w) (Class|KismetMathLibrary|BreakQuat Quaternion))
  (Development|PrintText 0 (Utilities|Text|FormatText "Quat (x: {x},y: {y},z: {z},w: {w})" _x _y _z _w) true false "(R=0.000000,G=0.660000,B=1.000000,A=1.000000)" 0.0))

(fn DebugUseVisualIndicator
  (params (Target :type Scene%20Component%20Object%20Reference))
  (bind _asbp_debug_visual_indicator (Utilities|Casting|CastToBP_DebugVisualIndicator (Components|GetOwner (Components|GetChildComponent Target 0)))
    (:then
      (return _asbp_debug_visual_indicator))
    (:CastFailed
      (Development|PrintString 0 "The passed scene component is not a child actor assigned BP_DebugVisualIndicator" true true "(R=1.000000,G=0.000000,B=0.000000,A=1.000000)" 2e+01))))

(fn ThrowScriptError
  (params (Error%20Class%20Location :type Text) (Error%20Function :type Text) (Error%20Message :type Text) (Expected :type Text) (Got :type Text))
  (Utilities|Debugging|RaiseScriptError (Utilities|String|ToString(Text) (Utilities|Text|FormatText "An error occurred in {Class Location} > {Function Location}. {Error Message}. Expected {Expected}, got:{Got}" Error%20Class%20Location Error%20Function Error%20Message Expected Got))))