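; Player pawn that serves as the camera and control hub for switching between Commander, Pilot, Targeting and Sensor modes.
; Mode changes swap input mappings and HUD layers, then use looping timers to blend camera settings and move onto the platform's attachment point.
; Commander mode selects hovered units via a collision sphere and issues orders; pilot inputs forward to the piloted platform's PMS component.
; Pausing reattaches the camera to a platform-provided viewpoint.
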(event OnComponentBeginOverlap(CollisionSphere)
  (params (OverlappedComponent :type Primitive%20Component%20Object%20Reference) (OtherActor :type Actor%20Object%20Reference) (OtherComp :type Primitive%20Component%20Object%20Reference) (OtherBodyIndex :type Integer) (bFromSweep :type Boolean) (SweepResult :type Hit%20Result%20Structure%20%28by%20ref%29))
  (bind _returnvalue (Actor|GetParentActor OtherActor))
  (bind _returnvalue_2 (Actor|GetComponentbyClass _returnvalue "/Game/Blueprints/Components/PMS_PlatformMovementSystem/PMS_AC.PMS_AC_C"))
  ;[0.15 0.15 0.15 0.5] Waypoint Mode
  (Utilities|IsValid _returnvalue
    (:Is%20Valid
      (Utilities|IsValid _returnvalue_2
        (:Is%20Valid
          (Class|BPIPMS|SetHovered(Message) _returnvalue_2 true)
          (Variables|Player|Modes|Commander|Components|SetHoveredPMS _returnvalue_2))))))

(event OnComponentEndOverlap(CollisionSphere)
  (params (OverlappedComponent :type Primitive%20Component%20Object%20Reference) (OtherActor :type Actor%20Object%20Reference) (OtherComp :type Primitive%20Component%20Object%20Reference) (OtherBodyIndex :type Integer))
  (bind _returnvalue (Actor|GetParentActor OtherActor))
  (bind _returnvalue_2 (Actor|GetComponentbyClass _returnvalue "/Game/Blueprints/Components/PMS_PlatformMovementSystem/PMS_AC.PMS_AC_C"))
  ;[0.15 0.15 0.15 0.5] Waypoint Mode
  (Utilities|IsValid _returnvalue
    (:Is%20Valid
      (Class|BPIPMS|SetHovered(Message) _returnvalue_2 false)
      (if (== _returnvalue_2 (Variables|Player|Modes|Commander|Components|GetHoveredPMS))
        (Variables|Player|Modes|Commander|Components|SetHoveredPMS 0)))))

(event EventChangeSpeedRange
  (params (RangeChange :type Float%20%28double-precision%29))
  ;[0.15 0.15 0.15 0.5] Pilot Mode
  (Class|BPIPMS|ChangeSpeedRange(Message) (Variables|Player|Modes|Pilot|Components|GetPilotedPMS) RangeChange))

(event EventMoveCamera
  (params (InputAction :type Vector :default "0, 0, 0"))
  ;[0.15 0.15 0.15 0.5] Waypoint Mode
  (Transformation|AddRelativeLocation (Variables|Player|Modes|Commander|Components|GetRoot) (Math|Vector|RotateVector (* InputAction 5e+02) (Math|Rotator|MakeRotator 0.0 0.0 (.yaw (Transformation|GetWorldRotation (Variables|Player|Camera|GetCamera))))) true false))

(event EventPitchDown
  (params (ActionValue :type Float%20%28double-precision%29) (IAState :type E_Player_IAInterface%20Enum :default "NewEnumerator0"))
  ;[0.15 0.15 0.15 0.5] Pilot Mode
  (Class|BPIPMS|PitchDown(Message) (Variables|Player|Modes|Pilot|Components|GetPilotedPMS) ActionValue IAState))

(event EventPitchUp
  (params (ActionValue :type Float%20%28double-precision%29) (IAState :type E_Player_IAInterface%20Enum :default "NewEnumerator0"))
  ;[0.15 0.15 0.15 0.5] Pilot Mode
  (Class|BPIPMS|PitchUp(Message) (Variables|Player|Modes|Pilot|Components|GetPilotedPMS) ActionValue IAState))

(event EventYawLeft
  (params (ActionValue :type Float%20%28double-precision%29) (IAState :type E_Player_IAInterface%20Enum :default "NewEnumerator0"))
  ;[0.15 0.15 0.15 0.5] Pilot Mode
  (Class|BPIPMS|YawLeft(Message) (Variables|Player|Modes|Pilot|Components|GetPilotedPMS) ActionValue IAState))

(event EventYawRight
  (params (ActionValue :type Float%20%28double-precision%29) (IAState :type E_Player_IAInterface%20Enum :default "NewEnumerator0"))
  ;[0.15 0.15 0.15 0.5] Pilot Mode
  (Class|BPIPMS|YawRight(Message) (Variables|Player|Modes|Pilot|Components|GetPilotedPMS) ActionValue IAState))

(event EventPauseGame
  (params (Pause :type Boolean))
  ;[0.15 0.15 0.15 0.5] Pause Camera Update
  (if Pause
    (ModeSwitching|Camera|PauseCameraUpdate false)
    (else
      (ModeSwitching|Camera|PauseCameraUpdate true))))

(event EventCameraLook
  (params (ActionValue :type Vector%202D%20Structure))
  ;[0.15 0.15 0.15 0.5] Camera look
  (switch Utilities|FlowControl|Switch|SwitchonECommonInputType (Class|CommonInputSubsystem|GetCurrentInputType (PlayerController|LocalPlayerSubsystems|GetCommonInputSubsystem (Game|GetPlayerController 0)))
    (:MouseAndKeyboard
      (Variables|Player|Controls|Camera|SetCameraPitchRate -1.0)
      (Variables|Player|Controls|Camera|SetCameraYawRate 2.0))
    (:Gamepad
      (Variables|Player|Controls|Camera|SetCameraPitchRate 1.0)
      (Variables|Player|Controls|Camera|SetCameraYawRate 1.0)))
  (Pawn|Input|AddControllerYawInput (/ (.x ActionValue) (Variables|Player|Controls|Camera|GetCameraYawRate)))
  (Pawn|Input|AddControllerPitchInput (* (/ (.y ActionValue) (Variables|Player|Controls|Camera|GetCameraYawRate)) (Variables|Player|Controls|Camera|GetCameraPitchRate))))

(event EventTick
  (params (DeltaSeconds :type Float%20%28single-precision%29)))

(event EventSelectHold
  (params (IAState :type E_Player_IAInterface%20Enum :default "NewEnumerator0") (HoldTime :type Float%20%28double-precision%29))
  (switch Utilities|FlowControl|Switch|SwitchonE_Player_IAInterface IAState
    (:NewEnumerator0
      (CallFunction|UpdateSelectHoldComponents false HoldTime)
      (Utilities|Array|Add (Variables|Player|Modes|Commander|Components|GetSelectedPMS) (Variables|Player|Modes|Commander|Components|GetHoveredPMS))
      (for _array_element (Variables|Player|Modes|Commander|Components|GetSelectedPMS)
        (Class|BPIPMS|SetSelected(Message) _array_element true)))
    (:NewEnumerator4
      (CallFunction|UpdateSelectHoldComponents true 0.0))))

(event EventSetMode
  (params (Mode :type E_Player_Modes%20Enum :default "NewEnumerator0") (Platform :type Actor%20Object%20Reference))
  ;[0.15 0.15 0.15 0.5] Mode switching
  (Variables|Player|Modes|SetCommandMode Mode)
  (ModeSwitching|HandleModeSwitching Platform))

(event EventSetPilotPlatform
  (params (Platform :type Actor%20Object%20Reference))
  (Variables|Player|Modes|Common|Components|SetCommandPlatform Platform))

(event EventOrderHold
  (params (IAState :type E_Player_IAInterface%20Enum :default "NewEnumerator0") (HoldTime :type Float%20%28double-precision%29))
  (bind _returnvalue (Game|GetPlayerController 0))
  (switch Utilities|FlowControl|Switch|SwitchonE_Player_IAInterface IAState
    (:NewEnumerator0
      (Utilities|FlowControl|DoOnce false :!label _label
        (:Completed
          (CallFunction|PushContenttoLayer _returnvalue "(TagName=\"UI.Layers.Modal\")" "/Game/HUD/Modes/CommanderMode/BPW_OrderHoldMenu.BPW_OrderHoldMenu_C"))))
    (:NewEnumerator4
      (CallFunction|PopContentfromLayer _returnvalue "(TagName=\"UI.Layers.Modal\")")
      (goto _label Reset))))

(event EventSelect
  (params (MultiSelect? :type Boolean))
  (bind _selectedpms (Variables|Player|Modes|Commander|Components|GetSelectedPMS))
  ;[0.15 0.15 0.15 0.5] Waypoint Mode
  (if MultiSelect?
    (Utilities|Array|Add (Variables|Player|Modes|Commander|Components|GetSelectedPMS) (Variables|Player|Modes|Commander|Components|GetHoveredPMS))
    (else
      (if (Utilities|Array|IsNotEmpty (Variables|Player|Modes|Commander|Components|GetSelectedPMS))
        (for _array_element _selectedpms
          (Class|BPIPMS|SetSelected(Message) _array_element false)))
      (Utilities|Array|Clear _selectedpms)
      (Utilities|Array|Add _selectedpms (Variables|Player|Modes|Commander|Components|GetHoveredPMS))))
  (for _array_element_2 (Variables|Player|Modes|Commander|Components|GetSelectedPMS)
    (Class|BPIPMS|SetSelected(Message) _array_element_2 true)))

(event EventIssueOrder
  (params (MultipleOrders :type Boolean))
  ;[0.15 0.15 0.15 0.5] Waypoint Mode
  (for _array_element (Variables|Player|Modes|Commander|Components|GetSelectedPMS)
    (Class|BPIPMS|ChangePossessionState(Message) _array_element "NewEnumerator1" (Game|GetPlayerController 0))
    (Class|BPIPMS|IssueOrder(Message) _array_element "NewEnumerator0" (Transformation|GetWorldLocation (Variables|Player|Modes|Commander|Components|GetControlSphere)) MultipleOrders)))

(event EventDecelerate
  (params (ActionValue :type Float%20%28double-precision%29) (IAState :type E_Player_IAInterface%20Enum :default "NewEnumerator0"))
  ;[0.15 0.15 0.15 0.5] Pilot Mode
  (Class|BPIPMS|Accelerate(Message) (Variables|Player|Modes|Pilot|Components|GetPilotedPMS) ActionValue IAState))

(event EventAccelerate
  (params (ActionValue :type Float%20%28double-precision%29) (IAState :type E_Player_IAInterface%20Enum :default "NewEnumerator0"))
  ;[0.15 0.15 0.15 0.5] Pilot Mode
  (Class|BPIPMS|Accelerate(Message) (Variables|Player|Modes|Pilot|Components|GetPilotedPMS) ActionValue IAState))

(event EventRollLeft
  (params (ActionValue :type Float%20%28double-precision%29) (IAState :type E_Player_IAInterface%20Enum :default "NewEnumerator0"))
  ;[0.15 0.15 0.15 0.5] Pilot Mode
  (Class|BPIPMS|RollLeft(Message) (Variables|Player|Modes|Pilot|Components|GetPilotedPMS) ActionValue IAState))

(event EventRollRight
  (params (ActionValue :type Float%20%28double-precision%29) (IAState :type E_Player_IAInterface%20Enum :default "NewEnumerator0"))
  ;[0.15 0.15 0.15 0.5] Pilot Mode
  (Class|BPIPMS|RollRight(Message) (Variables|Player|Modes|Pilot|Components|GetPilotedPMS) ActionValue IAState))

(fn ConstructionScript
  (bind _collisionsphere (Variables|Player|Modes|Commander|Components|GetCollisionSphere))
  (Collision|SetCollisionEnabled _collisionsphere "NoCollision")
  (Variables|/Script/Engine.PrimitiveComponent|SetbGenerateOverlapEvents _collisionsphere false))

(fn UpdateCameraSettings
  (bind _returnvalue (Utilities|Time|GetRealTimeSeconds))
  (bind _cameratransitionstarttime (Variables|Default|GetCameraTransitionStartTime))
  (bind _camera (Variables|Player|Camera|GetCamera))
  (bind _springarm (Variables|Player|Camera|GetSpringArm))
  (bind _commandercamerasettings (Variables|Player|Modes|Commander|Components|GetCommanderCameraSettings))
  (bind _springarm_2 (Variables|Player|Camera|GetSpringArm))
  (bind (_springarmlength _springarmsocketoffset _fieldofview) (Utilities|Struct|BreakS_PlatformCameraSettings _commandercamerasettings))
  (bind _returnvalue_2 (- _returnvalue _cameratransitionstarttime))
  (bind _returnvalue_3 (Math|Float|MapRangeClamped _returnvalue_2 0.0 1e+01 0.0 1.0))
  (if (Variables|Default|GetInitialCameraSetup)
    (if (Utilities|Enum|NotEqual(Enum) (Variables|Player|Modes|GetCommandMode) "NewEnumerator0")
      (bind _platform_camera_settings (Class|BPIPlatformInfoPassing|GetPlatformCameraSettings(Message) (Variables|Player|Modes|Common|Components|GetLastControlledPlatform)))
      (LocalVariables|SetTargetCameraSettings _platform_camera_settings)
      (else
        (LocalVariables|SetTargetCameraSettings (Variables|Player|Modes|Commander|Components|GetCommanderCameraSettings))))
    (if (== _returnvalue_3 1.0)
      (Utilities|Time|ClearandInvalidateTimerbyHandle (Variables|Default|GetCameraSettingsTimer))
      (else
        (Variables|/Script/Engine.SpringArmComponent|SetTargetArmLength _springarm (Math|Float|Lerp (Variables|/Script/Engine.SpringArmComponent|GetTargetArmLength _springarm) (.SpringArmLength (Utilities|Struct|BreakS_PlatformCameraSettings (LocalVariables|GetTargetCameraSettings))) _returnvalue_3))
        (Variables|/Script/Engine.SpringArmComponent|SetSocketOffset _springarm (Math|Vector|Lerp(Vector) (Variables|/Script/Engine.SpringArmComponent|GetSocketOffset _springarm) (.SpringArmSocketOffset (Utilities|Struct|BreakS_PlatformCameraSettings (LocalVariables|GetTargetCameraSettings))) _returnvalue_3))
        (Camera|SetFieldOfView _camera (Math|Float|Lerp (Variables|/Script/Engine.CameraComponent|GetFieldOfView _camera) (.FieldOfView (Utilities|Struct|BreakS_PlatformCameraSettings (LocalVariables|GetTargetCameraSettings))) _returnvalue_3))))
    (else
      (Variables|Default|SetInitialCameraSetup true)
      (Variables|/Script/Engine.SpringArmComponent|SetTargetArmLength _springarm_2 _springarmlength)
      (Variables|/Script/Engine.SpringArmComponent|SetSocketOffset _springarm_2 _springarmsocketoffset)
      (Camera|SetFieldOfView (Variables|Player|Camera|GetCamera) _fieldofview)
      (Utilities|Time|ClearandInvalidateTimerbyHandle (Variables|Default|GetCameraSettingsTimer)))))

(fn HandleModeSwitching
  (params (Platform :type Actor%20Object%20Reference))
  ;[0.15 0.15 0.15 0.5] Swap camera location, attachment status, UI, and input methods based on the new command mode
  (ModeSwitching|Components|SetLastControlledPlatform Platform)
  (ModeSwitching|Camera|HandleCameraTransition)
  (ModeSwitching|Components|ToggleCommanderUtilities false)
  (ModeSwitching|Components|GetInteractionRadius)
  (switch Utilities|FlowControl|Switch|SwitchonE_Player_Modes (Variables|Player|Modes|GetCommandMode)
    (:NewEnumerator0
      (ModeSwitching|HandleUIandInputChange (LocalVariables|GetNonCommanderMapping)))
    (:NewEnumerator1
      (ModeSwitching|HandleUIandInputChange (LocalVariables|GetNonPilotMapping))
      (Class|BPIPMS|ChangePossessionState(Message) (Variables|Player|Modes|Pilot|Components|GetPilotedPMS) "NewEnumerator0"))
    (:NewEnumerator2
      (ModeSwitching|HandleUIandInputChange (LocalVariables|GetNonTargetingMapping)))
    (:NewEnumerator3
      (ModeSwitching|HandleUIandInputChange (LocalVariables|GetNonSensorMapping)))))

(fn HandleSelectionEvent
  (params (MultiSelect? :type Boolean) (SelectedArray :type Array%20of%20Actor%20Component%20Object%20References) (NewSelection :type Actor%20Component%20Object%20Reference)))

(fn PauseCameraUpdate
  (params (Reset :type Boolean))
  (if Reset
    ;[0.15 0.15 0.15 0.5] Reset the camera to the correct settings for the control mode
    (Transformation|AttachComponentToComponent (Variables|Player|Camera|GetCamera) (Variables|Player|Camera|GetSpringArm) "None" "SnapToTarget" "SnapToTarget" "KeepRelative" true)
    (switch Utilities|FlowControl|Switch|SwitchonE_Player_Modes (Variables|Player|Modes|GetCommandMode)
      (:NewEnumerator0
        (Camera|SetFieldOfView (Variables|Player|Camera|GetCamera) (Utilities|Struct|BreakS_PlatformCameraSettings (Variables|Player|Modes|Commander|Components|GetCommanderCameraSettings)))
        (ModeSwitching|Components|ToggleCommanderUtilities false))
      (:NewEnumerator1
        (bind _platform_camera_settings (Class|BPIPlatformInfoPassing|GetPlatformCameraSettings(Message) (Variables|Player|Modes|Common|Components|GetLastControlledPlatform) :!label _label))
        (Camera|SetFieldOfView (Variables|Player|Camera|GetCamera) (Utilities|Struct|BreakS_PlatformCameraSettings _platform_camera_settings)))
      (:NewEnumerator2
        (goto _label))
      (:NewEnumerator3
        (goto _label)))
    (else
      ;[0.15 0.15 0.15 0.5] Update camera for the pause menu
      (bind _platform (Class|BPIPlatformInfoPassing|GetAttachedPlatform(Message) (Variables|Player|Modes|Common|Components|GetLastControlledPlatform)))
      (bind _pauselocation (Class|BPIShipSystems|GetPauseCameraLocation(Message) (Variables|/Script/Engine.ChildActorComponent|GetChildActor _platform)))
      (Transformation|AttachComponentToComponent (Variables|Player|Camera|GetCamera) _pauselocation "None" "SnapToTarget" "SnapToTarget" "KeepRelative" true)
      (Camera|SetFieldOfView (Variables|Player|Camera|GetCamera) (Utilities|Struct|BreakS_PlatformCameraSettings (Variables|Player|Camera|GetPauseCameraSettings)))
      (ModeSwitching|Components|ToggleCommanderUtilities true))))

(fn ToggleCommanderUtilities
  (params (PauseMode :type Boolean))
  (bind _collisionsphere (Variables|Player|Modes|Commander|Components|GetCollisionSphere))
  (bind _collisionsphere_2 (Variables|Player|Modes|Commander|Components|GetCollisionSphere))
  (if PauseMode
    ;[0.15 0.15 0.15 0.5] Turn off the visibility of all Commander Utilities
    (for _array_element (Variables|Player|Modes|Commander|Components|GetSelectedPMS) :!label _label
      (Class|BPIPMS|SetSelected(Message) _array_element false))
    (Development|SetHiddeninGame (Variables|Player|Modes|Commander|Components|GetControlSphere) true false)
    (Collision|SetCollisionEnabled _collisionsphere "NoCollision")
    (Variables|/Script/Engine.PrimitiveComponent|SetbGenerateOverlapEvents _collisionsphere false)
    (elif (Utilities|Enum|Equal(Enum) (Variables|Player|Modes|GetCommandMode) "NewEnumerator0")
      ;[0.15 0.15 0.15 0.5] Turn on the visibility of all Commander Utilities
      (for _array_element_2 (Variables|Player|Modes|Commander|Components|GetSelectedPMS)
        (Class|BPIPMS|SetSelected(Message) _array_element_2 true))
      (Development|SetHiddeninGame (Variables|Player|Modes|Commander|Components|GetControlSphere) false false)
      (Collision|SetCollisionEnabled _collisionsphere_2 "QueryOnly")
      (Variables|/Script/Engine.PrimitiveComponent|SetbGenerateOverlapEvents _collisionsphere_2 true)
      (else
        (goto _label)))))

(fn SetLastControlledPlatform
  (params (Platform :type Actor%20Object%20Reference))
  (bind _selectedpms (Variables|Player|Modes|Commander|Components|GetSelectedPMS))
  (if (Utilities|Array|IsEmpty _selectedpms)
    (Utilities|IsValid Platform
      (:Is%20Valid
        (Variables|Player|Modes|Common|Components|SetLastControlledPlatform Platform))
      (:Is%20Not%20Valid
        (Variables|Player|Modes|Common|Components|SetLastControlledPlatform (Variables|Player|Modes|Common|Components|GetCommandPlatform))
        (return)))
    (else
      (Variables|Player|Modes|Common|Components|SetLastControlledPlatform (Components|GetOwner (Utilities|Array|Get(acopy) _selectedpms (Utilities|Array|LastIndex _selectedpms)))))))

(fn GetInteractionRadius
  (if (Utilities|Enum|Equal(Enum) (Variables|Player|Modes|GetCommandMode) "NewEnumerator1")
    (bind _interactsphere (Class|BPIPlatformInfoPassing|GetPlatformInteractRadius(Message) (Components|GetOwner (Variables|Player|Modes|Pilot|Components|GetPilotedPMS))))
    (bind _output_get (Variables|Player|Modes|Pilot|Components|SetPilotedInteractRadius _interactsphere))
    (Default|EventInitializeInteractAC (Variables|Player|Modes|Pilot|Components|GetBP_Interact_AC) _output_get)
    (else
      (Variables|Player|Modes|Pilot|Components|SetPilotedInteractRadius 0)))
  (return))

(fn HandleCameraTransition
  (bind _lastcontrolledplatform (Variables|Player|Modes|Common|Components|GetLastControlledPlatform))
  (Utilities|Time|ClearandInvalidateTimerbyHandle (Variables|Default|GetCameraSettingsTimer))
  (Utilities|Time|ClearandInvalidateTimerbyHandle (Variables|Default|GetCameraTransitionTimer))
  (if (Utilities|Enum|NotEqual(Enum) (Variables|Player|Modes|GetCommandMode) "NewEnumerator0")
    (bind _attachmentpoint (Class|BPIPlatformInfoPassing|GetPilotAttachmentPoint(Message) (Variables|Player|Modes|Common|Components|GetLastControlledPlatform)))
    (Variables|Player|Modes|Pilot|Components|SetPilotAttachmentPoint _attachmentpoint)
    (Variables|Default|SetCameraTransitionStartTime (Utilities|Time|GetRealTimeSeconds))
    (bind _returnvalue (Utilities|Time|SetTimerbyFunctionName 0 "TransitionCameraLocation" (Utilities|Time|GetWorldDeltaSeconds) true true))
    (Variables|Default|SetCameraTransitionTimer _returnvalue)
    (if (Utilities|Enum|Equal(Enum) (Variables|Player|Modes|GetCommandMode) "NewEnumerator1")
      (Class|BPIPlatformInfoPassing|PlatformPossessionState(Message) _lastcontrolledplatform "NewEnumerator0" true)
      (else
        (Class|BPIPlatformInfoPassing|PlatformPossessionState(Message) _lastcontrolledplatform "NewEnumerator1" true)))
    (Class|BPIPlatformInfoPassing|GetPlatformCameraSettings(Message) _lastcontrolledplatform)
    (bind _returnvalue_2 (Utilities|Time|SetTimerbyFunctionName 0 "UpdateCameraSettings" (Utilities|Time|GetWorldDeltaSeconds) true true))
    (Variables|Default|SetCameraSettingsTimer _returnvalue_2)
    (Variables|Player|Modes|Pilot|Components|SetPilotedPMS (Actor|GetComponentbyClass _lastcontrolledplatform "/Game/Blueprints/Components/PMS_PlatformMovementSystem/PMS_AC.PMS_AC_C"))
    (else
      (Variables|Default|SetCameraTransitionStartTime (Utilities|Time|GetRealTimeSeconds))
      (Transformation|DetachFromComponent (Variables|Player|Modes|Commander|Components|GetRoot) "KeepWorld" "KeepRelative" "KeepRelative" true)
      (bind _returnvalue_3 (Utilities|Time|SetTimerbyFunctionName 0 "UpdateCameraSettings" (Utilities|Time|GetWorldDeltaSeconds) true true))
      (Variables|Default|SetCameraSettingsTimer _returnvalue_3))))

(fn HandleUIandInputChange
  (params (MappingsToRemove :type Array%20of%20Input%20Mapping%20Context%20Object%20References))
  (bind _returnvalue (Game|GetPlayerController 0))
  (bind _returnvalue_2 (PlayerController|LocalPlayerSubsystems|GetEnhancedInputLocalPlayerSubsystem _returnvalue))
  (for _array_element MappingsToRemove
    (Input|RemoveMappingContext (PlayerController|LocalPlayerSubsystems|GetEnhancedInputLocalPlayerSubsystem (Game|GetPlayerController 0)) _array_element "(bIgnoreAllPressedKeysUntilRelease=True,bForceImmediately=False,bNotifyUserSettings=False)"))
  (CallFunction|PopContentfromLayer _returnvalue "(TagName=\"UI.Layers.Game\")")
  (switch Utilities|FlowControl|Switch|SwitchonE_Player_Modes (Variables|Player|Modes|GetCommandMode)
    (:NewEnumerator0
      (CallFunction|PushContenttoLayer _returnvalue "(TagName=\"UI.Layers.Game\")" "/Game/HUD/Modes/CommanderMode/BPW_CommanderHUD.BPW_CommanderHUD_C")
      (Input|AddMappingContext _returnvalue_2 "/Game/Inputs/IMC_CommanderMode.IMC_CommanderMode" 10 "(bIgnoreAllPressedKeysUntilRelease=True,bForceImmediately=False,bNotifyUserSettings=False)"))
    (:NewEnumerator1
      (CallFunction|PushContenttoLayer _returnvalue "(TagName=\"UI.Layers.Game\")" "/Game/HUD/Modes/PilotMode/BPW_Hud_V1.BPW_Hud_V1_C")
      (Input|AddMappingContext _returnvalue_2 "/Game/Inputs/IMC_PilotMode.IMC_PilotMode" 10 "(bIgnoreAllPressedKeysUntilRelease=True,bForceImmediately=False,bNotifyUserSettings=False)"))
    (:NewEnumerator2
      (CallFunction|PushContenttoLayer _returnvalue "(TagName=\"UI.Layers.Game\")" "/Game/HUD/Modes/TargetingMode/BPW_TargetingMode.BPW_TargetingMode_C")
      (Input|AddMappingContext _returnvalue_2 "/Game/Inputs/IMC_TargetingMode.IMC_TargetingMode" 10 "(bIgnoreAllPressedKeysUntilRelease=True,bForceImmediately=False,bNotifyUserSettings=False)"))
    (:NewEnumerator3
      (CallFunction|PushContenttoLayer _returnvalue "(TagName=\"UI.Layers.Game\")" "/Game/HUD/Modes/PilotMode/BPW_Hud_V1.BPW_Hud_V1_C")
      (Input|AddMappingContext _returnvalue_2 "/Game/Inputs/IMC_SensorMode.IMC_SensorMode" 10 "(bIgnoreAllPressedKeysUntilRelease=True,bForceImmediately=False,bNotifyUserSettings=False)"))))

(fn TransitionCameraLocation
  (bind _returnvalue (Utilities|Time|GetRealTimeSeconds))
  (bind _cameratransitionstarttime (Variables|Default|GetCameraTransitionStartTime))
  (bind _returnvalue_2 (- _returnvalue _cameratransitionstarttime))
  (bind _returnvalue_3 (Math|Float|MapRangeClamped _returnvalue_2 0.0 1e+01 0.0 1.0))
  (if (== _returnvalue_3 1.0)
    (Transformation|AttachComponentToComponent (Variables|Player|Modes|Commander|Components|GetRoot) (Variables|Player|Modes|Pilot|Components|GetPilotAttachmentPoint) "None" "SnapToTarget" "SnapToTarget" "KeepRelative" true)
    (Utilities|Time|ClearandInvalidateTimerbyHandle (Variables|Default|GetCameraTransitionTimer))
    (else
      (Transformation|SetWorldLocation (Variables|Player|Modes|Commander|Components|GetRoot) (Math|Vector|Lerp(Vector) (Transformation|GetWorldLocation (Variables|Player|Modes|Commander|Components|GetRoot)) (Transformation|GetWorldLocation (Variables|Player|Modes|Pilot|Components|GetPilotAttachmentPoint)) _returnvalue_3) true false))))

(fn UpdateSelectHoldComponents
  (params (Reset :type Boolean) (HoldTime :type Float%20%28double-precision%29))
  (bind _returnvalue (Math|Float|MapRangeClamped HoldTime 1.0 1.5 0.0 1.0))
  (bind _controlsphere (Variables|Player|Modes|Commander|Components|GetControlSphere))
  (if Reset
    (Transformation|SetWorldScale3D _controlsphere "20.000000,20.000000,20.000000")
    (elif (>= _returnvalue 1.0)
      (return)
      (else
        (Transformation|SetWorldScale3D _controlsphere (Math|Vector|Lerp(Vector) (Transformation|GetWorldScale _controlsphere) "100.000000,100.000000,100.000000" _returnvalue))))))

(fn GetPilotedPlatform
  (bind _pilotedpms (Variables|Player|Modes|Pilot|Components|GetPilotedPMS))
  (Utilities|IsValid _pilotedpms
    (:Is%20Valid
      (return (Components|GetOwner _pilotedpms)))
    (:Is%20Not%20Valid
      (return (Variables|Player|Modes|Common|Components|GetCommandPlatform)))))

(fn GetPlayerCameraComponents
  (return (Variables|Player|Camera|GetCamera) (Variables|Player|Camera|GetSpringArm)))