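; BP_DamageZone is a damage-zone actor in the health system that hurts actors entering its Cube component.
; On begin overlap, it sends a fixed damage message to any actor implementing BPI_HealthInterface, avoiding casts to specific classes.
; Each Tick, if Move is valid, it offsets its vertical position by a scaled sine of a delta-time-derived value, without sweeping.
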(event OnComponentBeginOverlap(Cube)
  (params (OverlappedComponent :type Primitive%20Component%20Object%20Reference) (OtherActor :type Actor%20Object%20Reference) (OtherComp :type Primitive%20Component%20Object%20Reference) (OtherBodyIndex :type Integer) (bFromSweep :type Boolean) (SweepResult :type Hit%20Result%20Structure%20%28by%20ref%29))
  (if (Utilities|DoesObjectImplementInterface OtherActor "/Game/Blueprints/Components/HealthSystem/BPI_HealthInterface.BPI_HealthInterface_C")
    (Class|BPIHealthInterface|TakeDamage(Message) OtherActor 1e+01)))

(event EventBeginPlay)

(event Collision|EventActorBeginOverlap
  (params (OtherActor :type Actor%20Object%20Reference)))

(event EventTick
  (params (DeltaSeconds :type Float%20%28single-precision%29))
  (Variables|Default|SetDelta%20Seconds (+ DeltaSeconds (Variables|Default|GetDelta%20Seconds)))
  (Variables|Default|GetMove
    (:then
      (Transformation|SetActorLocation (+ (Transformation|GetActorLocation) (Math|Vector|MakeVector 0.0 0.0 (* (Math|Trig|Sin(Radians) (Variables|Default|GetDelta%20Seconds)) 1e+03))) false false))
    (:else)))

(fn ConstructionScript)