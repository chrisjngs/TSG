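; Health component that tracks an owning actor's health, subtracts damage and signals damage taken and component destruction.
; TakeDamage creates a screen-space BPW_HealthBar widget component on the owner when none exists, or refreshes the existing one.
; The bar's colour comes from a data table row by health-fraction thresholds, and functions show or hide it.
; The destruction check subtracts damage a second time, so it can fire before health reaches zero.
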(event EventBeginPlay)

(event EventTick
  (params (DeltaSeconds :type Float%20%28single-precision%29)))

(fn TakeDamage
  (params (DamageAmount :type Float%20%28double-precision%29))
  (Variables|Default|SetCurrentHealth (- (Variables|Default|GetCurrentHealth) DamageAmount))
  (Variables|Default|GetHealthBarComponent
    (:then
      (CallFunction|UpdateHealthBar))
    (:else
      (CallFunction|CreateHealthBar)))
  (Default|CallDamageTaken)
  (if (<= (- (Variables|Default|GetCurrentHealth) DamageAmount) 0.0)
    (Default|CallComponentDestrroyed)))

(fn SetStartingHealth
  (params (Health :type Float%20%28double-precision%29))
  (bind _output_get (Variables|Default|SetMaxHealth Health))
  (Variables|Default|SetCurrentHealth _output_get))

(fn CreateHealthBar
  (bind _returnvalue (Components|GetOwner))
  (Variables|Default|GetHealthBarComponent
    (:then)
    (:else
      (if (< (Variables|Default|GetCurrentHealth) (Variables|Default|GetMaxHealth))
        (bind _returnvalue_2 (Game|AddComponentbyClass _returnvalue "/Script/UMG.WidgetComponent" false (Math|Transform|MakeTransform "0, 0, 0" "0, 0, 0" "10.000000,10.000000,10.000000")))
        (Variables|Default|SetHealthBarComponent _returnvalue_2)
        (bind _returnvalue_3 (UserInterface|CreateWidget "/Game/Blueprints/Components/HealthSystem/BPW_HealthBar.BPW_HealthBar_C" (Game|GetPlayerController 0) (Variables|Default|GetMaxHealth) "(R=1.000000,G=0.001470,B=0.994769,A=1.000000)" (Components|GetOwner)))
        (bind _output_get (Variables|Default|SetHealthBar _returnvalue_3))
        (UserInterface|SetWidget (Variables|Default|GetHealthBarComponent) _output_get)
        (Class|WidgetComponent|SetWidgetSpace (Variables|Default|GetHealthBarComponent) "Screen")
        (Class|WidgetComponent|SetDrawSize (Variables|Default|GetHealthBarComponent) "(X=100.000000,Y=15.000000)")
        (Transformation|AttachComponentToComponent (Variables|Default|GetHealthBarComponent) (Variables|/Script/Engine.Actor|GetRootComponent _returnvalue) "None" "SnapToTarget" "KeepWorld" "KeepWorld" true)
        (CallFunction|UpdateHealthBar)))))

(fn UpdateHealthBar
  (bind _currenthealth (Variables|Default|GetCurrentHealth))
  (bind _healthbar (Variables|Default|GetHealthBar))
  (bind _maxhealth (Variables|Default|GetMaxHealth))
  (bind _returnvalue (Math|Float|MapRangeClamped _currenthealth 0.0 _maxhealth 0.0 1.0))
  ;[0.15 0.15 0.15 0.5] Get the health bar color if the health bar is created.
  (Variables|Default|GetHealthBar
    (:then
      (bind _returnvalue_2 (Utilities|GetDataTableRow (Variables|Default|GetHealthDataTable) "HealthBar")
        (:then
          ;[0.15 0.15 0.15 0.5] Set health bar color based on the percent left
          (if (== _returnvalue 1.0)
            (Variables|/Game/Blueprints/Components/HealthSystem/BPW_HealthBar.BPW_HealthBar_C|SetHealthBarColor _healthbar (.Fullhealth (Utilities|Struct|BreakS_HealthColors _returnvalue_2)))
            (elif (>= _returnvalue 0.8)
              (Variables|/Game/Blueprints/Components/HealthSystem/BPW_HealthBar.BPW_HealthBar_C|SetHealthBarColor _healthbar (.80Health (Utilities|Struct|BreakS_HealthColors _returnvalue_2)))
              (elif (>= _returnvalue 0.6)
                (Variables|/Game/Blueprints/Components/HealthSystem/BPW_HealthBar.BPW_HealthBar_C|SetHealthBarColor _healthbar (.60Health (Utilities|Struct|BreakS_HealthColors _returnvalue_2)))
                (elif (>= _returnvalue 0.4)
                  (Variables|/Game/Blueprints/Components/HealthSystem/BPW_HealthBar.BPW_HealthBar_C|SetHealthBarColor _healthbar (.40Health (Utilities|Struct|BreakS_HealthColors _returnvalue_2)))
                  (elif (>= _returnvalue 0.2)
                    (Variables|/Game/Blueprints/Components/HealthSystem/BPW_HealthBar.BPW_HealthBar_C|SetHealthBarColor _healthbar (.20Health (Utilities|Struct|BreakS_HealthColors _returnvalue_2)))
                    (elif (== _returnvalue 0.0)
                      (Variables|/Game/Blueprints/Components/HealthSystem/BPW_HealthBar.BPW_HealthBar_C|SetHealthBarColor _healthbar (.Destroyed (Utilities|Struct|BreakS_HealthColors _returnvalue_2))))))))))))
    (:else)))

(fn ShowHealthBar
  (bind _healthbar (Variables|Default|GetHealthBar)
    (:then
      (Variables|/Script/UMG.Widget|SetVisibility _healthbar "HitTestInvisible"))
    (:else)))

(fn HideHealthBar
  (bind _healthbar (Variables|Default|GetHealthBar)
    (:then
      (Variables|/Script/UMG.Widget|SetVisibility _healthbar "Hidden"))
    (:else)))