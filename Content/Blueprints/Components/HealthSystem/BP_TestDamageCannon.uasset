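; Test cannon in the health system folder that loads test missiles aimed at the player ship's core.
; Construction sizes two spheres: tracking overlap finds the ShipCore capsule and loads a missile, while engagement overlap calls FireProjectile.
; Loading spawns the missile at the barrel, passes tracking settings and binds its explode event.
; FireProjectile only checks validity and launches nothing; separate routines destroy and reload missiles after retriggerable delays.
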(event OnComponentBeginOverlap(TrackingRange_Collision)
  (params (OverlappedComponent :type Primitive%20Component%20Object%20Reference) (OtherActor :type Actor%20Object%20Reference) (OtherComp :type Primitive%20Component%20Object%20Reference) (OtherBodyIndex :type Integer) (bFromSweep :type Boolean) (SweepResult :type Hit%20Result%20Structure%20%28by%20ref%29))
  ;[0.15 0.15 0.15 0.5] Start tracking the player ship
  (bind _outactors (Actor|GetAllActorsOfClass "/Game/Actors/Ships/Ship_Core/Blueprints/BP_ShipSystem_Base.BP_ShipSystem_Base_C"))
  (if (== (Utilities|Array|Get(acopy) _outactors) OtherActor)
    (Variables|Default|SetPlayerShipToTrack (Utilities|Array|Get(acopy) (Actor|GetComponentsbyTag OtherActor "/Script/Engine.CapsuleComponent" "ShipCore")))
    (CallFunction|LoadNewProjectile)))

(event OnComponentBeginOverlap(EngagementRange_Collision)
  (params (OverlappedComponent :type Primitive%20Component%20Object%20Reference) (OtherActor :type Actor%20Object%20Reference) (OtherComp :type Primitive%20Component%20Object%20Reference) (OtherBodyIndex :type Integer) (bFromSweep :type Boolean) (SweepResult :type Hit%20Result%20Structure%20%28by%20ref%29))
  ;[0.15 0.15 0.15 0.5] Engage the player ship when it enters range
  (bind _playershiptotrack (Variables|Default|GetPlayerShipToTrack)
    (:then
      (if (== _playershiptotrack OtherActor)
        (Variables|Default|GetProjectileLoaded
          (:then
            _)
          (:else
            (CallFunction|LoadNewProjectile)))
        (CallFunction|FireProjectile)))
    (:else)))

(event Custom|LoadNewProjectile
  (bind _barrelexit (Variables|Default|GetBarrelExit))
  (bind _playershiptotrack (Variables|Default|GetPlayerShipToTrack))
  (bind _returnvalue (Transformation|GetWorldTransform _barrelexit))
  (bind _returnvalue_2 (Transformation|GetWorldTransform _playershiptotrack))
  (bind _location (Math|Transform|BreakTransform _returnvalue))
  (bind _location_2 (Math|Transform|BreakTransform _returnvalue_2))
  (bind _returnvalue_3 (Game|SpawnActorfromClass "/Game/Actors/WeaponSystems/Projectiles/Missiles/BP_BasicMissile_Test.BP_BasicMissile_Test_C" _returnvalue "Undefined" "MultiplyWithRoot" 0 true "NewEnumerator3" "/Game/Actors/WeaponSystems/Projectiles/__DataAssets/ZZZ_DefensiveBullet.ZZZ_DefensiveBullet" 0))
  (bind _output_get (Variables|Default|SetProjectile _returnvalue_3))
  (EventDispatchers|BindEventtoMissileExplode _output_get (EventDispatchers|CreateEvent :!event Custom|Event_DestroyMissile))
  (Transformation|SetActorRotation _output_get (Math|Rotator|FindLookatRotation _location _location_2))
  (Variables|/Game/Actors/WeaponSystems/Projectiles/Missiles/BP_BasicMissile_Test.BP_BasicMissile_Test_C|SetTrackingTarget (Variables|Default|GetProjectile) (Variables|Default|GetPlayerShipToTrack))
  (Variables|/Game/Actors/WeaponSystems/Projectiles/Missiles/BP_BasicMissile_Test.BP_BasicMissile_Test_C|SetTracking (Variables|Default|GetProjectile) (Variables|Default|GetTracking))
  (Utilities|Array|Add (Variables|/Game/Actors/WeaponSystems/Projectiles/BP_Projectile_Base.BP_Projectile_Base_C|GetActorsToIgnore (Variables|Default|GetProjectile)) self)
  (Collision|LineTraceByChannel _location _location_2 "TraceTypeQuery1" false 0 "ForOneFrame")
  (Variables|Default|SetProjectileLoaded true))

(event Custom|FireProjectile
  (bind _projectile (Variables|Default|GetProjectile)
    (:then)
    (:else)))

(event Custom|Event_DestroyMissile
  (bind _projectile (Variables|Default|GetProjectile)
    (:then
      (Actor|DestroyActor _projectile)
      (Utilities|FlowControl|RetriggerableDelay 0.5)
      (CallFunction|LoadNewProjectile)
      (Utilities|FlowControl|RetriggerableDelay 0.5)
      (CallFunction|FireProjectile))
    (:else)))

(fn ConstructionScript
  (Components|Sphere|SetSphereRadius (Variables|Default|GetTrackingRange_Collision) (Variables|Default|GetTrackingRange) true)
  (Components|Sphere|SetSphereRadius (Variables|Default|GetEngagementRange_Collision) (Variables|Default|GetEngagementRange) true))