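; Mission select indicator actor that shows a screen-space marker widget for a mission and broadcasts MissionClicked with its MissionDetails when clicked.
; Construction applies the SpawnHidden flag, creates the marker and hover pop-up widgets, and fills the pop-up with mission name and brief description.
; Cursor and controller hover drive the marker's hover begin/end, and MissionFocused also begins hover.
; Pop-up visibility and camera-relative side offset logic is disconnected.
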(event Custom|Event_ControllerHovered
  (Default|HoverBegin (Variables|Default|GetMissionMarker)))

(event Custom|Event_ControllerEndHovered
  (Default|HoverEnd (Variables|Default|GetMissionMarker)))

(event MouseInput|EventActorBeginCursorOver
  (Default|HoverBegin (Variables|Default|GetMissionMarker)))

(event EventMissionFocused
  (Default|HoverBegin (Variables|Default|GetMissionMarker)))

(event MouseInput|EventActorEndCursorOver
  (Default|HoverEnd (Variables|Default|GetMissionMarker)))

(event MouseInput|EventActorOnClicked
  (params (ButtonPressed :type Key%20Structure :default "None"))
  (Default|CallMissionClicked (Variables|Default|GetMissionDetails)))

(fn ConstructionScript
  (bind _widget (Variables|Default|GetWidget))
  (bind _popupwidget (Variables|Default|GetPopUpWidget))
  (bind _missiondetails (Variables|Default|GetMissionDetails))
  (bind (_missionname _briefdescription) (Utilities|Struct|BreakS_MissionData _missiondetails))
  (Rendering|SetActorHiddenInGame (Variables|Default|GetSpawnHidden))
  (bind _returnvalue (Game|ConstructObjectfromClass "/Game/Blueprints/Components/MissionSelectSystem/Icons/BPW_MissionMarker.BPW_MissionMarker_C"))
  (bind _output_get (Variables|Default|SetMissionMarker _returnvalue))
  (UserInterface|SetWidget _widget _output_get)
  (Class|WidgetComponent|SetWidgetSpace _widget "Screen")
  (Class|WidgetComponent|SetDrawSize _widget (* (Viewport|GetViewportSize) 0.001))
  (bind _returnvalue_2 (Game|ConstructObjectfromClass "/Game/HUD/PremadeWidgets/BPW_HoverPopup.BPW_HoverPopup_C"))
  (bind _output_get_2 (Variables|Default|SetMissionDetailsPopup _returnvalue_2))
  (UserInterface|SetWidget _popupwidget _output_get_2)
  (Class|WidgetComponent|SetWidgetSpace _popupwidget "Screen")
  (Class|WidgetComponent|SetDrawSize _popupwidget "(X=250.000000,Y=250.000000)")
  (Rendering|Components|TextRender|SetText (Variables|/Game/HUD/PremadeWidgets/BPW_HoverPopup.BPW_HoverPopup_C|GetTitle_Text (Variables|Default|GetMissionDetailsPopup)) _missionname)
  (Rendering|Components|TextRender|SetText (Variables|/Game/HUD/PremadeWidgets/Text/BPW_TextBlock.BPW_TextBlock_C|GetPremadeTextBlock_TXT (Variables|/Game/HUD/PremadeWidgets/BPW_HoverPopup.BPW_HoverPopup_C|GetBPW_DetailsText_TXT (Variables|Default|GetMissionDetailsPopup))) _briefdescription))