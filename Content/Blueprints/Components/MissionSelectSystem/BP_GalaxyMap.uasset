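; Galaxy map actor for mission selection that shows a PCG-generated spiral galaxy with clickable mission markers.
; Construction computes logarithmic-spiral arm points with random jitter and writes them to the PCG graph instance.
; SpawnMissionMarkers attaches hidden indicators with random missions at points read from a JSON export.
; Zoom events move and scale the actor on Tick, using camera FOV and the first marker's bounds, then hide the map after zooming in.
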(event Custom|Event_ZoomIntoMission
  (params (Mission :type S%20Mission%20Data%20Structure))
  ;[0.15 0.15 0.15 0.5] This is called from the bound event dispatcher in the mission marker actor
  (Variables|Default|SetDelta%20Seconds 0.0)
  (CallFunction|ZoomGalaxyMap false)
  (Variables|Default|SetZooming true)
  (Default|CallEnterMissionDetailedView Mission)
  (Variables|Default|SetUpdateVisiblility true))

(event Custom|Event_ZoomOutOfMission
  (Variables|Default|SetDelta%20Seconds 0.0)
  (CallFunction|ZoomGalaxyMap true)
  (Variables|Default|SetZooming true)
  (bind _output_get (Variables|Default|SetUpdateVisiblility false))
  (Rendering|SetActorHiddenInGame _output_get))

(event EventTick
  (params (DeltaSeconds :type Float%20%28single-precision%29))
  (Variables|Default|GetZooming
    (:then
      (Variables|Default|SetDelta%20Seconds (+ DeltaSeconds (Variables|Default|GetDelta%20Seconds)))
      (if (> (Variables|Default|GetDelta%20Seconds) 1.0)
        (Variables|Default|SetZooming false)
        (Rendering|SetActorHiddenInGame (Variables|Default|GetUpdateVisiblility))
        (else
          (Transformation|SetActorScale3D (Math|Interpolation|VInterpTo (Variables|MissionZoom|Vectors|GetCurrentScale) (Variables|MissionZoom|Vectors|GetNewScale) (Variables|Default|GetDelta%20Seconds) 1.1))
          (Transformation|SetActorLocation (Math|Interpolation|VInterpTo (Variables|MissionZoom|Vectors|GetCurrentLocation) (Variables|MissionZoom|Vectors|GetNewLocation) (Variables|Default|GetDelta%20Seconds) 1.1) false false))))
    (:else)))

(fn ConstructionScript
  (bind _returnvalue (Transformation|GetActorTransform))
  (bind _returnvalue_2 (Math|Random|RandomFloatinRange 0.0 0.004))
  (bind _starscale (Variables|Default|GetStarScale))
  (bind _pcg_generatedgalaxy (Variables|Default|GetPCG_GeneratedGalaxy))
  (bind _returnvalue_3 (* _starscale 0.001))
  (bind _graphinstance (Variables|/Script/PCG.PCGComponent|GetGraphInstance _pcg_generatedgalaxy))
  (bind _returnvalue_4 (- _returnvalue_3 _returnvalue_2))
  (bind _returnvalue_5 (+ _returnvalue_3 _returnvalue_2))
  (Class|PCGGraphParametersHelpers|SetInt32Parameter _graphinstance "NumberOfArms" (Variables|Default|GetNumberOfArms))
  (Effects|Components|ParticleSystem|SetFloatParameter _graphinstance "StartingRadius" (Variables|Default|GetStartingRadius%20%28a%29))
  (CallFunction|CalculateArmSpiral)
  (Effects|Components|ParticleSystem|SetVectorParameter _graphinstance "StarScale_Min" (Math|Vector|MakeVector _returnvalue_4 _returnvalue_4 _returnvalue_4))
  (Effects|Components|ParticleSystem|SetVectorParameter _graphinstance "StarScale_Max" (Math|Vector|MakeVector _returnvalue_5 _returnvalue_5 _returnvalue_5))
  (Variables|MissionZoom|Vectors|SetStartingScale (.scale _returnvalue))
  (Variables|MissionZoom|Vectors|SetStartingLocation (.location _returnvalue)))

(fn PCGConstruction
  (params (PCG%20Data :type PCG%20Data%20Collection%20Structure))
  (bind _output_get (Variables|Default|SetStartingArmSpacing (Math|Conversions|ToFloat(Integer) (/ (Variables|Default|GetNumberOfArms) 360))))
  (Effects|Components|ParticleSystem|SetFloatParameter "/Game/Blueprints/Components/MissionSelectSystem/PCG/PCG_SpiralGalaxy.PCG_SpiralGalaxy" "StartingArmSpacing" _output_get)
  (Effects|Components|ParticleSystem|SetFloatParameter "/Game/Blueprints/Components/MissionSelectSystem/PCG/PCG_SpiralGalaxy.PCG_SpiralGalaxy" "None" (Variables|Default|GetArmLength%20%28L%29))
  (Effects|Components|ParticleSystem|SetFloatParameter "/Game/Blueprints/Components/MissionSelectSystem/PCG/PCG_SpiralGalaxy.PCG_SpiralGalaxy" "None" (Variables|Default|GetSpiralTightness%20%28b%29))
  (Class|PCGGraphParametersHelpers|SetInt32Parameter "/Game/Blueprints/Components/MissionSelectSystem/PCG/PCG_SpiralGalaxy.PCG_SpiralGalaxy" "InitialPointCount" (Variables|Default|GetInitialPointCount%20%28N%29))
  (Effects|Components|ParticleSystem|SetFloatParameter "/Game/Blueprints/Components/MissionSelectSystem/PCG/PCG_SpiralGalaxy.PCG_SpiralGalaxy" "None" (Variables|Default|GetArmStartingAngle%20%28dOffset%29))
  (PCG|Generate (Variables|Default|GetPCG_GeneratedGalaxy) false))

(fn ForceRegen
  (Class|PCGComponent|GenerateLocal (Variables|Default|GetPCG_GeneratedGalaxy) true)
  (return))

(fn CalculateArmSpiral
  (bind _returnvalue (Math|Random|RandomFloatinRange -5.0 5.0))
  (bind _pcg_generatedgalaxy (Variables|Default|GetPCG_GeneratedGalaxy))
  (bind _initialpointcount__n_ (Variables|Default|GetInitialPointCount%20%28N%29))
  (bind _graphinstance (Variables|/Script/PCG.PCGComponent|GetGraphInstance _pcg_generatedgalaxy))
  (LocalVariables|SetMaxAngle (* (/ 1.0 (/ (Variables|Default|GetSpiralTightness%20%28b%29) (LocalVariables|GetSpiralTightnessRemap))) (Math|Float|Loge (+ (/ (* (Variables|Default|GetArmLength%20%28L%29) (/ (Variables|Default|GetSpiralTightness%20%28b%29) (LocalVariables|GetSpiralTightnessRemap))) (* (Variables|Default|GetStartingRadius%20%28a%29) (Math|Float|Sqrt (+ 1.0 (Math|Float|Power (/ (Variables|Default|GetSpiralTightness%20%28b%29) (LocalVariables|GetSpiralTightnessRemap)) 2.0))))) 1.0))))
  (LocalVariables|SetDeltaAngle (/ (LocalVariables|GetMaxAngle) (- _initialpointcount__n_ 1)))
  (for _index (range 0 _initialpointcount__n_)
    (LocalVariables|SetPointAngle (* _index (LocalVariables|GetDeltaAngle)))
    (LocalVariables|SetRadius (* (Variables|Default|GetStartingRadius%20%28a%29) (Class|KismetMathLibrary|Exp (* (/ (Variables|Default|GetSpiralTightness%20%28b%29) (LocalVariables|GetSpiralTightnessRemap)) (* _index (LocalVariables|GetDeltaAngle))))))
    (Utilities|FlowControl|Sequence
      (:then_0
        (Effects|Components|ParticleSystem|SetVectorParameter _graphinstance (Utilities|String|StringToName (Utilities|String|ToString(Text) (Utilities|Text|FormatText "TransformPoint_0{index}_Min" (+ _index 1)))) (- (Math|Vector|MakeVector (* (LocalVariables|GetRadius) (Math|Trig|Cos(Degrees) (+ (LocalVariables|GetPointAngle) (Variables|Default|GetArmStartingAngle%20%28dOffset%29)))) 0.0 (* (LocalVariables|GetRadius) (Math|Trig|Sin(Degrees) (+ (LocalVariables|GetPointAngle) (Variables|Default|GetArmStartingAngle%20%28dOffset%29))))) _returnvalue)))
      (:then_1
        (Effects|Components|ParticleSystem|SetVectorParameter _graphinstance (Utilities|String|StringToName (Utilities|String|ToString(Text) (Utilities|Text|FormatText "TransformPoint_0{index}_Max" (+ _index 1)))) (+ (Math|Vector|MakeVector (* (LocalVariables|GetRadius) (Math|Trig|Cos(Degrees) (+ (LocalVariables|GetPointAngle) (Variables|Default|GetArmStartingAngle%20%28dOffset%29)))) 0.0 (* (LocalVariables|GetRadius) (Math|Trig|Sin(Degrees) (+ (LocalVariables|GetPointAngle) (Variables|Default|GetArmStartingAngle%20%28dOffset%29))))) _returnvalue))
        (Effects|Components|ParticleSystem|SetVectorParameter _graphinstance "ActorLocation" (Transformation|GetActorLocation))))))

(fn SpawnMissionMarkers
  (bind _returnvalue (Transformation|GetActorTransform))
  (bind _pcgpointvectors (CallFunction|ReadPCGJsonExport (Variables|Default|GetJsonFilePath)))
  (for _index (range 0 (Variables|Default|GetNumberOfMissionPoints))
    (bind _returnvalue_2 (Game|SpawnActorfromClass "/Game/Blueprints/Components/MissionSelectSystem/BP_MissionSelectIndicator.BP_MissionSelectIndicator_C" (Math|Transform|MakeTransform (Utilities|Array|Get(acopy) _pcgpointvectors (Math|Random|RandomIntegerinRange 0 (- (Utilities|Array|Length _pcgpointvectors) 1))) (.rotation _returnvalue) (/ (.scale _returnvalue) 15.0)) "Undefined" "MultiplyWithRoot" 0 (CallFunction|GetRandomMission) true 0))
    (Utilities|Array|Add (Variables|Default|GetAddedMissionMarkers) _returnvalue_2)
    (Transformation|AttachActorToActor _returnvalue_2 self "None" "KeepWorld" "SnapToTarget" "KeepRelative" true)
    (Rendering|SetActorHiddenInGame _returnvalue_2 true)
    (EventDispatchers|BindEventtoMissionClicked _returnvalue_2 (EventDispatchers|CreateEvent :!event Custom|Event_ZoomIntoMission)))
  (return (Variables|Default|GetAddedMissionMarkers)))

(fn ZoomGalaxyMap
  (params (ZoomOut :type Boolean))
  (bind _returnvalue (Game|GetPlayerCameraManager 0))
  (bind _zoomedscreen_ (Variables|MissionZoom|GetZoomedScreen%25))
  (bind _addedmissionmarkers (Variables|Default|GetAddedMissionMarkers))
  (bind _returnvalue_2 (Camera|GetFOVAngle _returnvalue))
  (bind _returnvalue_3 (Camera|GetCameraLocation _returnvalue))
  (bind _output (Utilities|Array|Get(acopy) _addedmissionmarkers))
  (bind (_origin _boxextent) (Collision|GetActorBounds _output false true))
  (bind _returnvalue_4 (/ _returnvalue_2 2.0))
  (bind _returnvalue_5 (Math|Trig|DegreesToRadians _returnvalue_4))
  (bind _returnvalue_6 (Math|Vector|GetMaxElement _boxextent))
  (bind _returnvalue_7 (- _returnvalue_3 _origin))
  (bind _returnvalue_8 (Math|Trig|Tan(Radians) _returnvalue_5))
  (bind _returnvalue_9 (Math|Vector|VectorLength _returnvalue_7))
  (bind _returnvalue_10 (* _returnvalue_6 _returnvalue_8))
  (bind _returnvalue_11 (* _returnvalue_9 _zoomedscreen_))
  (bind _returnvalue_12 (/ _returnvalue_11 _returnvalue_10))
  (Variables|MissionZoom|Vectors|SetCurrentLocation (Transformation|GetActorLocation))
  (Variables|MissionZoom|Vectors|SetCurrentScale (Transformation|GetActorScale3D))
  (if ZoomOut
    ;[0.15 0.15 0.15 0.5] If the map is being zoomed out, then just set everything back to its original position and scale
    (Variables|MissionZoom|Vectors|SetNewLocation (Variables|MissionZoom|Vectors|GetStartingLocation))
    (Variables|MissionZoom|Vectors|SetNewScale (Variables|MissionZoom|Vectors|GetStartingScale))
    (else
      (Variables|MissionZoom|Vectors|SetNewScale (Math|Conversions|ToVector(Float) _returnvalue_12))
      (Variables|MissionZoom|Vectors|SetNewLocation (+ (Variables|MissionZoom|Vectors|GetCurrentLocation) (- (Variables|MissionZoom|Vectors|GetStartingLocation) (Math|Transform|TransformLocation (Math|Transform|MakeTransform (Variables|MissionZoom|Vectors|GetCurrentLocation) (Transformation|GetActorRotation) (Variables|MissionZoom|Vectors|GetCurrentScale)) (* (Math|Transform|InverseTransformLocation (Transformation|GetActorTransform) (Transformation|GetWorldLocation (Variables|/Game/Blueprints/Components/MissionSelectSystem/BP_MissionSelectIndicator.BP_MissionSelectIndicator_C|GetDefaultSceneRoot _output))) _returnvalue_12))))))))

(fn ToggleMissionMarkers
  (params (Hide/Show :type Boolean))
  (for _array_element (Variables|Default|GetAddedMissionMarkers)
    (Rendering|SetActorHiddenInGame _array_element Hide/Show)))