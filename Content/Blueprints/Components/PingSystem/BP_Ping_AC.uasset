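; Actor component for a sonar-like ping that highlights detected objects with an outline.
; SendPing spawns a radius-scaled BP_PingSphere at the source and binds to its object-detected event.
; Each detection is line-traced from the source to confirm visibility, then highlighted through BPI_Ping or given the environment outline overlay material.
; RangeFinding, uncalled here, computes echo distance and round-trip time from sensor speed.
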(event Custom|BindPing
  (EventDispatchers|BindEventtoEventObjectDetected (Variables|Default|GetPingSphere) (delegate Custom|ValidateReturn)))

(event Custom|ValidateReturn
  (params (HitResult :type Actor%20Object%20Reference))
  (bind _validobjects (CallFunction|ValidateContact (Variables|Default|GetPingSource_Global) HitResult))
  (CallFunction|OutlineContact (.HitComponent (Collision|BreakHitResult _validobjects)) (.HitActor (Collision|BreakHitResult _validobjects))))

(fn SendPing
  (params (Ping%20Radius%20in%20Km :type Float%20%28double-precision%29) (PingActor :type Actor%20Object%20Reference) (SourceComponents :type Actor%20Component%20Object%20Reference) (SourceActor :type Actor%20Object%20Reference))
  ;[0.15 0.15 0.15 0.5] Send out a ping from a source with a set radius
  (Variables|Default|SetPingSource_Global PingActor)
  (LocalVariables|SetPing%20Radius Ping%20Radius%20in%20Km)
  (bind _returnvalue (Game|SpawnActorfromClass "/Game/Blueprints/Components/PingSystem/BP_PingSphere.BP_PingSphere_C" (Transformation|GetActorTransform PingActor) "Undefined" "MultiplyWithRoot" 0 (LocalVariables|GetPing%20Radius) SourceComponents SourceActor 0))
  (Variables|Default|SetPingSphere _returnvalue)
  (CallFunction|BindPing))

(fn RangeFinding
  (params (PingLocation :type Vector) (ReturnLocations :type Hit%20Result%20Structure))
  (bind (_bblockinghit _binitialoverlap _time _distance _location _impactpoint _normal _impactnormal _physmat _hitactor) (Collision|BreakHitResult ReturnLocations))
  (LocalVariables|SetPingSource PingLocation)
  (bind _output_get (LocalVariables|SetReturnDistance (Math|Vector|VectorLength (- (LocalVariables|GetPingSource) _impactpoint))))
  (Utilities|Map|Add (LocalVariables|GetReturnMap) _hitactor (Collision|MakeHitResult false false (/ (* _output_get 2.0) (Variables|Default|GetSpeed%20of%20Sensor)) (LocalVariables|GetReturnDistance) (LocalVariables|GetPingSource) _impactpoint "0,0,1" "0,0,1" 0 _hitactor))
  (return (LocalVariables|GetReturnMap)))

(fn ValidateContact
  (params (PingSource :type Actor%20Object%20Reference) (ObjectsInRange :type Actor%20Object%20Reference))
  (bind _returnvalue (Transformation|GetActorLocation PingSource))
  ;[0.15 0.15 0.15 0.5] Run a line trace from the source of the ping to the contact. If the line trace hits the object it's expecting, it returns its hit information.
  (bind _outhit (Collision|LineTraceByChannel _returnvalue (Transformation|GetActorLocation ObjectsInRange) "TraceTypeQuery1" true 0 "None"))
  (if (== (.HitActor (Collision|BreakHitResult _outhit)) ObjectsInRange)
    (return _outhit _returnvalue)))

(fn OutlineContact
  (params (ComponentToOutline :type Actor%20Component%20Object%20Reference) (OwningActor :type Actor%20Object%20Reference))
  ;[0.15 0.15 0.15 0.5] Get the mesh of an actor and then change its overlay material to the outline material
  (bind _asmesh_component (Utilities|Casting|CastToMeshComponent ComponentToOutline))
  (if (Utilities|DoesObjectImplementInterface OwningActor "/Game/Blueprints/Components/PingSystem/BPI_Ping.BPI_Ping_C")
    (Class|BPIPing|HighlightActor(Message) OwningActor _asmesh_component)
    (else
      (Rendering|Material|SetOverlayMaterial _asmesh_component "/Game/Blueprints/Components/PingSystem/OutlineEnvironment_MTL.OutlineEnvironment_MTL" :!class /Script/Engine.MeshComponent))))

(fn ContactType
  (return "NewEnumerator0"))

(fn ObjectDetected
  (params (DetectedObjectHit_In :type Hit%20Result%20Structure) (SensorThatDetected_In :type Actor%20Component%20Object%20Reference))
  (return "" 0))