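; BP_PingTestActor is a test actor for the ping system that reports its ping contact type and handles the end of a ping highlight.
; OutlineStart optionally snaps a supplied crosshair component to the root, waits on a retriggerable delay, then clears overlay materials on all mesh components.
; When a crosshair is included, it is then destroyed, with debug prints reporting the result.
; ObjectDetected is an empty stub.
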(event EventOutlineStart
  (params (TimeOfHighlight :type Float%20%28double-precision%29) (CrosshairComponent :type Widget%20Component%20Object%20Reference) (IncludeWidget :type Boolean))
  (bind _returnvalue (Actor|GetComponentsByClass "/Script/Engine.MeshComponent"))
  ;[0.15 0.15 0.15 0.5] Start a timer to remove the overlay material and then destroy the widget
  (if IncludeWidget
    (Variables|Default|SetCrosshair%20Component CrosshairComponent)
    (Transformation|AttachComponentToComponent CrosshairComponent (Variables|Default|GetDefaultSceneRoot) "None" "SnapToTarget" "KeepWorld" "KeepWorld" true)
    (Utilities|FlowControl|RetriggerableDelay TimeOfHighlight)
    (for _array_element _returnvalue
      (Rendering|Material|SetOverlayMaterial _array_element 0 :!class /Script/Engine.MeshComponent))
    (Utilities|IsValid (Variables|Default|GetCrosshair%20Component)
      (:Is%20Valid
        (Components|DestroyComponent (Variables|Default|GetCrosshair%20Component))
        (Development|PrintString (Utilities|String|ToString(Text) (Utilities|Text|FormatText "The widget was destroyed. it is now \"{widget}\"" (Variables|Default|GetCrosshair%20Component)))))
      (:Is%20Not%20Valid
        (Development|PrintString "The given widget was not valid")))
    (else
      (Utilities|FlowControl|RetriggerableDelay TimeOfHighlight)
      (for _array_element_2 _returnvalue
        (Rendering|Material|SetOverlayMaterial _array_element_2 0 :!class /Script/Engine.MeshComponent)))))

(fn ConstructionScript)

(fn ContactType
  (return (Variables|Default|GetPing%20Contact%20Type)))

(fn ObjectDetected
  (params (DetectedObjectHit_In :type Hit%20Result%20Structure) (SensorThatDetected_In :type Actor%20Component%20Object%20Reference))
  (return "" 0))