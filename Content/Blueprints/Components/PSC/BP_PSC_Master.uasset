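; BP_PSC_Master is a ship platform's PSC, coordinating its weapon and sensor controllers.
; Initialization finds both controllers among the platform components by interface, gets their AI controllers, passes weapons and faction to weapons AI and registers itself with sensor AI.
; Logged contacts that are targetable and of another faction are stored and forwarded to weapons AI.
; Open-fire commands by weapon category and faction changes are relayed through interface messages.
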(event Custom|Event_GetAIControllers
  (Variables|AI|Controllers|SetAIWeaponController (AI|GetAIController (Variables|AI|Pawns|GetWeaponController)))
  (WeaponSystem|Init|InitializeWeaponController)
  (bind _output_get (Variables|AI|Controllers|SetAISensorController (AI|GetAIController (Variables|AI|Pawns|GetSensorController))))
  (Class|BPISensorController|AssignPSC(Message) _output_get self))

(event EventSetPlatformFaction
  (params (Faction :type E_FriendFoe%20Enum :default "NewEnumerator0"))
  (bind _output_get (Variables|Initialize|SetFaction Faction))
  (Class|BPIWeaponController|SetFaction(Message) (Variables|AI|Controllers|GetAIWeaponController) _output_get))

(event EventSetPlatformComponents
  (params (ShipComponent :type S%20Ship%20Child%20Components%20Structure))
  (Variables|Initialize|SetPlatformComponents ShipComponent))

(event EventInitializePSC
  (bind (_foundcontroller _valid) (CallFunction|GetInterfaceComponent (Variables|Initialize|GetPlatformComponents) "/Game/Blueprints/Components/WeaponSystem/BPI_WeaponController.BPI_WeaponController_C"))
  (if _valid
    (Variables|AI|Pawns|SetWeaponController _foundcontroller))
  (bind (_foundcontroller_2 _valid_2) (CallFunction|GetInterfaceComponent (Variables|Initialize|GetPlatformComponents) "/Game/Blueprints/Components/SensorSystem/BPI_SensorController.BPI_SensorController_C"))
  (if _valid_2
    (Variables|AI|Pawns|SetSensorController _foundcontroller_2))
  (CallFunction|EventGetAIControllers))

(event EventAssignPlatform
  (params (AttachedPlatform :type Actor%20Object%20Reference))
  (Variables|Initialize|SetAttached%20Platform AttachedPlatform))

(event EventLogNewContact
  (params (NewContact :type Actor%20Object%20Reference))
  (SensorSystem|Updates|HandleNewContact NewContact))

(event EventSetOpenFire
  (params (FireState :type Boolean) (WeaponType :type E_WS_WeaponFireCategory%20Enum :default "NewEnumerator0"))
  (Class|BPIWeaponController|SetOpenFire(Message) (Variables|AI|Controllers|GetAIWeaponController) WeaponType FireState))

(fn ConstructionScript)

(fn HandleNewContact
  (params (NewContact :type Actor%20Object%20Reference))
  (if (Utilities|DoesObjectImplementInterface NewContact "/Game/Actors/WeaponSystems/BPI_Targetable.BPI_Targetable_C")
    (bind _targetable (Class|BPITargetable|GetTargetable(Message) NewContact))
    (if _targetable
      (bind _factiontype (Class|BPITargetable|GetFactionType(Message) NewContact))
      (if (Utilities|Enum|NotEqual(Enum) _factiontype (Variables|Initialize|GetFaction))
        (Utilities|Array|AddUnique (Variables|Contacts|GetContacts) NewContact)
        (Class|BPIWeaponController|NewContact(Message) (Variables|AI|Controllers|GetAIWeaponController) NewContact)))))

(fn InitializeWeaponController
  (bind _aiweaponcontroller (Variables|AI|Controllers|GetAIWeaponController))
  (Class|BPIWeaponController|SetPlatformComponents(Message) _aiweaponcontroller (Variables|Initialize|GetAttached%20Platform) (Variables|Initialize|GetPlatformComponents))
  (bind _defensiveweapons (Class|BPIPSC|GetDefensiveWeapons(Message) (Variables|Initialize|GetAttached%20Platform)))
  (if (Utilities|Array|IsNotEmpty _defensiveweapons)
    (Class|BPIWeaponController|InitiailzeDefensiveWeapons(Message) _aiweaponcontroller _defensiveweapons))
  (bind _offensiveweapons (Class|BPIPSC|GetOffensiveWeapons(Message) (Variables|Initialize|GetAttached%20Platform)))
  (if (Utilities|Array|IsNotEmpty _offensiveweapons)
    (Class|BPIWeaponController|InitiailzeOffensiveWeapons(Message) _aiweaponcontroller _offensiveweapons))
  (bind _missilelaunchers (Class|BPIPSC|GetMissileLaunchers(Message) (Variables|Initialize|GetAttached%20Platform)))
  (if (Utilities|Array|IsNotEmpty _missilelaunchers)
    (Class|BPIWeaponController|InitiailzeMissileLaunchers(Message) _aiweaponcontroller _missilelaunchers))
  (Class|BPIWeaponController|SetFaction(Message) _aiweaponcontroller (Variables|Initialize|GetFaction)))

(fn GetDefensiveWeapons
  (return 0))

(fn GetMissileLaunchers
  (return 0))

(fn GetOffensiveWeapons
  (return 0))

(fn GetPlatformComponents
  (return 0))

(fn GetPlatformFaction
  (return (Variables|Initialize|GetFaction)))

(fn GetPSCControllers
  (return (Variables|AI|Controllers|GetAIWeaponController) (Variables|AI|Controllers|GetAISensorController)))