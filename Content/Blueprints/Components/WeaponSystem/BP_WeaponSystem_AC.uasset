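; Weapon system actor component that aims its owning weapon at a target and supports ship attachment selection and swapping.
; InitializeAC caches tagged yaw, pitch and roll meshes plus a data asset, which toggleable Tick feeds into RotateWeapon to set WeaponInPosition.
; It also relays fire and reload through dispatchers, initializes ammo and gathers tagged muzzle transforms.
; Helpers handle outline overlays, hover popups and cycling hologram attachment classes; old widget generation is disconnected.
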(event Custom|Event_GenerateWidget
  (params (OwningActor :type Actor%20Soft%20Object%20Reference) (WidgetLocation :type Scene%20Component%20Soft%20Object%20Reference))
  ;[0.15 0.15 0.15 0.5] Old hover widget
)

(event Custom|Event_Reload
  (Default|CallReload))

(event Custom|Event_Fire
  (Default|CallFire))

(event Custom|Event_ToggleTick
  (params (TickEnable :type Boolean))
  ;[0.15 0.15 0.15 0.5] Used to change the tick status
  (Components|Tick|SetComponentTickEnabled TickEnable))

(event EventTick
  (params (DeltaSeconds :type Float%20%28single-precision%29))
  (bind _weaponinposition (CallFunction|RotateWeapon (Variables|WeaponSystem|Initialize|GetYaw%20Component) (Variables|WeaponSystem|Initialize|GetPitch%20Component) (Variables|WeaponSystem|Initialize|GetRoll%20Component) true true false (Variables|Default|GetTarget%20Location) (Variables|Default|GetDataAsset) (Utilities|Time|GetWorldDeltaSeconds) (Variables|WeaponSystem|Initialize|GetAttached%20Platform) (Variables|WeaponSystem|Initialize|GetOwningActor)))
  (Variables|Default|SetWeaponInPosition _weaponinposition))

(fn RenderInteractionWidget
  (params (WidgetTransform :type Transform) (SystemInfo :type BP%20Weapon%20System%20Base%20PDA%20Object%20Reference))
  (bind _widget (Variables|Default|GetWidget))
  (bind _returnvalue (UserInterface|CreateWidget "/Game/HUD/PremadeWidgets/BPW_HoverPopup.BPW_HoverPopup_C" (Game|GetPlayerController 0)))
  (bind _output_get (Variables|HoverEvent|HoverOnly|SetHoverPopup _returnvalue))
  (UserInterface|SetWidget _widget _output_get)
  (Transformation|SetWorldLocation _widget (Transformation|GetWorldLocation (Variables|Default|GetWidget)) false false)
  (Rendering|Components|TextRender|SetText (Variables|/Game/HUD/PremadeWidgets/BPW_HoverPopup.BPW_HoverPopup_C|GetTitle_Text _output_get) (Utilities|Text|ToText(Name) (Variables|/Game/Actors/WeaponSystems/__DataAssets/BP_WeaponSystem_Base_PDA.BP_WeaponSystem_Base_PDA_C|GetWeaponName SystemInfo)))
  (Rendering|Components|TextRender|SetText (Variables|/Game/HUD/PremadeWidgets/Text/BPW_TextBlock.BPW_TextBlock_C|GetPremadeTextBlock_TXT (Variables|/Game/HUD/PremadeWidgets/BPW_HoverPopup.BPW_HoverPopup_C|GetBPW_DetailsText_TXT _output_get)) (Utilities|Text|ToText(String) (Utilities|String|Append "Tracking Range : " (Utilities|String|ToString(Float) (Variables|/Game/Actors/WeaponSystems/__DataAssets/BP_WeaponSystem_Base_PDA.BP_WeaponSystem_Base_PDA_C|GetTrackingRange SystemInfo))))))

(fn HighlightSelectionon
  (params (Actor :type Actor%20Object%20Reference))
  (bind _owningactor (Variables|WeaponSystem|Initialize|GetOwningActor))
  (Utilities|IsValid _owningactor
    (:Is%20Valid
      (for _array_element (Actor|GetComponentsByClass _owningactor "/Script/Engine.StaticMeshComponent")
        (Rendering|Material|SetOverlayMaterial _array_element "/Game/Blueprints/Components/CustomizationSystem/Hologram_OutlineEnvironment_MTL.Hologram_OutlineEnvironment_MTL" :!class /Script/Engine.MeshComponent)))))

(fn HighlightSelectionOff
  (params (Actor :type Actor%20Object%20Reference))
  (Utilities|IsValid Actor
    (:Is%20Valid
      (for _array_element (Actor|GetComponentsByClass Actor "/Script/Engine.StaticMeshComponent")
        (Rendering|Material|SetOverlayMaterial _array_element 0 :!class /Script/Engine.MeshComponent)))))

(fn RemoveInteractionWidget
  (params (Widget :type Widget%20Component%20Object%20Reference))
  (Utilities|IsValid Widget
    (:Is%20Valid
      (Rendering|SetVisibility Widget false false))))

(fn SelectonClick
  (bind _owningactor (Variables|WeaponSystem|Initialize|GetOwningActor)
    (:then
      (if (Class|Actor|IsChildActor _owningactor)
        (return _owningactor)))
    (:else)))

(fn CycleAttachment
  (params (Attachment :type Actor%20Object%20Reference) (ParentComponent :type Scene%20Component%20Object%20Reference))
  (bind _attachmentclassarray (LocalVariables|GetAttachmentClassArray))
  (LocalVariables|GetAttachmentClass
    (:then
      _)
    (:else
      (bind _output_get (LocalVariables|SetAttachmentClass (Utilities|ResolveSoftReference (Utilities|GetClass Attachment))))))
  (Utilities|IsValid Attachment
    (:Is%20Valid
      (LocalVariables|SetArrayIndex (Utilities|Array|FindItem _attachmentclassarray _output_get))
      (if (>= (Utilities|Array|FindItem _attachmentclassarray _output_get) (- (Utilities|Array|Length _attachmentclassarray) 1))
        (LocalVariables|SetArrayIndex 0)
        (else
          (LocalVariables|SetArrayIndex (+ (LocalVariables|GetArrayIndex) 1))))
      (bind _returnvalue (Game|SpawnActorfromClass (Utilities|ResolveSoftReference (Utilities|Array|Get(acopy) (LocalVariables|GetAttachmentClassArray) (LocalVariables|GetArrayIndex))) (Transformation|GetActorTransform Attachment) "Undefined" "MultiplyWithRoot" 0 0))
      (LocalVariables|SetAttachmentClass (Utilities|ResolveSoftReference (Utilities|GetClass _returnvalue)))
      (Transformation|AttachActorToActor _returnvalue (Components|GetOwner ParentComponent) "None" "KeepWorld" "KeepWorld" "SnapToTarget" true)
      (for _array_element (Actor|GetComponentsByClass _returnvalue "/Script/Engine.StaticMeshComponent")
        (Utilities|IsValid _array_element
          (:Is%20Valid
            (Rendering|Material|SetMaterial _array_element 0 "/Game/Actors/Structures/ProxySpaceStation/Materials/Hologram_MTL_Inst.Hologram_MTL_Inst"))))
      (Actor|DestroyActor Attachment))
    (:Is%20Not%20Valid
      (Utilities|Debugging|RaiseScriptError "An error occurred: No valid parent to attach to."))))

(fn GetOwningActor
  (params (Child :type Actor%20Object%20Reference))
  (return (Components|GetOwner Child)))

(fn ValidateAttachmentPoint
  (params (AttachmentToCheck :type Actor%20Object%20Reference))
  (bind _returnvalue (Components|GetOwner AttachmentToCheck))
  (Utilities|IsValid _returnvalue
    (:Is%20Valid
      (LocalVariables|SetValidCheck true)
      (LocalVariables|SetPoint (Actor|GetComponentbyClass _returnvalue "/Script/Engine.SceneComponent")))
    (:Is%20Not%20Valid
      (bind _returnvalue_2 (Game|AddComponentbyClass (Actor|GetAttachParentActor AttachmentToCheck) "/Script/Engine.SceneComponent" true (Transformation|GetActorTransform AttachmentToCheck)))
      ;[0.15 0.15 0.15 0.5] This isn't attaching properly to include the rotation of the hologram
      (Transformation|AttachComponentToComponent _returnvalue_2 (Variables|/Script/Engine.Actor|GetRootComponent AttachmentToCheck) "None" "SnapToTarget" "SnapToTarget" "SnapToTarget" true)
      (LocalVariables|SetPoint _returnvalue_2)
      (LocalVariables|SetValidCheck true)))
  (return (LocalVariables|GetValidCheck) (LocalVariables|GetPoint)))

(fn InitializeAmmo
  (params (MaxAmmo :type Integer))
  (bind _output_get (Variables|Ammunition|SetMaxAmmo MaxAmmo))
  (Variables|Ammunition|SetCurrentAmmo _output_get))

(fn GetProjectileStart
  ;[0.15 0.15 0.15 0.5] Get the transform of any scene components with the tag "ProjectileStartPoint" and add them to the returned array.
  (for _array_element (Actor|GetComponentsbyTag (Components|GetOwner) "/Script/Engine.SceneComponent" "ProjectileStartPoint")
    (Utilities|Array|Add (LocalVariables|GetTempTransformArray) (Transformation|GetWorldTransform _array_element)))
  (return (LocalVariables|GetTempTransformArray)))

(fn InitializeAC
  (params (NewParam :type BP%20Weapon%20System%20Base%20PDA%20Object%20Reference))
  (bind _output_get (Variables|WeaponSystem|Initialize|SetOwningActor (Components|GetOwner)))
  (Variables|WeaponSystem|Initialize|SetYaw%20Component (Class|Actor|FindComponentbyTag _output_get "/Script/Engine.StaticMeshComponent" "Yaw"))
  (Variables|WeaponSystem|Initialize|SetPitch%20Component (Class|Actor|FindComponentbyTag _output_get "/Script/Engine.StaticMeshComponent" "Pitch"))
  (Variables|WeaponSystem|Initialize|SetRoll%20Component (Class|Actor|FindComponentbyTag _output_get "/Script/Engine.StaticMeshComponent" "Roll"))
  (bind _dataasset (Class|BPIWeaponSystem|GetDataAsset(Message) (Variables|WeaponSystem|Initialize|GetOwningActor)))
  (Variables|Default|SetDataAsset _dataasset))