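; Sensor system component that scans ships: while scanning, it sphere-traces from the camera each tick for BPI_Scannable actors.
; Deep scan gathers the target's attached meshes and rebuilds them with its "ShipBase" mesh as hologram-material instanced static meshes.
; A timer lerps the hologram from the target to before the camera, scaled by bounds and FOV, then opens the deep-scan widget.
; Other events rotate the hologram or tear it down.
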(event Custom|Event_ToggleScanning
  (params (On/Off :type Boolean))
  (Components|Tick|SetComponentTickEnabled On/Off))

(event Custom|Event_StartDeepScan
  (bind _scannedstaticmeshcount (Variables|Default|GetScannedStaticMeshCount))
  (bind _hitactor (Variables|Default|GetHitActor)
    (:then
      (CallFunction|EventToggleScanning false)
      (bind (_parentactor _attachedactors) (Class|BPIScannable|GetScannedComponents(Message) _hitactor))
      (Variables|Default|SetAttachedComponents _attachedactors)
      (Variables|Default|GetGatheredComponents
        (:then
          (Variables|Default|GetHologramCreated
            (:then)
            (:else
              (Utilities|FlowControl|Sequence
                (:then_0
                  ;[0.15 0.15 0.15 0.5] Get the parent static mesh actor of the hit actor. Then create an instance of it at its location
                  (bind _array_element (Utilities|Array|ForEachLoopwithBreak (Components|GetChildrenComponents _parentactor true) :!label _label)
                    (:LoopBody
                      (if (Components|ComponentHasTag _array_element "ShipBase")
                        (Variables|Default|SetPlatformBase _array_element)
                        (goto _label Break)))
                    (:Completed
                      (bind _asstatic_mesh_component (Utilities|Casting|CastToStaticMeshComponent (Variables|Default|GetPlatformBase)))
                      (bind _returnvalue (Game|AddComponentbyClass (Game|Player|GetPlayerPawn 0) "/Script/Engine.InstancedStaticMeshComponent" true (Math|Transform|MakeTransform "0, 0, 0")))
                      (Components|StaticMesh|SetStaticMesh _returnvalue (Variables|/Script/Engine.StaticMeshComponent|GetStaticMesh _asstatic_mesh_component))
                      (Components|InstancedStaticMesh|AddInstance _returnvalue (Math|Transform|MakeTransform "0, 0, 0" (.Rotation (Math|Transform|BreakTransform (Transformation|GetWorldTransform _asstatic_mesh_component))) (.Scale (Math|Transform|BreakTransform (Transformation|GetWorldTransform _asstatic_mesh_component)))) false)
                      (bind _output_get (Variables|Default|SetInstancedBase _returnvalue))
                      (for _index (range 0 (Rendering|Material|GetNumMaterials _output_get))
                        (Rendering|Material|SetMaterial _output_get _index "/Game/Actors/Structures/ProxySpaceStation/Materials/Hologram_MTL_Inst.Hologram_MTL_Inst")))))
                (:then_1
                  ;[0.15 0.15 0.15 0.5] Create instances of all of the attached static mesh components on the hit actor.
                  (bind (_keypin _valuepin) (Utilities|Map|ForEachLoop(Map) (Variables|Default|GetScannedStaticMeshCount))
                    (:then
                      (bind _returnvalue_2 (Game|AddComponentbyClass (Game|Player|GetPlayerPawn 0) "/Script/Engine.InstancedStaticMeshComponent" true (Math|Transform|MakeTransform "0, 0, 0")))
                      (Utilities|Array|Add (Variables|Default|GetInstancedComponents) _returnvalue_2)
                      (Components|StaticMesh|SetStaticMesh _returnvalue_2 _keypin)
                      (for _index_2 (range 0 (- _valuepin 1))
                        (Utilities|Array|Clear (Variables|Default|GetTempArray))
                        (for _array_element_2 (Variables|Default|GetStaticMeshes)
                          (if (== _keypin (Variables|/Script/Engine.StaticMeshComponent|GetStaticMesh _array_element_2))
                            (Utilities|Array|Add (Variables|Default|GetTempArray) _array_element_2))))
                      (for _array_element_3 (Variables|Default|GetTempArray)
                        (Components|InstancedStaticMesh|AddInstance _returnvalue_2 (Math|Transform|MakeTransform (- (.Location (Math|Transform|BreakTransform (Transformation|GetWorldTransform _array_element_3))) (.Location (Math|Transform|BreakTransform (Transformation|GetActorTransform (Variables|Default|GetHitActor))))) (.Rotation (Math|Transform|BreakTransform (Transformation|GetWorldTransform _array_element_3))) (.Scale (Math|Transform|BreakTransform (Transformation|GetWorldTransform _array_element_3)))) true)
                        (Transformation|AttachComponentToComponent _returnvalue_2 (Variables|Default|GetInstancedBase) "None" "SnapToTarget" "KeepRelative" "KeepRelative" true)
                        (for _index_3 (range 0 (Rendering|Material|GetNumMaterials _returnvalue_2))
                          (Rendering|Material|SetMaterial _returnvalue_2 _index_3 "/Game/Actors/Structures/ProxySpaceStation/Materials/Hologram_MTL_Inst.Hologram_MTL_Inst"))))
                    (:CompletedPin
                      (Variables|Default|SetHologramCreated true))))
                (:then_2
                  (Variables|Default|SetStartTime (Utilities|Time|GetRealTimeSeconds))
                  (bind _returnvalue_3 (Utilities|Time|SetTimerbyEvent (EventDispatchers|CreateEvent :!event Custom|Event_LerpHologramTransform) (Utilities|Time|GetWorldDeltaSeconds) true true))
                  (Variables|Default|SetHologramMoveTimer _returnvalue_3))))))
        (:else
          ;[0.15 0.15 0.15 0.5] Get all of the attached static mesh components that will be instanced later
          ;;[0.15 0.15 0.15 0.5] This gets the child actor in each weapon actor, then gets the components that make up that child actor.
          (for _array_element_4 (Variables|Default|GetAttachedComponents)
            (for _array_element_5 (Actor|GetComponentsByClass _array_element_4 "/Script/Engine.ChildActorComponent")
              (for _array_element_6 (Components|GetChildrenComponents _array_element_5 true)
                (bind _asstatic_mesh_component_2 (Utilities|Casting|CastToStaticMeshComponent _array_element_6))
                (if (Utilities|Map|Contains (Variables|Default|GetScannedStaticMeshCount) (Variables|/Script/Engine.StaticMeshComponent|GetStaticMesh _asstatic_mesh_component_2))
                  (Utilities|Map|Add _scannedstaticmeshcount (Variables|/Script/Engine.StaticMeshComponent|GetStaticMesh _asstatic_mesh_component_2) (+ (.Value (Utilities|Map|Find _scannedstaticmeshcount (Variables|/Script/Engine.StaticMeshComponent|GetStaticMesh _asstatic_mesh_component_2))) 1))
                  (Utilities|Array|Add (Variables|Default|GetStaticMeshes) _asstatic_mesh_component_2)
                  (else
                    (Utilities|Map|Add _scannedstaticmeshcount (Variables|/Script/Engine.StaticMeshComponent|GetStaticMesh _asstatic_mesh_component_2) 1)
                    (Utilities|Array|Add (Variables|Default|GetStaticMeshes) _asstatic_mesh_component_2))))))
          (Variables|Default|SetGatheredComponents true))))
    (:else
      (Development|PrintString "No valid hit actor"))))

(event Custom|Event_RotateHologram
  (params (RotationVector :type Vector%202D%20Structure))
  (bind _instancedbase (Variables|Default|GetInstancedBase)
    (:then
      (Transformation|AddWorldRotation _instancedbase (Math|Rotator|MakeRotator (* (.y RotationVector) 5.0) 0.0 (* (.x RotationVector) 5.0)) false false))
    (:else)))

(event Custom|Event_EndDeepScan
  (bind _instancedcomponents (Variables|Default|GetInstancedComponents))
  (CallFunction|EventToggleScanning true)
  (Class|InstancedStaticMeshComponent|RemoveInstance (Variables|Default|GetInstancedBase))
  (Components|DestroyComponent (Variables|Default|GetInstancedBase))
  (Variables|Default|SetInstancedBase 0)
  (for _array_element _instancedcomponents
    (Components|InstancedStaticMesh|ClearInstances _array_element)
    (Components|DestroyComponent _array_element))
  (Utilities|Array|Clear _instancedcomponents)
  (Variables|Default|SetGatheredComponents false)
  (Variables|Default|SetHologramCreated false)
  (CallFunction|FocusGame (Game|GetPlayerController 0))
  (Utilities|Time|ClearandInvalidateTimerbyHandle (Variables|Default|GetHologramMoveTimer)))

(event Custom|Event_LerpHologramTransform
  (bind _returnvalue (Utilities|Time|GetRealTimeSeconds))
  (bind _returnvalue_2 (Game|GetPlayerController 0))
  (bind _starttime (Variables|Default|GetStartTime))
  (bind _returnvalue_3 (- _returnvalue _starttime))
  (bind _playercameramanager (Variables|/Script/Engine.PlayerController|GetPlayerCameraManager _returnvalue_2))
  (bind _returnvalue_4 (Math|Float|MapRangeClamped _returnvalue_3 0.0 3.0 1.0 0.0))
  (bind _returnvalue_5 (Transformation|GetActorLocation _playercameramanager))
  (bind _returnvalue_6 (Transformation|GetActorForwardVector _playercameramanager))
  (bind _returnvalue_7 (* _returnvalue_6 3e+02))
  (bind _returnvalue_8 (+ _returnvalue_5 _returnvalue_7))
  (Transformation|SetWorldTransform (Variables|Default|GetInstancedBase) (Math|Transform|Lerp(Transform) (Math|Transform|MakeTransform _returnvalue_8 (Math|Conversions|RotationFromXVector (CallFunction|GetActorBoundVector (Variables|Default|GetHitActor) "Right")) (CallFunction|GetHologramScale 3.0 _returnvalue_8)) (Transformation|GetActorTransform (Variables|Default|GetHitActor)) _returnvalue_4) false false)
  (if (<= _returnvalue_4 0.0)
    (CallFunction|PushContenttoLayer (Game|GetPlayerController 0) "(TagName=\"UI.Layers.GameMenu\")" "/Game/HUD/Modes/SensorMode/BPW_SM_DeepScan.BPW_SM_DeepScan_C")
    (Utilities|Time|ClearandInvalidateTimerbyHandle (Variables|Default|GetHologramMoveTimer))))

(event EventTick
  (params (DeltaSeconds :type Float%20%28single-precision%29))
  (bind _returnvalue (Game|GetPlayerController 0))
  (bind _playercameramanager (Variables|/Script/Engine.PlayerController|GetPlayerCameraManager _returnvalue))
  (bind _returnvalue_2 (Transformation|GetActorLocation _playercameramanager))
  (bind (_outhit _returnvalue_3) (Collision|SphereTraceForObjects _returnvalue_2 (+ _returnvalue_2 (* (Transformation|GetActorForwardVector _playercameramanager) 5e+05)) 2e+02 (Utilities|Array|MakeArray "ObjectTypeQuery1" "ObjectTypeQuery2" "ObjectTypeQuery3") false 0 "ForOneFrame"))
  (if _returnvalue_3
    (if (Utilities|DoesObjectImplementInterface (.HitActor (Collision|BreakHitResult _outhit)) "/Game/Blueprints/Components/SensorSystem/BPI_Scannable.BPI_Scannable_C")
      (bind _output_get (Variables|Default|SetHitActor (.HitActor (Collision|BreakHitResult _outhit))))
      (Development|PrintText (Utilities|Text|FormatText "Hit Actor parent that gets stored {actor}" _output_get) true false "(R=0.042347,G=0.608696,B=0.000000,A=1.000000)" 0.0)
      (else
        (Development|PrintText (Utilities|Text|FormatText "Hit {actor} but it is not scannable" (.HitActor (Collision|BreakHitResult _outhit))) true false "(R=0.608696,G=0.000000,B=0.000000,A=1.000000)" 0.0)
        (Variables|Default|SetGatheredComponents false :!label _label)
        (Variables|Default|SetHitActor 0)))
    (else
      (Development|PrintString "No hit actor from sphere trace" true false "(R=0.000000,G=0.660000,B=1.000000,A=1.000000)" 0.0)
      (goto _label))))

(fn InitializeSAC)

(fn CreateScannedHologram)

(fn HandleHologramRotation
  (params (RotationAmount :type Vector%202D%20Structure)))

(fn RotatewithOffset
  (params (Point :type Vector) (RotationToAdd :type Rotator) (InstanceLocation :type Vector))
  (bind _returnvalue (Components|GetOwner))
  (LocalVariables|SetToPointVector (- InstanceLocation Point))
  (Transformation|SetActorLocation _returnvalue Point false true)
  (Class|Actor|AddActorWorldRotation _returnvalue RotationToAdd)
  (Transformation|AddActorWorldOffset _returnvalue (Math|Vector|RotateVector (LocalVariables|GetToPointVector) RotationToAdd)))

(fn GetRelativeLocation
  (params (InstanceIndex :type Integer) (ISMComponent :type Instanced%20Static%20Mesh%20Component%20Object%20Reference))
  (return (.Location (Math|Transform|BreakTransform (Math|Transform|MakeRelativeTransform (.OutInstanceTransform (Components|InstancedStaticMesh|GetInstanceTransform (Variables|Default|GetInstancedBase) 0 false)) (.OutInstanceTransform (Components|InstancedStaticMesh|GetInstanceTransform ISMComponent InstanceIndex false)))))))

(fn GetHologramScale
  (params (Screen%25 :type Float%20%28double-precision%29) (DesiredLocation :type Vector))
  (bind _returnvalue (Game|GetPlayerCameraManager 0))
  (return (Math|Conversions|ToVector(Float) (/ (* (Math|Vector|VectorLength (- (Camera|GetCameraLocation _returnvalue) DesiredLocation)) Screen%25) (* (Math|Vector|GetMaxElement (.BoxExtent (Collision|GetActorBounds (Variables|Default|GetHitActor) false true))) (Math|Trig|Tan(Radians) (Math|Trig|DegreesToRadians (/ (Camera|GetFOVAngle _returnvalue) 2.0))))))))