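; Actor component that tracks a commander's reputation as total, allocated and available pools, along with a commander level.
; Gains and losses move the level against thresholds in ReputationTable, indexed by row order, resetting the total to that level's starting value.
; Demotion grants half the level's span, and losses cannot drop below row 2.
; Changes recompute availability, flag over-allocation and are sent to the game instance for saving.
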(event EventBeginPlay)

(event EventInitializeSkirmishReputation
  (params (NewTotal :type Integer) (CommanderLevel :type Integer) (Allocated :type Integer))
  (Variables|Reputation|Counts|SetTotalReputation NewTotal)
  (Variables|Commander|SetCommanderLevel CommanderLevel)
  (CallFunction|SetAvailableReputation)
  (Utility|SaveReputation))

(event EventUpdateReputation
  (params (UpdateAmount :type Integer) (Add/Sub :type Boolean))
  (if Add/Sub
    (Reputation|Updates|GainReputation UpdateAmount)
    (else
      (Reputation|Updates|LoseReputation UpdateAmount))))

(fn AllocateReputation
  (params (ReputationToAllocate :type Integer))
  (if (<= (+ (Variables|Reputation|Counts|GetAllocatedReputation) ReputationToAllocate) (Variables|Reputation|Counts|GetTotalReputation))
    (Variables|Reputation|Counts|SetAllocatedReputation (+ (Variables|Reputation|Counts|GetAllocatedReputation) ReputationToAllocate))
    (CallFunction|SetAvailableReputation)
    (Utility|SaveReputation)
    (return true)
    (else
      (return false))))

(fn SetTotalReputation
  (params (CommanderLevel :type Integer) (UseSaveData :type Boolean) (SaveData :type BP%20Player%20Ship%20Save%20Data%20Object%20Reference))
  (bind _commanderreputation (Variables|/Game/Blueprints/SaveLoadSystem/BP_PlayerShipSaveData.BP_PlayerShipSaveData_C|GetCommanderReputation SaveData))
  (bind (_total _allocated _available _commanderlevel) (Utilities|Struct|BreakS_SavedReputation _commanderreputation))
  (if UseSaveData
    (if (> _total 0)
      (Variables|Reputation|Counts|SetTotalReputation _total)
      (Variables|Reputation|Counts|SetAllocatedReputation _allocated)
      (Variables|Reputation|Counts|SetAvailableReputation _available)
      (Variables|Commander|SetCommanderLevel _commanderlevel)
      (return)
      (else
        _)))
  (bind _output_get (Variables|Commander|SetCommanderLevel CommanderLevel))
  (bind _row (Utility|GetDatafromTable _output_get))
  (Variables|Reputation|Counts|SetTotalReputation (Utilities|Struct|BreakS_ReputationLevels _row))
  (CallFunction|SetAvailableReputation)
  (Utility|SaveReputation)
  (return))

(fn UnallocateReputation
  (params (ReputationToUnallocate :type Integer))
  (Variables|Reputation|Counts|SetAllocatedReputation (- (Variables|Reputation|Counts|GetAllocatedReputation) ReputationToUnallocate))
  (CallFunction|SetAvailableReputation)
  (Utility|SaveReputation)
  (return))

(fn GainReputation
  (params (AmountGained :type Integer))
  (Variables|Reputation|Counts|SetTotalReputation (+ (Variables|Reputation|Counts|GetTotalReputation) AmountGained))
  (CallFunction|SetAvailableReputation)
  (bind _row (Utility|GetDatafromTable (+ (Variables|Commander|GetCommanderLevel) 1)))
  (if (>= (Variables|Reputation|Counts|GetTotalReputation) (Utilities|Struct|BreakS_ReputationLevels _row))
    (Development|PrintText (Utilities|Text|FormatText "Total reputation is greater than the required threshold. {total}/{required}" (Variables|Reputation|Counts|GetTotalReputation) (Utilities|Struct|BreakS_ReputationLevels _row)))
    (Variables|Commander|SetCommanderLevel (+ (Variables|Commander|GetCommanderLevel) 1))
    (Development|PrintString "Leveled Up!!!" true true "(R=1.000000,G=0.814847,B=0.002428,A=1.000000)" 5.0)
    (Reputation|Initialize|SetTotalReputation (Variables|Commander|GetCommanderLevel) false)
    (else
      (Utility|SaveReputation))))

(fn GetDatafromTable
  (params (CommanderLevel :type Integer))
  (bind _reputationtable (Variables|Reputation|BaseInfo|GetReputationTable))
  (bind _outrownames (DataTable|GetDataTableRowNames _reputationtable))
  (bind _returnvalue (Utilities|GetDataTableRow _reputationtable (Utilities|Array|Get(acopy) _outrownames CommanderLevel))
    (:then
      (return _returnvalue))
    (:RowNotFound
      (CallFunction|ThrowScriptError "BP_ReputationSystem_AC" "GetDataFromTable" "Tried to get the data table row by name but no row was found." "A row name" (Utilities|Text|ToText(Name) (Utilities|Array|Get(acopy) _outrownames CommanderLevel))))))

(fn LoseReputation
  (params (AmountLost :type Integer))
  (bind _row (Utility|GetDatafromTable 2))
  (if (>= (- (Variables|Reputation|Counts|GetTotalReputation) AmountLost) (Utilities|Struct|BreakS_ReputationLevels _row))
    (Variables|Reputation|Counts|SetTotalReputation (- (Variables|Reputation|Counts|GetTotalReputation) AmountLost))
    (CallFunction|SetAvailableReputation)
    (bind _row_2 (Utility|GetDatafromTable (Variables|Commander|GetCommanderLevel)))
    (if (<= (Variables|Reputation|Counts|GetTotalReputation) (Utilities|Struct|BreakS_ReputationLevels _row_2))
      (if (>= (- (Variables|Commander|GetCommanderLevel) 1) 2)
        (Variables|Commander|SetCommanderLevel (- (Variables|Commander|GetCommanderLevel) 1))
        (Development|PrintString "Level Lost!!!" true true "(R=0.608696,G=0.000000,B=0.000000,A=1.000000)" 5.0)
        (Reputation|Initialize|SetTotalReputation (Variables|Commander|GetCommanderLevel) false)
        ;[0.15 0.15 0.15 0.5] Add half of the required amount of reputation so that players don't start at the bottom when demoted.
        (bind _row_3 (Utility|GetDatafromTable (Variables|Commander|GetCommanderLevel)))
        (bind _row_4 (Utility|GetDatafromTable (+ (Variables|Commander|GetCommanderLevel) 1)))
        (Reputation|Updates|GainReputation (/ (- (Utilities|Struct|BreakS_ReputationLevels _row_4) (Utilities|Struct|BreakS_ReputationLevels _row_3)) 2))
        (else
          (Utility|SaveReputation)))
      (else
        (Utility|SaveReputation)))
    (else
      (Variables|Reputation|Counts|SetTotalReputation (Utilities|Struct|BreakS_ReputationLevels _row))
      (CallFunction|SetAvailableReputation)
      (Utility|SaveReputation))))

(fn SaveReputation
  (Class|BPISaveGame|UpdatePlayerCommanderReputation(Message) (Game|GetGameInstance) (Utilities|Struct|MakeS_SavedReputation (Variables|Reputation|Counts|GetTotalReputation) (Variables|Reputation|Counts|GetAllocatedReputation) (Variables|Reputation|Counts|GetAvailableReputation) (Variables|Commander|GetCommanderLevel))))

(fn SetAvailableReputation
  (bind _output_get (Variables|Reputation|Counts|SetAvailableReputation (- (Variables|Reputation|Counts|GetTotalReputation) (Variables|Reputation|Counts|GetAllocatedReputation))))
  (if (< _output_get 0)
    (Variables|Default|SetOverAllocated true)
    (else
      (Variables|Default|SetOverAllocated false))))

(fn GetCurrentReputation
  (return (Variables|Reputation|Counts|GetTotalReputation) (Variables|Reputation|Counts|GetAllocatedReputation) (Variables|Reputation|Counts|GetAvailableReputation) (Variables|Commander|GetCommanderLevel)))