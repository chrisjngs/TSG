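; Actor component that lets its owner interact with nearby actors implementing BPI_Interact, showing an on-screen icon at the target.
; Overlap events from a supplied collision component maintain the in-range list, whose newest entry becomes the active target.
; A screen-space widget component created at BeginPlay displays that target's interaction type.
; IA_Interact triggers Press targets immediately, while Hold targets use a temporarily bound dispatcher to update progress and fire after a fixed duration.
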(event Custom|EventComponentBeginOverlap
  (params (OverlappedComponent :type Primitive%20Component%20Object%20Reference) (OtherActor :type Actor%20Object%20Reference) (OtherComp :type Primitive%20Component%20Object%20Reference) (OtherBodyIndex :type Integer) (bFromSweep :type Boolean) (SweepResult :type Hit%20Result%20Structure%20%28by%20ref%29))
  ;[0.15 0.15 0.15 0.5] When the actor overlaps something, check to see if it is interactable. If it is then add it to the array. When leaving the range, remove the object from the array.
  (if (Utilities|DoesObjectImplementInterface OtherActor "/Game/Blueprints/Components/InteractionSystem/BPI_Interact.BPI_Interact_C")
    (Utilities|Array|AddUnique (Variables|Default|GetInteractablesInRange) OtherActor)
    (CallFunction|RenderInteractionWidget)))

(event Custom|EventComponentEndOverlap
  (params (OverlappedComponent :type Primitive%20Component%20Object%20Reference) (OtherActor :type Actor%20Object%20Reference) (OtherComp :type Primitive%20Component%20Object%20Reference) (OtherBodyIndex :type Integer))
  ;[0.15 0.15 0.15 0.5] When the actor overlaps something, check to see if it is interactable. If it is then add it to the array. When leaving the range, remove the object from the array.
  (if (Utilities|DoesObjectImplementInterface OtherActor "/Game/Blueprints/Components/InteractionSystem/BPI_Interact.BPI_Interact_C")
    (Utilities|Array|RemoveItem (Variables|Default|GetInteractablesInRange) OtherActor)
    (CallFunction|RenderInteractionWidget)))

(event Custom|InteractWithActiveInteractable
  (Class|BPIInteract|Interact(Message) (CallFunction|GetActiveInteractable) (Components|GetOwner)))

(event Custom|InteractBegin
  (bind _activeinteractable (CallFunction|GetActiveInteractable))
  (Utilities|IsValid _activeinteractable
    (:Is%20Valid
      (bind _type (Class|BPIInteract|GetInteractType(Message) _activeinteractable))
      (switch Utilities|FlowControl|Switch|SwitchonE_InteractionTypes _type
        (:NewEnumerator0
          (CallFunction|InteractwithActiveInteractable)
          (Widget|SetVisibility (Variables|Default|GetInteractWidget) "Hidden"))
        (:NewEnumerator1
          (EventDispatchers|BindEventtoInteractionHoldBegin (delegate Custom|InteractHold)))))))

(event Custom|InteractHold
  (params (HoldTime :type Float%20%28double-precision%29))
  (bind _interactwidget (Variables|Default|GetInteractWidget))
  (bind _interactwidget_2 (Variables|Default|GetInteractWidget)
    (:then
      (Class|BPIInteract|InteractProgress(Message) _interactwidget_2 (/ HoldTime 1.0)))
    (:else
      _))
  (if (> HoldTime 1.0)
    (CallFunction|InteractwithActiveInteractable)
    (EventDispatchers|UnbindEventfromInteractionHoldBegin (delegate Custom|InteractHold))
    (Class|BPIInteract|InteractProgress(Message) _interactwidget 0.0)
    (Widget|SetVisibility _interactwidget "Hidden")))

(event Custom|Event_InitializeInteractAC
  (params (InteractionCapsule :type Capsule%20Component%20Object%20Reference))
  ;[0.15 0.15 0.15 0.5] Initialize the interact AC
  (CallFunction|InitializeInteractAC InteractionCapsule))

(event Input|EnhancedActionEvents|EnhancedInputActionIA_Interact
  (params (ActionValue :type Boolean) (ElapsedSeconds :type Float%20%28double-precision%29) (TriggeredSeconds :type Float%20%28double-precision%29) (InputAction :type Input%20Action%20Object%20Reference :default "/Game/Inputs/Gameplay/IA_Interact.IA_Interact"))
  (bind _interactwidget (Variables|Default|GetInteractWidget))
  (:Started
    (CallFunction|InteractBegin))
  (:Ongoing
    (Default|CallInteractionHoldBegin ElapsedSeconds))
  (:Canceled
    (EventDispatchers|UnbindallEventsfromInteractionHoldBegin :!label _label)
    (Utilities|IsValid _interactwidget
      (:Is%20Valid
        (Class|BPIInteract|InteractProgress(Message) _interactwidget 0.0))))
  (:Completed
    (goto _label)))

(event EventBeginPlay
  ;[0.15 0.15 0.15 0.5] Create the interact widget that will be rendered when an interactable object is in range
  (bind _returnvalue (Game|AddComponentbyClass (Components|GetOwner) "/Script/UMG.WidgetComponent" true))
  (Class|WidgetComponent|SetWidgetSpace _returnvalue "Screen")
  (Class|WidgetComponent|SetDrawSize _returnvalue "(X=50.000000,Y=50.000000)")
  (Variables|Default|SetInteractionWidgetComponent _returnvalue))

(fn RenderInteractionWidget
  (bind _activeinteractable (CallFunction|GetActiveInteractable))
  (bind _interactionwidgetcomponent (Variables|Default|GetInteractionWidgetComponent))
  (Utilities|IsValid (Utilities|Array|Get(acopy) (Variables|Default|GetInteractablesInRange))
    (:Is%20Valid
      (bind _returnvalue (UserInterface|CreateWidget "/Game/Blueprints/Components/InteractionSystem/BPW_InteractIcon.BPW_InteractIcon_C" (Game|GetPlayerController 0)))
      (bind _output_get (Variables|Default|SetInteractWidget _returnvalue))
      (bind _type (Class|BPIInteract|GetInteractType(Message) _activeinteractable))
      (Variables|/Game/Blueprints/Components/InteractionSystem/BPW_InteractIcon.BPW_InteractIcon_C|SetInteractionType _output_get _type)
      (UserInterface|SetWidget _interactionwidgetcomponent _output_get)
      (Transformation|SetWorldLocation _interactionwidgetcomponent (Transformation|GetActorLocation _activeinteractable) false false))
    (:Is%20Not%20Valid
      (UserInterface|SetWidget (Variables|Default|GetInteractionWidgetComponent) 0))))

(fn GetActiveInteractable
  (bind _interactablesinrange (Variables|Default|GetInteractablesInRange))
  (return (Utilities|Array|Get(acopy) _interactablesinrange (Utilities|Array|LastIndex _interactablesinrange))))

(fn InitializeInteractAC
  (params (InteractionRadius :type Capsule%20Component%20Object%20Reference))
  (bind _interactionradius (Variables|Default|GetInteractionRadius)
    (:then
      (EventDispatchers|UnbindallEventsfromOnComponentBeginOverlap _interactionradius)
      (EventDispatchers|UnbindallEventsfromOnComponentEndOverlap _interactionradius))
    (:else
      _))
  (bind _output_get (Variables|Default|SetInteractionRadius InteractionRadius))
  (Collision|BindEventtoOnComponentBeginOverlap _output_get (EventDispatchers|CreateEvent :!event Custom|EventComponentBeginOverlap))
  (Collision|BindEventtoOnComponentEndOverlap _output_get (EventDispatchers|CreateEvent :!event Custom|EventComponentEndOverlap)))