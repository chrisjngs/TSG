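; Euler-to-quaternion Blueprint with hand-written rotation math helpers.
; CalculateQuaternion converts roll, pitch and yaw in degrees to a quaternion using half-angle sine and cosine products, also returning its components.
; QuaternianRotationMatrix builds a matrix from axis-angle quaternion terms, multiplies it by the actor's transform and returns the rotation without applying it.
; AddActorLocalRotationQuaternion applies a plain rotator delta, ignoring its quaternion input.
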(fn CalculateQuaternion
  (params (Roll%20In :type Float%20%28double-precision%29) (Pitch%20In :type Float%20%28double-precision%29) (Yaw%20In :type Float%20%28double-precision%29))
  ;[0.15 0.15 0.15 0.5] Convert Degrees to Radians
  (LocalVariables|SetRoll_Var (Math|Trig|DegreesToRadians Roll%20In))
  (LocalVariables|SetPitch_Var (Math|Trig|DegreesToRadians Pitch%20In))
  (LocalVariables|SetYaw_Var (Math|Trig|DegreesToRadians Yaw%20In))
  ;[0.15 0.15 0.15 0.5] Get sin and cos of pitch roll and yaw
  (LocalVariables|Setcy (Math|Trig|Cos(Radians) (* (LocalVariables|GetYaw_Var) 0.5)))
  (LocalVariables|Setsy (Math|Trig|Sin(Radians) (* (LocalVariables|GetYaw_Var) 0.5)))
  (LocalVariables|Setcr (Math|Trig|Cos(Radians) (* (LocalVariables|GetRoll_Var) 0.5)))
  (LocalVariables|Setsr (Math|Trig|Sin(Radians) (* (LocalVariables|GetRoll_Var) 0.5)))
  (LocalVariables|Setcp (Math|Trig|Cos(Radians) (* (LocalVariables|GetPitch_Var) 0.5)))
  (LocalVariables|Setsp (Math|Trig|Sin(Radians) (* (LocalVariables|GetPitch_Var) 0.5)))
  (bind _output_get (LocalVariables|SetQuaternion (Class|KismetMathLibrary|MakeQuat (- (* (* (LocalVariables|Getcy) (LocalVariables|Getsr)) (LocalVariables|Getcp)) (* (* (LocalVariables|Getsy) (LocalVariables|Getcr)) (LocalVariables|Getsp))) (+ (* (* (LocalVariables|Getcy) (LocalVariables|Getcr)) (LocalVariables|Getsp)) (* (* (LocalVariables|Getsy) (LocalVariables|Getsr)) (LocalVariables|Getcp))) (- (* (* (LocalVariables|Getsy) (LocalVariables|Getcr)) (LocalVariables|Getcp)) (* (* (LocalVariables|Getcy) (LocalVariables|Getsr)) (LocalVariables|Getsp))) (+ (* (* (LocalVariables|Getcy) (LocalVariables|Getcr)) (LocalVariables|Getcp)) (* (* (LocalVariables|Getsy) (LocalVariables|Getsr)) (LocalVariables|Getsp))))))
  (return _output_get (- (* (* (LocalVariables|Getcy) (LocalVariables|Getsr)) (LocalVariables|Getcp)) (* (* (LocalVariables|Getsy) (LocalVariables|Getcr)) (LocalVariables|Getsp))) (+ (* (* (LocalVariables|Getcy) (LocalVariables|Getcr)) (LocalVariables|Getsp)) (* (* (LocalVariables|Getsy) (LocalVariables|Getsr)) (LocalVariables|Getcp))) (- (* (* (LocalVariables|Getsy) (LocalVariables|Getcr)) (LocalVariables|Getcp)) (* (* (LocalVariables|Getcy) (LocalVariables|Getsr)) (LocalVariables|Getsp))) (+ (* (* (LocalVariables|Getcy) (LocalVariables|Getcr)) (LocalVariables|Getcp)) (* (* (LocalVariables|Getsy) (LocalVariables|Getsr)) (LocalVariables|Getsp)))))

(fn AddActorLocalRotation(Quaternion)
  (params (Actor :type Actor%20Object%20Reference) (Roll :type Float%20%28double-precision%29) (Pitch :type Float%20%28double-precision%29) (Yaw :type Float%20%28double-precision%29) (Quaternian :type Quat%20Structure))
  (Transformation|AddActorLocalRotation Actor (Math|Rotator|MakeRotator Roll Pitch Yaw) false false))

(fn QuaternianRotationMatrix
  (params (Rotation%20Vector%20Axis :type Vector%20%28by%20ref%29) (Angle :type Float%20%28double-precision%29%20%28by%20ref%29) (Actor :type Actor%20Object%20Reference%20%28by%20ref%29))
  ;[0.15 0.15 0.15 0.5] Initialize Q0
  (LocalVariables|SetQ0 (Math|Trig|Cos(Radians) (Math|Trig|DegreesToRadians (/ Angle 2.0))))
  ;[0.15 0.15 0.15 0.5] Initialize SinValue
  (LocalVariables|SetSinValue (Math|Trig|Sin(Radians) (Math|Trig|DegreesToRadians (/ Angle 2.0))))
  ;[0.15 0.15 0.15 0.5] Initialize MVector NormalizedVector
  (LocalVariables|SetNormalized%20Vector (* (Math|Vector|Normalize Rotation%20Vector%20Axis) (LocalVariables|GetSinValue)))
  ;[0.15 0.15 0.15 0.5] Make Quaternion Values Matrix
  (bind _output_get (LocalVariables|SetQuaternionMatrix (Utilities|Struct|MakeMatrix (Utilities|Struct|MakePlane (LocalVariables|GetQ0) (- (+ (* (Math|Float|Square (.y (LocalVariables|GetNormalized%20Vector))) 2.0) (* (Math|Float|Square (.z (LocalVariables|GetNormalized%20Vector))) 2.0)) 1.0) (- (* (* (LocalVariables|GetQ0) (.z (LocalVariables|GetNormalized%20Vector))) 2.0) (* (* (.y (LocalVariables|GetNormalized%20Vector)) (.x (LocalVariables|GetNormalized%20Vector))) 2.0)) (+ (* (* (.y (LocalVariables|GetNormalized%20Vector)) (LocalVariables|GetQ0)) 2.0) (* (* (.z (LocalVariables|GetNormalized%20Vector)) (.x (LocalVariables|GetNormalized%20Vector))) 2.0))) (Utilities|Struct|MakePlane (LocalVariables|GetQ0) (- (* (* (LocalVariables|GetQ0) (.z (LocalVariables|GetNormalized%20Vector))) 2.0) (* (* (.y (LocalVariables|GetNormalized%20Vector)) (.x (LocalVariables|GetNormalized%20Vector))) 2.0)) (- (+ (* (Math|Float|Square (.x (LocalVariables|GetNormalized%20Vector))) 2.0) (* (Math|Float|Square (.z (LocalVariables|GetNormalized%20Vector))) 2.0)) 1.0) (+ (* (* (.y (LocalVariables|GetNormalized%20Vector)) (LocalVariables|GetQ0)) 2.0) (* (* (.z (LocalVariables|GetNormalized%20Vector)) (.x (LocalVariables|GetNormalized%20Vector))) 2.0))) (Utilities|Struct|MakePlane (LocalVariables|GetQ0) (- (* (* (.y (LocalVariables|GetNormalized%20Vector)) (LocalVariables|GetQ0)) 2.0) (* (* (.z (LocalVariables|GetNormalized%20Vector)) (.x (LocalVariables|GetNormalized%20Vector))) 2.0)) (+ (* (* (LocalVariables|GetQ0) (.x (LocalVariables|GetNormalized%20Vector))) 2.0) (* (* (.z (LocalVariables|GetNormalized%20Vector)) (.y (LocalVariables|GetNormalized%20Vector))) 2.0)) (- (+ (* (Math|Float|Square (.y (LocalVariables|GetNormalized%20Vector))) 2.0) (* (Math|Float|Square (.x (LocalVariables|GetNormalized%20Vector))) 2.0)) 1.0)) (Utilities|Struct|MakePlane (LocalVariables|GetQ0) 0.0 0.0 0.0))))
  (bind _output_get_2 (LocalVariables|SetRotatedMatrix (* _output_get (Math|Transform|ToMatrix(Transform) (Transformation|GetActorTransform Actor)))))
  ;[0.15 0.15 0.15 0.5] Final Transform actor with the final quaternion values
  (return (.Rotation (Math|Transform|BreakTransform (Math|Conversions|ToTransform(Vector) _output_get_2)))))