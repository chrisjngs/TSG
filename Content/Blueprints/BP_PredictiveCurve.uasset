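; BP_PredictiveCurve is an unfinished Blueprint that appears intended to compute points along a predicted curve from a starting location and velocity.
; Its PredictiveCurvePoints function only copies the location, length, velocity and point count inputs into variables.
; Disconnected fragments hold an empty loop, a straight-line SetStartAndEnd endpoint, point-array filling with debug printing, and a return node.
; None of those fragments execute, so no curve is produced.
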(fn PredictiveCurvePoints
  (params (StartingLocation :type Vector) (CurveLength :type Float%20%28double-precision%29) (StartingVelocity :type Vector) (TotalNumberOfPoints :type Integer))
  ;[0.15 0.15 0.15 0.5] Establish variables
  (LocalVariables|SetFirstPoint StartingLocation)
  (LocalVariables|SetFurthestPoint CurveLength)
  (LocalVariables|SetStarting%20Velocity StartingVelocity)
  (LocalVariables|SetNumberOfPoints TotalNumberOfPoints))